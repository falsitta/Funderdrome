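; Turret rocket projectile Blueprint that stages the deployment of three rocket meshes, then ignites and spins.
; A Tick-driven timer staggers the meshes over the first second, lerping each toward local origin and playing its fin-opening animation once.
; After that, smoke and flare effects switch on and the actor rolls continuously.
; A Destroy event removes meshes and flares but only deactivates the smoke.
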(event EventBeginPlay)

(event EventDestroy
  ;[1 1 1] Destroy rocket and deactivate smoke trail
  (Components|DestroyComponent (Variables|Default|GetFlare))
  (Components|DestroyComponent (Variables|Default|GetRocket_Test2))
  (Components|Activation|Deactivate (Variables|Default|GetSmokeTrail)))

(event EventTick
  (params (DeltaSeconds :type Float%20%28single-precision%29))
  (bind _rocket_test (Variables|Default|GetRocket_Test))
  (bind _rocket_test1 (Variables|Default|GetRocket_Test1))
  (bind _rocket_test2 (Variables|Default|GetRocket_Test2))
  (Variables|Default|SetDT DeltaSeconds)
  (if (> (Variables|Default|Gettimer) 1.0)
    (Utilities|FlowControl|Sequence
      (:then_0
        (Utilities|FlowControl|DoOnce false
          (:Completed
            (Components|Activation|SetActive (Variables|Default|Getsmoke1) true false))))
      (:then_1
        _))
    (Transformation|AddActorLocalRotation (Math|Rotator|MakeRotator (* (Variables|Default|GetDT) 1e+03) 0.0 0.0) false false)
    (else
      (if (> (Variables|Default|Gettimer) 0.25)
        (if (> (Variables|Default|Gettimer) 0.5)
          (if (> (Variables|Default|Gettimer) 0.75)
            _
            (else
              (Utilities|FlowControl|Sequence
                (:then_0
                  (Utilities|FlowControl|DoOnce false
                    (:Completed
                      (Components|Animation|PlayAnimation _rocket_test "/Game/BluePrint/Turret/TestTurret/openFin.openFin" false))))
                (:then_1
                  (Transformation|SetRelativeLocation _rocket_test (Math|Vector|Lerp(Vector) (Variables|/Script/Engine.SceneComponent|GetRelativeLocation _rocket_test) "0, 0, 0" 0.05) false false)
                  (Transformation|SetRelativeLocation _rocket_test2 (Math|Vector|Lerp(Vector) (Variables|/Script/Engine.SceneComponent|GetRelativeLocation _rocket_test2) "0, 0, 0" 0.05) false false :!label _label)
                  (Transformation|SetRelativeLocation _rocket_test1 (Math|Vector|Lerp(Vector) (Variables|/Script/Engine.SceneComponent|GetRelativeLocation _rocket_test1) "0, 0, 0" 0.05) false false :!label _label_2)))))
          (else
            (Utilities|FlowControl|Sequence
              (:then_0
                (Utilities|FlowControl|DoOnce false
                  (:Completed
                    (Components|Animation|PlayAnimation _rocket_test2 "/Game/BluePrint/Turret/TestTurret/openFin.openFin" false))))
              (:then_1
                (goto _label)))))
        (else
          (Utilities|FlowControl|Sequence
            (:then_0
              (Utilities|FlowControl|DoOnce false
                (:Completed
                  (Components|Animation|PlayAnimation _rocket_test1 "/Game/BluePrint/Turret/TestTurret/openFin.openFin" false))))
            (:then_1
              (goto _label_2)))))
      (Variables|Default|Settimer (+ (Variables|Default|GetDT) (Variables|Default|Gettimer))))))

(fn ConstructionScript)

(fn ReturnMesh
  ;[1 1 1] Return projectile's mesh
  (return 0))
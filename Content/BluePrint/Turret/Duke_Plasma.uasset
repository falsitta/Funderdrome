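; Duke_Plasma is a plasma projectile Blueprint, filed with the turret assets, that explodes on impact.
; On the first hit of its collision component, a DoOnce gate disables collision, fires the ExplosionForce radial impulse, runs PlasmaPayload at that location and destroys the plasma ball component.
; It then applies full radial damage, taking amount and radius from ExplosionForce so the physics push and damage share one source.
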(event OnComponentHit(CollisionComponent)
  (params (HitComponent :type Primitive%20Component%20Object%20Reference) (OtherActor :type Actor%20Object%20Reference) (OtherComp :type Primitive%20Component%20Object%20Reference) (NormalImpulse :type Vector :default "0, 0, 0") (Hit :type Hit%20Result%20Structure%20%28by%20ref%29))
  (bind _explosionforce (Variables|Default|GetExplosionForce))
  ;[1 1 1] Only on first impact
  (Utilities|FlowControl|DoOnce false
    (:Completed
      (Collision|SetCollisionEnabled (Variables|Default|GetCollisionComponent) "NoCollision")
      ;[1 1 1] Fire impulse
      (Class|RadialForceComponent|FireImpulse (Variables|Default|GetExplosionForce))
      ;[1 1 1] Execute payload
      (Default|Execute (Variables|Default|GetPlasmaPayload) (Transformation|GetWorldLocation (Variables|Default|GetExplosionForce)))
      ;[1 1 1] Destroy plasma ball
      (Components|DestroyComponent (Variables|Default|GetPlasmaBall))
      ;[1 1 1] Apply damage
      (Game|Damage|ApplyRadialDamage (Variables|/Script/Engine.RadialForceComponent|GetDestructibleDamage _explosionforce) (Transformation|GetWorldLocation _explosionforce) (Variables|/Script/Engine.RadialForceComponent|GetRadius _explosionforce) "/Script/Engine.DamageType" 0 self 0 true "ECC_Visibility"))))

(fn ConstructionScript)
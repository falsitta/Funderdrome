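; Duke_Grenade is a turret grenade projectile that explodes on impact, with optional distance and timed fuses.
; Tick measures travel from the BeginPlay start location and a Delay handles the timer; both call Explode, which shares a DoOnce with component hit.
; Detonation disables collision, fires a radial impulse and payload effect, attaches an impact decal and destroys the child-actor grenade.
; Radial damage reuses the explosion force's radius and destructible damage.
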(event OnComponentHit(CollisionComponent)
  (params (HitComponent :type Primitive%20Component%20Object%20Reference) (OtherActor :type Actor%20Object%20Reference) (OtherComp :type Primitive%20Component%20Object%20Reference) (NormalImpulse :type Vector :default "0, 0, 0") (Hit :type Hit%20Result%20Structure%20%28by%20ref%29))
  (bind _explosionforce (Variables|Default|GetExplosionForce))
  ;[1 1 1] On hit or explode event
  (Utilities|FlowControl|DoOnce false
    (:Completed
      (Collision|SetCollisionEnabled (Variables|Default|GetCollisionComponent) "NoCollision")
      ;[1 1 1] Save hit result
      (Variables|Default|SetHitResult Hit)
      ;[1 1 1] Fire impulse
      (Class|RadialForceComponent|FireImpulse (Variables|Default|GetExplosionForce))
      ;[1 1 1] Execute payload
      (Default|Execute (Variables|Default|GetSimpleExplosionPayload) (Transformation|GetWorldLocation (Variables|Default|GetExplosionForce)))
      ;[1 1 1] Save hit component
      (Variables|Default|SetHitComponent (.HitComponent (Collision|BreakHitResult (Variables|Default|GetHitResult))))
      ;[1 1 1] Spawn decal
      (Class|GameplayStatics|SpawnDecalAttached "/Game/ProjectilesPack/Materials/Bullet/M_Impact_Decal.M_Impact_Decal" "200.000000,200.000000,200.000000" (Variables|Default|GetHitComponent) "None" (.Location (Collision|BreakHitResult (Variables|Default|GetHitResult))) (Math|Conversions|RotationFromXVector (.Normal (Collision|BreakHitResult (Variables|Default|GetHitResult)))) "KeepWorldPosition" 6.0)
      ;[1 1 1] Destroy grenade
      (Class|AdvancedProjectile|Destroy(Message) (Variables|/Script/Engine.ChildActorComponent|GetChildActor (Variables|Default|GetBP_Grenade)))
      ;[1 1 1] Apply damage
      (Game|Damage|ApplyRadialDamage (Variables|/Script/Engine.RadialForceComponent|GetDestructibleDamage _explosionforce) (Transformation|GetWorldLocation _explosionforce) (Variables|/Script/Engine.RadialForceComponent|GetRadius _explosionforce) "/Script/Engine.DamageType" 0 self 0 false "ECC_Visibility"))))

(event Custom|Explode
  (bind _explosionforce (Variables|Default|GetExplosionForce))
  ;[1 1 1] On hit or explode event
  (Utilities|FlowControl|DoOnce false
    (:Completed
      (Collision|SetCollisionEnabled (Variables|Default|GetCollisionComponent) "NoCollision")
      ;[1 1 1] Save hit result
      (Variables|Default|SetHitResult (stale OnComponentHit(CollisionComponent) Hit))
      ;[1 1 1] Fire impulse
      (Class|RadialForceComponent|FireImpulse (Variables|Default|GetExplosionForce))
      ;[1 1 1] Execute payload
      (Default|Execute (Variables|Default|GetSimpleExplosionPayload) (Transformation|GetWorldLocation (Variables|Default|GetExplosionForce)))
      ;[1 1 1] Save hit component
      (Variables|Default|SetHitComponent (.HitComponent (Collision|BreakHitResult (Variables|Default|GetHitResult))))
      ;[1 1 1] Spawn decal
      (Class|GameplayStatics|SpawnDecalAttached "/Game/ProjectilesPack/Materials/Bullet/M_Impact_Decal.M_Impact_Decal" "200.000000,200.000000,200.000000" (Variables|Default|GetHitComponent) "None" (.Location (Collision|BreakHitResult (Variables|Default|GetHitResult))) (Math|Conversions|RotationFromXVector (.Normal (Collision|BreakHitResult (Variables|Default|GetHitResult)))) "KeepWorldPosition" 6.0)
      ;[1 1 1] Destroy grenade
      (Class|AdvancedProjectile|Destroy(Message) (Variables|/Script/Engine.ChildActorComponent|GetChildActor (Variables|Default|GetBP_Grenade)))
      ;[1 1 1] Apply damage
      (Game|Damage|ApplyRadialDamage (Variables|/Script/Engine.RadialForceComponent|GetDestructibleDamage _explosionforce) (Transformation|GetWorldLocation _explosionforce) (Variables|/Script/Engine.RadialForceComponent|GetRadius _explosionforce) "/Script/Engine.DamageType" 0 self 0 false "ECC_Visibility"))))

(event EventBeginPlay
  ;[1 1 1] Get start location
  (Variables|Default|SetStartLocation (Transformation|GetWorldLocation (Variables|Default|GetCollisionComponent)))
  ;[1 1 1] Explode after specified amount of time
  (if (Variables|Default|GetUseExplodeTime)
    (Utilities|FlowControl|Delay (Variables|Default|GetExplodeTime))
    (CallFunction|Explode)))

(event EventTick
  (params (DeltaSeconds :type Float%20%28single-precision%29))
  ;[1 1 1] Explode after specified amount of distance
  (if (Variables|Default|GetUseExplodeDistance)
    (if (>= (Math|Vector|VectorLength (- (Transformation|GetWorldLocation (Variables|Default|GetCollisionComponent)) (Variables|Default|GetStartLocation))) (Variables|Default|GetExplodeDistance))
      (CallFunction|Explode))))

(fn ConstructionScript)
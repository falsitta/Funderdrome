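; RandomAimController is a controller for a possessed FunderDromeTurretBase pawn that switches the turret's firing on and off.
; BeginPlay caches the turret and starts it firing.
; Tick accumulates time and, every five seconds, sets the firing flag from a FlipFlop.
; Despite the name, the one-second random yaw and pitch logic is disconnected, so the controller never changes the aim.
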(event EventBeginPlay
  (bind _asfunder_drome_turret_base (Utilities|Casting|CastToFunderDromeTurretBase (Pawn|GetControlledPawn)))
  (bind _output_get (Variables|Default|SetTurret _asfunder_drome_turret_base))
  (Variables|/Game/BluePrint/Turret/FunderDromeTurretBase.FunderDromeTurretBase_C|SetFireing _output_get true))

(event EventTick
  (params (DeltaSeconds :type Float%20%28single-precision%29))
  (Utilities|FlowControl|Sequence
    (:then_0
      (bind _output_get (Variables|Default|Settimer (+ (Variables|Default|Gettimer) DeltaSeconds)))
      (if (> _output_get 5.0)
        (Variables|Default|Settimer 0.0)
        (bind _isa (Utilities|FlowControl|FlipFlop)
          (:A
            _)
          (:B
            _))
        (Variables|/Game/BluePrint/Turret/FunderDromeTurretBase.FunderDromeTurretBase_C|SetFireing (Variables|Default|GetTurret) _isa)))))

(fn ConstructionScript)
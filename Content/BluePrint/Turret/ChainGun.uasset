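; Chain gun turret weapon Blueprint that loads its setup from the WeaponData table.
; WeaponFire accumulates time to pace shots at the table's fire rate, line tracing from the muzzle toward the camera's aim with random cone spread.
; Hits damage drome cars and test payloads, then call WeaponEffect for flag-gated impact sound, particles and decal.
; Firing also sets zoom FOV and builds heat until overheat locks the gun and notifies the player controller.
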(event Custom|WeaponDamage
  (params (Object :type Object%20Object%20Reference) (Location :type Vector) (Normal :type Vector) (AttachToComponent :type Scene%20Component%20Object%20Reference))
  (bind _self self)
  (bind _asfunder_drome_car_base (Utilities|Casting|CastToFunderDromeCarBase Object)
    (:then
      (Game|Damage|ApplyDamage _asfunder_drome_car_base 2.0 0 _self))
    (:CastFailed
      (bind _astest_payload_bp (Utilities|Casting|CastToTestPayloadBP Object)
        (:then
          (Game|Damage|ApplyDamage _astest_payload_bp 5.0 0 _self))
        (:CastFailed
          _))))
  (CallFunction|WeaponEffect false Location Normal AttachToComponent))

(event Custom|WeaponEffect
  (params (Hit? :type Boolean) (Location :type Vector) (Normal :type Vector) (AttachToComponent :type Scene%20Component%20Object%20Reference))
  (if Hit?
    (Audio|PlaySoundatLocation "/Game/Sound/newbullet_Cue.newbullet_Cue" Location "0, 0, 0" 0.2)
    (bind _returnvalue (Effects|SpawnEmitteratLocation "/Game/ProjectilesPack/Particles/Bullet/P_BulletImpact.P_BulletImpact" Location (Math|Conversions|RotationFromXVector (+ Normal "0,90.000000, 0"))))
    (Transformation|SetRelativeScale3D _returnvalue "3.000000,3.000000,3.000000")
    (Class|GameplayStatics|SpawnDecalAttached "/Game/ProjectilesPack/Materials/Bullet/M_Impact_Decal.M_Impact_Decal" "25.000000,25.000000,25.000000" AttachToComponent "None" Location (Math|Conversions|RotationFromXVector Normal) "KeepWorldPosition" 6.0)))

(event EventBeginPlay
  (|CallParentFunction)
  (bind _returnvalue (Utilities|GetDataTableRow "/Game/BluePrint/AllLevels/WeaponData.WeaponData" (Utilities|String|StringToName (Utilities|String|EnumtoString (Variables|Default|GetChainGun))))
    (:then
      (Variables|Default|SetWeaponSetup _returnvalue))))

(event Collision|EventActorBeginOverlap
  (params (OtherActor :type Actor%20Object%20Reference)))

(event EventTick
  (params (DeltaSeconds :type Float%20%28single-precision%29))
  (|CallParentFunction DeltaSeconds))

(event EventWeaponFire
  (bind _weaponsetup (Variables|Default|GetWeaponSetup))
  (bind _weaponmuzzle (Variables|Default|GetWeaponMuzzle))
  (bind _camera (Variables|Default|GetCamera))
  (bind _camera_2 (Variables|Default|GetCamera))
  (bind _returnvalue (Transformation|GetSocketTransform _weaponmuzzle "Muzzle_Socket" "RTS_World"))
  (bind _location (Math|Transform|BreakTransform _returnvalue))
  (|CallParentFunction)
  (if (Math|Boolean|ANDBoolean (Variables|Default|GetFireing) (Variables|Default|GetTurrentReady) (Variables|Default|GetChainGunFiring) (not (Variables|Default|GetOverHeat?)))
    (bind _output_get (Variables|Default|SetChainGunTimer (+ (Variables|Default|GetCoolDownRefreshRate) (Variables|Default|GetChainGunTimer))))
    (if (>= _output_get (.firerate _weaponsetup))
      (Variables|Default|SetChainGunTimer (- _output_get (.firerate _weaponsetup)))
      (Utilities|FlowControl|Sequence
        (:then_0
          (bind (_outhit _returnvalue_2) (Collision|LineTraceByChannel _location (+ (* (Math|Rotator|GetRotationXVector (Math|Rotator|CombineRotators (Math|Rotator|MakeRotator 0.0 (Math|Random|RandomFloatinRange (* (.weaponspread _weaponsetup) -1.0) (.weaponspread _weaponsetup)) 0.0) (Math|Rotator|CombineRotators (Math|Rotator|MakeRotator (Math|Random|RandomFloatinRange -1.8e+02 1.8e+02) 0.0 0.0) (Math|Conversions|RotationFromXVector (- (+ (Transformation|GetWorldLocation _camera_2) (* (Math|Vector|GetForwardVector _camera_2) 1e+05)) _location))))) 5e+03) _location) "TraceTypeQuery1" true 0 "ForOneFrame" true "(R=1.000000,G=0.000000,B=0.000000,A=1.000000)" "(R=0.000000,G=1.000000,B=0.000000,A=1.000000)" 0.5))
          (if _returnvalue_2
            (CallFunction|WeaponDamage (.HitActor (Collision|BreakHitResult _outhit)) (.Location (Collision|BreakHitResult _outhit)) (.Normal (Collision|BreakHitResult _outhit)) (.HitComponent (Collision|BreakHitResult _outhit)))
            (else
              (CallFunction|WeaponEffect (.bBlockingHit (Collision|BreakHitResult _outhit)) (.Location (Collision|BreakHitResult _outhit)) (.Normal (Collision|BreakHitResult _outhit))))))
        (:then_1
          (if (Variables|Default|GetZoom)
            (Camera|SetFieldOfView _camera 55.0)
            (else
              (Camera|SetFieldOfView _camera 85.0)))
          (bind _result (Math|Float|IncrementFloat (Variables|Default|GetHeatAccu))
            (:%20%20
              (if (> _result 1e+02)
                (Variables|Default|SetOverHeat? true)
                (Variables|Default|SetTimer 2.0)
                (bind _asultradrome_player_controller (Utilities|Casting|CastToUltradrome_PlayerController (Pawn|GetController)))
                (Default|OverHeat _asultradrome_player_controller)))))))))

(fn ConstructionScript
  (|CallParentFunction))
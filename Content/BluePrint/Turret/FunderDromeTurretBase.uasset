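; Player-possessed turret base for Ultradrome/FunderDrome, with spring-arm camera aiming, FOV zoom, unpack animations and switchable weapons.
; Pickups fill weapon and ammo arrays from the WeaponData table and update the player controller's UI.
; Looping timers poll fire input and run per-weapon cooldowns.
; The minigun line-traces with spread to damage cars and payloads, while other weapons pass muzzle location and direction to the game mode's WeaponFired.
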(event Custom|TargetKill)

(event Custom|WeaponPickup%20Server
  (params (NewParam :type Duke_WeaponType%20Enum))
  (CallFunction|WeaponPickup NewParam)
  (CallFunction|WeaponPickupSoundCue))

(event Custom|WeaponDamage
  (params (Object :type Object%20Object%20Reference) (Location :type Vector) (Normal :type Vector) (AttachToComponent :type Scene%20Component%20Object%20Reference))
  (bind _self self)
  (bind _asfunder_drome_car_base (Utilities|Casting|CastToFunderDromeCarBase Object)
    (:then
      (Game|Damage|ApplyDamage _asfunder_drome_car_base 2.0 0 _self))
    (:CastFailed
      (bind _astest_payload_bp (Utilities|Casting|CastToTestPayloadBP Object)
        (:then
          (Game|Damage|ApplyDamage _astest_payload_bp 5.0 0 _self))
        (:CastFailed
          _))))
  (CallFunction|WeaponEffect true Location Normal AttachToComponent))

(event Custom|DoRotate
  (params (Rot :type Vector))
  ;[1 1 1] CameraRotation
  (Variables|Replicated|SetCameraRot Rot))

(event Custom|Firing
  ;[1 1 1] Fire & Ammo Handle
  (if (Variables|Default|GetFireing)
    (bind _returnvalue (Utilities|GetDataTableRow "/Game/BluePrint/AllLevels/WeaponData.WeaponData" (Utilities|Array|Get(acopy) (Variables|Replicated|GetObtainedWeaponNames) (Variables|Default|GetcurrentWeapon)))
      (:then
        (switch Utilities|FlowControl|Switch|SwitchonDuke_WeaponType (.WeaponType (Utilities|Struct|BreakWeaponInfo _returnvalue))
          (:NewEnumerator0
            (if (Variables|Default|GetInCoolDownMiniGun)
              (CallFunction|FireFailed :!label _label)
              (else
                (if (Variables|Default|GettestFire) :!label _label_2
                  _
                  (else
                    _))
                (if (or (> (Utilities|Array|Get(acopy) (Variables|Replicated|GetCurrentAmmo) (Variables|Default|GetcurrentWeapon)) 0) (.UnlimitedAmmo (Utilities|Struct|BreakWeaponInfo _returnvalue)))
                  (CallFunction|WeaponFire)
                  (switch Utilities|FlowControl|Switch|SwitchonDuke_WeaponType (.WeaponType (Utilities|Struct|BreakWeaponInfo _returnvalue))
                    (:NewEnumerator0
                      (Variables|Default|SetInCoolDownMiniGun true)
                      (Variables|Default|SetCoolDownTimerMiniGun (.FireRate (Utilities|Struct|BreakWeaponInfo _returnvalue))))
                    (:NewEnumerator1
                      (Variables|Default|SetInCoolDownGrenadeLauncher true)
                      (Variables|Default|SetCoolDownTimerGrenadeLauncher (.FireRate (Utilities|Struct|BreakWeaponInfo _returnvalue))))
                    (:NewEnumerator2
                      (Variables|Default|SetInCoolDownPlasmaGun true)
                      (Variables|Default|SetCoolDownTimerPlasmaGun (.FireRate (Utilities|Struct|BreakWeaponInfo _returnvalue))))
                    (:NewEnumerator3
                      (Variables|Default|SetInCoolDownRailGun true)
                      (Variables|Default|SetCoolDownTimerRailGun (.FireRate (Utilities|Struct|BreakWeaponInfo _returnvalue)))))
                  (else
                    (goto _label))))))
          (:NewEnumerator1
            (if (Variables|Default|GetInCoolDownGrenadeLauncher)
              (goto _label)
              (else
                (goto _label_2))))
          (:NewEnumerator2
            (if (Variables|Default|GetInCoolDownPlasmaGun)
              (goto _label)
              (else
                (goto _label_2))))
          (:NewEnumerator3
            (if (Variables|Default|GetInCoolDownRailGun)
              (goto _label)
              (else
                (goto _label_2)))))))))

(event Custom|TurretSetup_Server
  ;[1 1 1] Turret FirstSetup
  (Variables|Default|SetcurrentWeapon 0)
  (Utilities|Array|Clear (Variables|Replicated|GetCurrentAmmo))
  (Utilities|Array|Clear (Variables|Replicated|GetObtainedWeaponNames))
  (Utilities|Array|Clear (Variables|Replicated|GetObtainedWeapons))
  (CallFunction|WeaponPickup (Variables|Default|GetDefaultWeapon))
  (Variables|Replicated|SetTurrentReady true))

(event Custom|WeaponEffect
  (params (Hit? :type Boolean) (Location :type Vector) (Normal :type Vector) (AttachToComponent :type Scene%20Component%20Object%20Reference))
  (Audio|PlaySoundatLocation "/Game/Sound/MinigunImpack_Cue.MinigunImpack_Cue" (.Location (Math|Transform|BreakTransform (Transformation|GetSocketTransform (Variables|Default|GetWeaponMuzzle) "Muzzle_Socket" "RTS_World"))))
  (if Hit?
    (Audio|PlaySoundatLocation "/Game/Sound/newbullet_Cue.newbullet_Cue" Location)
    (bind _returnvalue (Effects|SpawnEmitteratLocation "/Game/ProjectilesPack/Particles/Bullet/P_BulletImpact.P_BulletImpact" Location (Math|Conversions|RotationFromXVector (+ Normal "0,90.000000, 0"))))
    (Transformation|SetRelativeScale3D _returnvalue "3.000000,3.000000,3.000000")
    (Class|GameplayStatics|SpawnDecalAttached "/Game/ProjectilesPack/Materials/Bullet/M_Impact_Decal.M_Impact_Decal" "25.000000,25.000000,25.000000" AttachToComponent "None" Location (Math|Conversions|RotationFromXVector Normal) "KeepWorldPosition" 6.0)))

(event Custom|UpdateWeapon
  (params (Current :type Integer))
  ;[1 1 1] Update UI
  (bind _asultradrome_player_controller (Utilities|Casting|CastToUltradrome_PlayerController (Game|GetPlayerController 0)))
  (Default|WeaponUpdate _asultradrome_player_controller false (Utilities|Array|Get(acopy) (Variables|Replicated|GetObtainedWeaponNames) Current) (Utilities|Array|Get(acopy) (Variables|Replicated|GetCurrentAmmo) Current)))

(event Custom|UpdateAmmo
  (params (NewAmmo :type Integer))
  ;[1 1 1] Update UI
  (bind _asultradrome_player_controller (Utilities|Casting|CastToUltradrome_PlayerController (Game|GetPlayerController 0)))
  (Default|WeaponUpdate _asultradrome_player_controller true (Utilities|Array|Get(acopy) (Variables|Replicated|GetObtainedWeaponNames) NewAmmo) NewAmmo))

(event Custom|WeaponPickup%20SoundCue)

(event Custom|FireFailed)

(event Custom|WeaponFire
  (bind _weaponmuzzle (Variables|Default|GetWeaponMuzzle))
  (bind _weaponmuzzle_2 (Variables|Default|GetWeaponMuzzle))
  (bind _camera (Variables|Default|GetCamera))
  (bind _returnvalue (Transformation|GetSocketTransform _weaponmuzzle_2 "Muzzle_Socket" "RTS_World"))
  (bind _returnvalue_2 (Math|Vector|GetForwardVector _camera))
  (bind _returnvalue_3 (Transformation|GetWorldLocation _camera))
  (bind _returnvalue_4 (Transformation|GetSocketTransform _weaponmuzzle "Muzzle_Socket" "RTS_World"))
  (bind (_roll _pitch _yaw) (Math|Rotator|BreakRotator (.rotation _returnvalue)))
  (bind _returnvalue_5 (* _returnvalue_2 1e+05))
  (bind (_location _rotation) (Math|Transform|BreakTransform _returnvalue_4))
  (bind _returnvalue_6 (+ _returnvalue_3 _returnvalue_5))
  (bind _returnvalue_7 (- _returnvalue_6 _location))
  (bind _returnvalue_8 (Math|Conversions|RotationFromXVector _returnvalue_7))
  (bind (_roll_2 _pitch_2 _yaw_2) (Math|Rotator|BreakRotator _returnvalue_8))
  ;[1 1 1] Non gravity projectile
  (bind _returnvalue_9 (Utilities|GetDataTableRow "/Game/BluePrint/AllLevels/WeaponData.WeaponData" (Utilities|Array|Get(acopy) (Variables|Replicated|GetObtainedWeaponNames) (Variables|Default|GetcurrentWeapon)))
    (:then
      (bind _asultradrome_player_controller (Utilities|Casting|CastToUltradrome_PlayerController (Pawn|GetController))
        (:then
          (Default|FireRumble _asultradrome_player_controller (.WeaponType (Utilities|Struct|BreakWeaponInfo _returnvalue_9))))
        (:CastFailed
          _))
      (if (.GravityEffect (Utilities|Struct|BreakWeaponInfo _returnvalue_9))
        ;[1 1 1] Projectile affected by gravity
        (CallFunction|SpawnProjectile (.WeaponType (Utilities|Struct|BreakWeaponInfo _returnvalue_9)) (not (.UnlimitedAmmo (Utilities|Struct|BreakWeaponInfo _returnvalue_9))) (.location _returnvalue) (Math|Rotator|GetRotationXVector (Math|Rotator|MakeRotator 0.0 (+ _pitch (Variables|Default|GetGravityOffset)) _yaw)))
        (elif (Utilities|Enum|NotEqual(Enum) (.WeaponType (Utilities|Struct|BreakWeaponInfo _returnvalue_9)) "NewEnumerator0")
          (CallFunction|SpawnProjectile (.WeaponType (Utilities|Struct|BreakWeaponInfo _returnvalue_9)) true _location (Math|Rotator|GetRotationXVector _returnvalue_8))
          (if (== (.Projectile (Utilities|Struct|BreakWeaponInfo _returnvalue_9)) "/Game/BluePrint/Turret/Duke_Grenade.Duke_Grenade_C")
            (Audio|PlaySoundatLocation "/Game/Sound/Grenade_Launcher_SOUND_Effect_Cue.Grenade_Launcher_SOUND_Effect_Cue" (.Location (Math|Transform|BreakTransform (Math|Transform|MakeTransform _location (Math|Rotator|MakeRotator _roll_2 (+ _pitch_2 (Math|Random|RandomFloatinRange (* (.WeaponSpread (Utilities|Struct|BreakWeaponInfo _returnvalue_9)) -1.0) (.WeaponSpread (Utilities|Struct|BreakWeaponInfo _returnvalue_9)))) (+ _yaw_2 (Math|Random|RandomFloatinRange (* (.WeaponSpread (Utilities|Struct|BreakWeaponInfo _returnvalue_9)) -1.0) (.WeaponSpread (Utilities|Struct|BreakWeaponInfo _returnvalue_9)))))))) (.Rotation (Math|Transform|BreakTransform (Math|Transform|MakeTransform _location (Math|Rotator|MakeRotator _roll_2 (+ _pitch_2 (Math|Random|RandomFloatinRange (* (.WeaponSpread (Utilities|Struct|BreakWeaponInfo _returnvalue_9)) -1.0) (.WeaponSpread (Utilities|Struct|BreakWeaponInfo _returnvalue_9)))) (+ _yaw_2 (Math|Random|RandomFloatinRange (* (.WeaponSpread (Utilities|Struct|BreakWeaponInfo _returnvalue_9)) -1.0) (.WeaponSpread (Utilities|Struct|BreakWeaponInfo _returnvalue_9)))))))) 1.0 1.0 0.0 "/Game/Sound/BulletAttenuation.BulletAttenuation")
            (elif (== (.Projectile (Utilities|Struct|BreakWeaponInfo _returnvalue_9)) "/Game/BluePrint/Turret/Duke_Plasma.Duke_Plasma_C")
              (Audio|PlaySoundatLocation "/Game/Sound/Common/PlasmaImpact.PlasmaImpact" (.Location (Math|Transform|BreakTransform (Math|Transform|MakeTransform _location (Math|Rotator|MakeRotator _roll_2 (+ _pitch_2 (Math|Random|RandomFloatinRange (* (.WeaponSpread (Utilities|Struct|BreakWeaponInfo _returnvalue_9)) -1.0) (.WeaponSpread (Utilities|Struct|BreakWeaponInfo _returnvalue_9)))) (+ _yaw_2 (Math|Random|RandomFloatinRange (* (.WeaponSpread (Utilities|Struct|BreakWeaponInfo _returnvalue_9)) -1.0) (.WeaponSpread (Utilities|Struct|BreakWeaponInfo _returnvalue_9)))))))) (.Rotation (Math|Transform|BreakTransform (Math|Transform|MakeTransform _location (Math|Rotator|MakeRotator _roll_2 (+ _pitch_2 (Math|Random|RandomFloatinRange (* (.WeaponSpread (Utilities|Struct|BreakWeaponInfo _returnvalue_9)) -1.0) (.WeaponSpread (Utilities|Struct|BreakWeaponInfo _returnvalue_9)))) (+ _yaw_2 (Math|Random|RandomFloatinRange (* (.WeaponSpread (Utilities|Struct|BreakWeaponInfo _returnvalue_9)) -1.0) (.WeaponSpread (Utilities|Struct|BreakWeaponInfo _returnvalue_9)))))))) 1.0 1.0 0.0 "/Game/Sound/BulletAttenuation.BulletAttenuation")
              (elif (== (.Projectile (Utilities|Struct|BreakWeaponInfo _returnvalue_9)) "/Game/BluePrint/Turret/Duke_Railgun.Duke_Railgun_C")
                (Audio|PlaySoundatLocation "/Game/Sound/RailgunShoot_Cue.RailgunShoot_Cue" (.Location (Math|Transform|BreakTransform (Math|Transform|MakeTransform _location (Math|Rotator|MakeRotator _roll_2 (+ _pitch_2 (Math|Random|RandomFloatinRange (* (.WeaponSpread (Utilities|Struct|BreakWeaponInfo _returnvalue_9)) -1.0) (.WeaponSpread (Utilities|Struct|BreakWeaponInfo _returnvalue_9)))) (+ _yaw_2 (Math|Random|RandomFloatinRange (* (.WeaponSpread (Utilities|Struct|BreakWeaponInfo _returnvalue_9)) -1.0) (.WeaponSpread (Utilities|Struct|BreakWeaponInfo _returnvalue_9)))))))) (.Rotation (Math|Transform|BreakTransform (Math|Transform|MakeTransform _location (Math|Rotator|MakeRotator _roll_2 (+ _pitch_2 (Math|Random|RandomFloatinRange (* (.WeaponSpread (Utilities|Struct|BreakWeaponInfo _returnvalue_9)) -1.0) (.WeaponSpread (Utilities|Struct|BreakWeaponInfo _returnvalue_9)))) (+ _yaw_2 (Math|Random|RandomFloatinRange (* (.WeaponSpread (Utilities|Struct|BreakWeaponInfo _returnvalue_9)) -1.0) (.WeaponSpread (Utilities|Struct|BreakWeaponInfo _returnvalue_9)))))))) 1.0 1.0 0.0 "/Game/Sound/BulletAttenuation.BulletAttenuation"))))
          (else
            (bind (_outhit _returnvalue_10) (Collision|LineTraceByChannel _location (+ (* (Math|Rotator|GetRotationXVector (Math|Rotator|CombineRotators (Math|Rotator|MakeRotator 0.0 (Math|Random|RandomFloatinRange (* (.WeaponSpread (Utilities|Struct|BreakWeaponInfo _returnvalue_9)) -1.0) (.WeaponSpread (Utilities|Struct|BreakWeaponInfo _returnvalue_9))) 0.0) (Math|Rotator|CombineRotators (Math|Rotator|MakeRotator (Math|Random|RandomFloatinRange -1.8e+02 1.8e+02) 0.0 0.0) _returnvalue_8))) 5e+04) _location) "TraceTypeQuery1" true 0 "ForDuration" true "(R=1.000000,G=0.000000,B=0.000000,A=1.000000)" "(R=0.000000,G=1.000000,B=0.000000,A=1.000000)" 0.5))
            (if _returnvalue_10
              (CallFunction|WeaponDamage (.HitActor (Collision|BreakHitResult _outhit)) (.Location (Collision|BreakHitResult _outhit)) (.Normal (Collision|BreakHitResult _outhit)) (.HitComponent (Collision|BreakHitResult _outhit)))
              (else
                (CallFunction|WeaponEffect false "0, 0, 0" "0, 0, 0")))))))))

(event Custom|WeaponSwitchCoolDown
  ;[1 1 1] Weapon Switch Cooldown
  (if (not (<= (Variables|Default|GetWeaponSwitchTimer) 0.0))
    (Variables|Default|SetWeaponSwitchTimer (- (Variables|Default|GetWeaponSwitchTimer) (Variables|Default|GetCoolDownRefreshRate)))))

(event Custom|ClientTag
  (Variables|Default|SetClient true)
  (Variables|Default|SetSpringRot (Math|Rotator|MakeRotator 0.0 0.0 (.Yaw (Math|Rotator|BreakRotator (Transformation|GetWorldRotation (Variables|Default|GetDefaultSceneRoot)))))))

(event Custom|CoolDown
  (bind _cooldownrefreshrate (Variables|Default|GetCoolDownRefreshRate))
  ;[1 1 1] Cooldown Handle
  (Utilities|FlowControl|Sequence
    (:then_0
      (if (Variables|Default|GetInCoolDownMiniGun)
        (if (<= (- (Variables|Default|GetCoolDownTimerMiniGun) _cooldownrefreshrate) 0.0)
          (Variables|Default|SetInCoolDownMiniGun false)
          (Variables|Default|SetCoolDownTimerMiniGun 0.0)
          (else
            (Variables|Default|SetCoolDownTimerMiniGun (- (Variables|Default|GetCoolDownTimerMiniGun) _cooldownrefreshrate))))))
    (:then_1
      (if (Variables|Default|GetInCoolDownGrenadeLauncher)
        (if (<= (- (Variables|Default|GetCoolDownTimerGrenadeLauncher) _cooldownrefreshrate) 0.0)
          (Variables|Default|SetInCoolDownGrenadeLauncher false)
          (Variables|Default|SetCoolDownTimerGrenadeLauncher 0.0)
          (else
            (Variables|Default|SetCoolDownTimerGrenadeLauncher (- (Variables|Default|GetCoolDownTimerGrenadeLauncher) _cooldownrefreshrate))))))
    (:then_2
      (if (Variables|Default|GetInCoolDownPlasmaGun)
        (if (<= (- (Variables|Default|GetCoolDownTimerPlasmaGun) _cooldownrefreshrate) 0.0)
          (Variables|Default|SetInCoolDownPlasmaGun false)
          (Variables|Default|SetCoolDownTimerPlasmaGun 0.0)
          (else
            (Variables|Default|SetCoolDownTimerPlasmaGun (- (Variables|Default|GetCoolDownTimerPlasmaGun) _cooldownrefreshrate))))))
    (:then_3
      (if (Variables|Default|GetInCoolDownRailGun)
        (if (<= (- (Variables|Default|GetCoolDownTimerRailGun) _cooldownrefreshrate) 0.0)
          (Variables|Default|SetInCoolDownRailGun false)
          (Variables|Default|SetCoolDownTimerRailGun 0.0)
          (else
            (Variables|Default|SetCoolDownTimerRailGun (- (Variables|Default|GetCoolDownTimerRailGun) _cooldownrefreshrate))))))))

(event Custom|SpawnProjectile
  (params (WeaponType :type Duke_WeaponType%20Enum) (NeedAmmo? :type Boolean) (Location :type Vector) (Forward :type Vector))
  ;[1 1 1] Projectile
  (Default|WeaponFired (.AsFunder%20Drome%20Base%20Mode (Utilities|Casting|CastToFunderDromeBaseMode (Game|GetGameMode))) self WeaponType Location Forward))

(event Custom|Weapon%20Swap
  (params (Up :type Boolean))
  (bind _currentammo (Variables|Replicated|GetCurrentAmmo))
  (bind _returnvalue (Utilities|Array|LastIndex _currentammo))
  ;[1 1 1] WeaponSwtich
  (if Up
    (if (== (Variables|Replicated|GetCurrentWeapon) _returnvalue)
      (Variables|Replicated|SetCurrentWeapon 0)
      (else
        (Variables|Replicated|SetCurrentWeapon (+ (Variables|Replicated|GetCurrentWeapon) 1))
        (Audio|PlaySoundatLocation "/Game/Sound/Common/WeaponSwap_Cue.WeaponSwap_Cue" (Transformation|GetActorLocation) :!label _label)))
    (elif (== (Variables|Replicated|GetCurrentWeapon) 0)
      (Variables|Replicated|SetCurrentWeapon _returnvalue)
      (else
        (Variables|Replicated|SetCurrentWeapon (- (Variables|Replicated|GetCurrentWeapon) 1))
        (goto _label))))
  (CallFunction|UpdateWeapon (Variables|Replicated|GetCurrentWeapon)))

(event Custom|Target%20Hit
  ;[1 1 1] Target Hit
  (bind _asultradrome_player_controller (Utilities|Casting|CastToUltradrome_PlayerController (Pawn|GetController)))
  (Default|TargetHit _asultradrome_player_controller))

(event EventBeginPlay
  (bind _cooldownrefreshrate (Variables|Default|GetCoolDownRefreshRate))
  ;[1 1 1] TimerSetup
  (Utilities|Time|SetTimerbyEvent (delegate Custom|CoolDown) _cooldownrefreshrate true)
  (Utilities|Time|SetTimerbyEvent (delegate Custom|Firing) _cooldownrefreshrate true)
  ;[1 1 1] Weapon Switch Cooldown
  (Utilities|Time|SetTimerbyEvent (delegate Custom|WeaponSwitchCoolDown) (Variables|Default|GetCoolDownRefreshRate) true)
  (bind _returnvalue (Rendering|Material|CreateDynamicMaterialInstance (Variables|Default|GetWeaponMuzzle) 2 "/Game/Models/Minigun/Material__37.Material__37" :!class /Script/Engine.PrimitiveComponent))
  (Variables|Default|SetcurrentMat _returnvalue)
  (CallFunction|WeaponPickup (Variables|Default|GetDefaultWeapon))
  (CallFunction|UpdateAmmo (Utilities|Array|Get(acopy) (Variables|Replicated|GetCurrentAmmo) (Variables|Replicated|GetCurrentWeapon))))

(event EventActorBeginOverlap
  (params (OtherActor :type Actor%20Object%20Reference)))

(event EventPossessed
  (params (NewController :type Controller%20Object%20Reference))
  (CallFunction|ClientTag)
  (bind _asultradrome_player_controller (Utilities|Casting|CastToUltradrome_PlayerController NewController))
  (Default|SetupUI _asultradrome_player_controller false (Variables|Replicated|GetTeam)))

(event EventTick
  (params (DeltaSeconds :type Float%20%28single-precision%29))
  (bind _springarm (Variables|Default|GetSpringArm))
  (bind _camera (Variables|Default|GetCamera))
  (bind _relativerotation (Variables|/Script/Engine.SceneComponent|GetRelativeRotation _springarm))
  (Variables|Default|SetDeltaT DeltaSeconds)
  (if (and (Variables|Replicated|GetTurrentReady) (Variables|Default|GetNotInAnimation))
    (Utilities|FlowControl|Sequence
      (:then_0
        ;[1 1 1] ZoomHandle
        (if (Variables|Default|GetZoom)
          (if (>= (Variables|Default|Getzoomtimer) 0.0)
            (Variables|Default|Setzoomtimer (- (Variables|Default|Getzoomtimer) (Variables|Default|GetDeltaT)))
            (Variables|/Script/Engine.CameraComponent|SetFieldOfView _camera (Math|Float|Lerp 6e+01 9e+01 (/ (Variables|Default|Getzoomtimer) (Variables|Default|GetZoomTime)))))
          (elif (>= (Variables|Default|Getzoomtimer) 0.0)
            (Variables|Default|Setzoomtimer (- (Variables|Default|Getzoomtimer) (Variables|Default|GetDeltaT)))
            (Variables|/Script/Engine.CameraComponent|SetFieldOfView _camera (Math|Float|Lerp 9e+01 6e+01 (/ (Variables|Default|Getzoomtimer) (Variables|Default|GetZoomTime)))))))
      (:then_1
        (if (Variables|Default|GetClient)
          (CallFunction|DoRotate (Math|Vector|MakeVector 0.0 (.pitch _relativerotation) (.yaw _relativerotation)))
          ;[1 1 1] CameraRotation
          (if (Variables|Default|GetInverted)
            (Variables|Default|SetSpringRot (Math|Rotator|MakeRotator 0.0 (Math|Float|Clamp(Float) (+ (- 0.0 (* (Variables|Default|GetPitch) 9e+01 (Variables|Default|GetDeltaT))) (.pitch (Variables|Default|GetSpringRot))) (Variables|Default|GetMinPitch) (Variables|Default|GetMaxPitch)) (+ (.yaw (Variables|Default|GetSpringRot)) (* (Variables|Default|GetYaw) 1.5e+02 (Variables|Default|GetDeltaT)))))
            (else
              (Variables|Default|SetSpringRot (Math|Rotator|MakeRotator 0.0 (Math|Float|Clamp(Float) (+ (.pitch (Variables|Default|GetSpringRot)) (* (Variables|Default|GetPitch) 9e+01 (Variables|Default|GetDeltaT))) (Variables|Default|GetMinPitch) (Variables|Default|GetMaxPitch)) (+ (.yaw (Variables|Default|GetSpringRot)) (* (Variables|Default|GetYaw) 1.5e+02 (Variables|Default|GetDeltaT)))))))
          (Transformation|SetWorldRotation (Variables|Default|GetSpringArm) (Math|Rotator|MakeRotator 0.0 (.Pitch (Math|Rotator|BreakRotator (Variables|Default|GetSpringRot))) (.Yaw (Math|Rotator|BreakRotator (Variables|Default|GetSpringRot)))) false false))))))

(event Input|ActionEvents|InputActionFire
  (params (Key :type Key%20Structure :default "AnyKey"))
  ;[1 1 1] Fire Input Handle
  (:Pressed
    (Variables|Default|SetFireing true))
  (:Released
    (Variables|Default|SetFireing false)))

(event Input|ActionEvents|InputActionZoomIn
  (params (Key :type Key%20Structure :default "AnyKey"))
  ;[1 1 1] ZoomInput
  (:Pressed
    (Variables|Default|SetZoom true)
    (if (>= (Variables|Default|Getzoomtimer) 0.0) :!label _label
      (Variables|Default|Setzoomtimer (- (Variables|Default|GetZoomTime) (Variables|Default|Getzoomtimer)))
      (else
        (Variables|Default|Setzoomtimer (Variables|Default|GetZoomTime)))))
  (:Released
    (Variables|Default|SetZoom false)
    (goto _label)))

(event Input|ActionEvents|InputActionWeaponSwapLeft
  (params (Key :type Key%20Structure :default "AnyKey"))
  ;[1 1 1] WeaponSwtich
  (:Pressed
    (Utilities|FlowControl|DoOnce false :!label _label
      (:Completed
        (if (<= (Variables|Default|GetWeaponSwitchTimer) 0.0)
          (CallFunction|WeaponSwap true)
          (Variables|Default|SettestFire true)
          (if (> (Utilities|Array|Length (Variables|Replicated|GetCurrentAmmo)) 1)
            (Variables|Default|SetWeaponSwitchTimer 1.0))))))
  (:Released
    (goto _label Reset)))

(event Input|ActionEvents|InputActionWeaponSwapRight
  (params (Key :type Key%20Structure :default "AnyKey"))
  ;[1 1 1] WeaponSwtich
  (:Pressed
    (Utilities|FlowControl|DoOnce false :!label _label
      (:Completed
        (if (<= (Variables|Default|GetWeaponSwitchTimer) 0.0)
          (CallFunction|WeaponSwap false)
          (Variables|Default|SettestFire false)
          (if (> (Utilities|Array|Length (Variables|Replicated|GetCurrentAmmo)) 1)
            (Variables|Default|SetWeaponSwitchTimer 1.0))))))
  (:Released
    (goto _label Reset)))

(event Input|AxisEvents|InputAxisCameraYaw
  (params (AxisValue :type Float%20%28single-precision%29))
  (Variables|Default|SetYaw AxisValue))

(event Input|AxisEvents|InputAxisCameraPitch
  (params (AxisValue :type Float%20%28single-precision%29))
  (Variables|Default|SetPitch AxisValue))

(event Custom|WeaponReadyNormal
  (bind _weaponmuzzle (Variables|Default|GetWeaponMuzzle))
  (Rendering|SetVisibility (Variables|Default|GetWeaponMuzzle) true true)
  (Variables|Default|SetNotInAnimation false)
  (Components|Animation|SetAnimationMode _weaponmuzzle "AnimationSingleNode")
  (Components|Animation|PlayAnimation _weaponmuzzle "/Game/Animations/MuzzleUnpackNormal.MuzzleUnpackNormal" false)
  (Components|Animation|PlayAnimation (Variables|Default|GetWeaponBase) "/Game/Animations/TestAnim.TestAnim" false)
  (Utilities|FlowControl|Delay 3.5)
  (Transformation|SetRelativeRotation (Variables|Default|GetSpringArm) "0, 0, 0" false false)
  (Components|Animation|SetAnimationMode _weaponmuzzle "AnimationBlueprint")
  (Variables|Default|SetNotInAnimation true))

(event Custom|WeaponReadySlow
  (bind _weaponmuzzle (Variables|Default|GetWeaponMuzzle))
  (Rendering|SetVisibility (Variables|Default|GetWeaponMuzzle) true true)
  (Variables|Default|SetNotInAnimation false)
  (Components|Animation|SetAnimationMode _weaponmuzzle "AnimationSingleNode")
  (Components|Animation|PlayAnimation _weaponmuzzle "/Game/Animations/MuzzleUnpackNormal.MuzzleUnpackNormal" false)
  (Components|Animation|PlayAnimation (Variables|Default|GetWeaponBase) "/Game/Animations/TestAnim.TestAnim" false)
  (Components|Timeline|SetPlayRate _weaponmuzzle 0.5)
  (Utilities|FlowControl|Delay 8.0)
  (Transformation|SetRelativeRotation (Variables|Default|GetSpringArm) "0, 0, 0" false false)
  (Components|Animation|SetAnimationMode _weaponmuzzle "AnimationBlueprint")
  (Variables|Default|SetNotInAnimation true))

(fn ConstructionScript)

(fn OnRepCurrentAmmo
  (Utilities|Casting|CastToUltradrome_GameInstance (Game|GetGameInstance)))

(fn WeaponPickup
  (params (WeaponType :type Duke_WeaponType%20Enum))
  (bind _currentammo (Variables|Replicated|GetCurrentAmmo))
  (bind _obtainedweaponnames (Variables|Replicated|GetObtainedWeaponNames))
  (LocalVariables|Set%20GotWeaponName (Utilities|String|StringToName (Utilities|String|EnumtoString WeaponType)))
  (bind _returnvalue (Utilities|GetDataTableRow "/Game/BluePrint/AllLevels/WeaponData.WeaponData" (LocalVariables|Get%20GotWeaponName))
    (:then
      (LocalVariables|SetWeaponDataTemp _returnvalue)
      (if (Utilities|Array|ContainsItem _obtainedweaponnames (LocalVariables|Get%20GotWeaponName))
        (if (not (.UnlimitedAmmo (Utilities|Struct|BreakWeaponInfo (LocalVariables|GetWeaponDataTemp))))
          (Utilities|Array|SetArrayElem _currentammo (Utilities|Array|FindItem (Variables|Replicated|GetObtainedWeaponNames) (LocalVariables|Get%20GotWeaponName)) (Math|Integer|Clamp(Integer) (+ (Utilities|Array|Get(acopy) _currentammo (Utilities|Array|FindItem (Variables|Replicated|GetObtainedWeaponNames) (LocalVariables|Get%20GotWeaponName))) (.PickUpAmmo (Utilities|Struct|BreakWeaponInfo (LocalVariables|GetWeaponDataTemp)))) 0 (.MaxAmmo (Utilities|Struct|BreakWeaponInfo (LocalVariables|GetWeaponDataTemp)))))
          (CallFunction|UpdateAmmo (Utilities|Array|Get(acopy) _currentammo (Variables|Replicated|GetCurrentWeapon))))
        (else
          (Utilities|Array|AddUnique _obtainedweaponnames (LocalVariables|Get%20GotWeaponName))
          (if (.UnlimitedAmmo (Utilities|Struct|BreakWeaponInfo (LocalVariables|GetWeaponDataTemp)))
            (Utilities|Array|Add _currentammo (.MaxAmmo (Utilities|Struct|BreakWeaponInfo (LocalVariables|GetWeaponDataTemp))))
            (else
              (Utilities|Array|Add _currentammo (.PickUpAmmo (Utilities|Struct|BreakWeaponInfo (LocalVariables|GetWeaponDataTemp)))))))))))
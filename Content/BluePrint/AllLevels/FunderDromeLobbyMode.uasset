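; Server-side game mode for the Funderdrome lobby, tracking players, car seat choices and map settings before a match.
; Joins, logouts, name changes and polling timers maintain LobbyList, which is pushed with server settings to lobby controllers.
; Game mode settings rebuild car placeholders by team, where PlayerSetup claims free driver or gunner seats.
; LaunchGame starts a short countdown, then runs servertravel with game mode, player and team limits in the URL.
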(event Custom|LaunchGame
  ;[1 1 1] Confirm & launch Game
  (bind _returnvalue (Utilities|Time|SetTimerbyEvent (delegate Custom|LobbyEnd) 3.0))
  (Variables|Default|SetLobbyEndTimer _returnvalue)
  (for _array_element (Variables|Default|GetPlayerList)
    (Default|LobbyEndTimer _array_element))
  (Variables|/Game/BluePrint/AllLevels/Ultradrome_GameInstance.Ultradrome_GameInstance_C|SetGameModeSetup (.AsUltradrome%20Game%20Instance (Utilities|Casting|CastToUltradrome_GameInstance (Game|GetGameInstance))) (Variables|Default|GetMapMode)))

(event Custom|UpdatePlayerName
  (params (NewName :type String) (ControllerRef :type Player%20Controller%20Object%20Reference))
  (bind _lobbylist (Variables|Default|GetLobbyList))
  (bind (_array_element _array_index) (Utilities|Array|ForEachLoopwithBreak _lobbylist :!label _label)
    (:LoopBody
      (if (== (.PlayerController (Utilities|Struct|BreakPlayerLobbyInfo _array_element)) ControllerRef)
        (bind _structout (Utilities|Struct|SetmembersinPlayerLobbyInfo _array_element (Utilities|Text|ToText(String) NewName)))
        (Utilities|Array|SetArrayElem _lobbylist _array_index _structout)
        (goto _label Break)))))

(event Custom|Update
  ;[1 1 1] Tick, Initialize, Check Player Number & start Lobby Mode (Most Importantly, ADD ALL PLAYER INTO PLACEHOLDERS!) (And yeah, Damn Networks.)
  (for _array_element (Variables|Default|GetLobbyList)
    (Default|UpdateServerSettings (.PlayerController (Utilities|Struct|BreakPlayerLobbyInfo _array_element)) (Variables|Default|GetMapName) (Variables|Default|GetMapMode)))
  (CallFunction|UpdateAllPlayers))

(event Custom|Initializ
  ;[1 1 1] Tick, Initialize, Check Player Number & start Lobby Mode (Most Importantly, ADD ALL PLAYER INTO PLACEHOLDERS!) (And yeah, Damn Networks.)
  (EventDispatchers|BindEventtoNameUpdate (delegate Custom|UpdatePlayerName))
  (|CallParentFunction)
  (Utilities|Time|SetTimerbyEvent (delegate Custom|Update) 1.0 true))

(event Custom|CheckPlayer
  (bind _lobbylist (Variables|Default|GetLobbyList))
  (bind _outactors (Actor|GetAllActorsOfClass "/Game/BluePrint/AllLevels/FunderdromeLobbyController.FunderdromeLobbyController_C"))
  (bind _array_element (Utilities|Array|ForEachLoopwithBreak _outactors)
    (:LoopBody
      (bind (_array_element_2 _array_index) (Utilities|Array|ForEachLoopwithBreak _lobbylist :!label _label)
        (:LoopBody
          (if (== (.PlayerController (Utilities|Struct|BreakPlayerLobbyInfo _array_element_2)) _array_element)
            (goto _label Break)
            (elif (== _array_index (Utilities|Array|LastIndex _lobbylist))
              (Utilities|Array|AddUnique _lobbylist (Utilities|Struct|MakePlayerLobbyInfo _array_element false false 0 0 (Utilities|Text|ToText(String) (Variables|/Game/BluePrint/AllLevels/Ultradrome_PlayerState.Ultradrome_PlayerState_C|GetDisplayName (.AsUltradrome%20Player%20State (Utilities|Casting|CastToUltradrome_PlayerState (Variables|/Script/Engine.Controller|GetPlayerState _array_element))))))))))))
    (:Completed
      (CallFunction|UpdateAllPlayers))))

(event Custom|AllPlayerUpdateServerSettings
  (params (MapName :type String) (GameMode :type Game%20Modes%20Structure))
  (bind _lobbylist (Variables|Default|GetLobbyList))
  (Variables|Default|SetMapName MapName)
  (CallFunction|ServerUpadeCarList GameMode)
  (Utilities|FlowControl|Delay 1.0)
  ;[1 1 1] Set All Players to Not Chooce
  (for (_array_element _array_index) _lobbylist
    (bind _structout (Utilities|Struct|SetmembersinPlayerLobbyInfo _array_element false))
    (Utilities|Array|SetArrayElem _lobbylist _array_index _structout))
  ;[1 1 1] Server Settings Update to everyone
  (for _array_element_2 (Variables|Default|GetPlayerList)
    (bind _asfunderdrome_lobby_controller (Utilities|Casting|CastToFunderdromeLobbyController _array_element_2))
    (Default|UpdateServerSettings _asfunderdrome_lobby_controller MapName GameMode)
    (Default|UpdatePlayers _asfunderdrome_lobby_controller (Variables|Default|GetLobbyList))))

(event Custom|LobbyEnd
  (bind _gamemapstring (Variables|Default|GetGameMapString))
  (bind _gamemodesting (Variables|Default|GetGameModeSting))
  (bind _serversettingmaxteam (Variables|ServerSettings|GetServerSettingMaxTeam))
  (bind _serversettingmaxplayer (Variables|ServerSettings|GetServerSettingMaxPlayer))
  (bind _returnvalue (Utilities|String|ToString(Integer) _serversettingmaxteam))
  (bind _returnvalue_2 (Utilities|String|ToString(Integer) _serversettingmaxplayer))
  (bind _returnvalue_3 (Utilities|String|Append "servertravel " _gamemapstring "?game=/Game/MyBluePrint/AllLevels/" _gamemodesting "?game_MaxPlayer=" _returnvalue_2 "?UMaxTeam=" _returnvalue))
  ;[1 1 1] Confirm & launch Game
  (for _array_element (Variables|Default|GetPlayerList)
    (Default|ShowLoadingScreen _array_element)
    (Variables|/Game/BluePrint/AllLevels/Ultradrome_PlayerController.Ultradrome_PlayerController_C|SetMapName _array_element (Variables|Default|GetMapName)))
  (Development|PrintString _returnvalue_3 true true "(R=0.000000,G=0.660000,B=1.000000,A=1.000000)" 2e+01)
  (Development|ExecuteConsoleCommand _returnvalue_3 (Game|GetPlayerController 0)))

(event Custom|UpdateAllPlayers
  ;[1 1 1] Update All Players Status
  (for _array_element (Variables|Default|GetPlayerList)
    (bind _asfunderdrome_lobby_controller (Utilities|Casting|CastToFunderdromeLobbyController _array_element))
    (Default|UpdatePlayers _asfunderdrome_lobby_controller (Variables|Default|GetLobbyList))))

(event EventBeginPlay
  (CallFunction|Initializ)
  (Utilities|Time|SetTimerbyEvent (delegate Custom|CheckPlayer) 3.0 true)
  (Development|PrintString "init" true true "(R=0.000000,G=0.660000,B=1.000000,A=1.000000)" 1e+01))

(event EventOnSwapPlayerControllers
  (params (OldPC :type Player%20Controller%20Object%20Reference) (NewPC :type Player%20Controller%20Object%20Reference))
  ;[1 1 1] Tick, Initialize, Check Player Number & start Lobby Mode (Most Importantly, ADD ALL PLAYER INTO PLACEHOLDERS!) (And yeah, Damn Networks.)
  (bind _asfunderdrome_lobby_controller (Utilities|Casting|CastToFunderdromeLobbyController NewPC))
  (Utilities|Array|AddUnique (Variables|Default|GetPlayerList) _asfunderdrome_lobby_controller)
  (Default|AquirePlayerName _asfunderdrome_lobby_controller)
  (bind _asultradrome_player_state (Utilities|Casting|CastToUltradrome_PlayerState (Variables|/Script/Engine.Controller|GetPlayerState _asfunderdrome_lobby_controller)))
  (Utilities|Array|Add (Variables|Default|GetLobbyList) (Utilities|Struct|MakePlayerLobbyInfo _asfunderdrome_lobby_controller false false 0 0 (Utilities|Text|ToText(String) (Variables|/Game/BluePrint/AllLevels/Ultradrome_PlayerState.Ultradrome_PlayerState_C|GetDisplayName _asultradrome_player_state))))
  (Default|DeathRemoveUI _asfunderdrome_lobby_controller)
  (Default|ShowLobbyMenu _asfunderdrome_lobby_controller)
  (Default|UpdateServerSettings _asfunderdrome_lobby_controller (Variables|Default|GetMapName) (Variables|Default|GetMapMode))
  (CallFunction|UpdateAllPlayers))

(event EventPostLogin
  (params (NewPlayer :type Player%20Controller%20Object%20Reference))
  (bind _asfunderdrome_lobby_controller (Utilities|Casting|CastToFunderdromeLobbyController NewPlayer))
  ;[1 1 1] Tick, Initialize, Check Player Number & start Lobby Mode (Most Importantly, ADD ALL PLAYER INTO PLACEHOLDERS!) (And yeah, Damn Networks.)
  (|CallParentFunction NewPlayer)
  (bind _asultradrome_player_state (Utilities|Casting|CastToUltradrome_PlayerState (Variables|/Script/Engine.Controller|GetPlayerState NewPlayer)))
  (Default|AquireName _asultradrome_player_state)
  (Development|PrintString (Variables|/Game/BluePrint/AllLevels/Ultradrome_PlayerState.Ultradrome_PlayerState_C|GetDisplayName _asultradrome_player_state) true true "(R=1.000000,G=0.060358,B=0.000000,A=1.000000)")
  (Utilities|Array|Add (Variables|Default|GetLobbyList) (Utilities|Struct|MakePlayerLobbyInfo _asfunderdrome_lobby_controller false false 0 0 (Utilities|Text|ToText(String) (Variables|/Game/BluePrint/AllLevels/Ultradrome_PlayerState.Ultradrome_PlayerState_C|GetDisplayName _asultradrome_player_state))))
  (Default|ShowLobbyMenu _asfunderdrome_lobby_controller)
  (Default|UpdateServerSettings _asfunderdrome_lobby_controller (Variables|Default|GetMapName) (Variables|Default|GetMapMode))
  (CallFunction|UpdateAllPlayers))

(event EventTick
  (params (DeltaSeconds :type Float%20%28single-precision%29)))

(event EventOnLogout
  (params (ExitingController :type Controller%20Object%20Reference))
  (bind _lobbylist (Variables|Default|GetLobbyList))
  ;[1 1 1] Player Left
  (|CallParentFunction ExitingController)
  (bind _array_element (Utilities|Array|ForEachLoopwithBreak _lobbylist :!label _label)
    (:LoopBody
      (if (== (.PlayerController (Utilities|Struct|BreakPlayerLobbyInfo _array_element)) ExitingController)
        (Utilities|Array|RemoveItem _lobbylist _array_element)
        (goto _label Break)))
    (:Completed
      (CallFunction|UpdateAllPlayers))))

(fn ConstructionScript
  (|CallParentFunction)
  (Utilities|Array|Clear (Variables|Default|GetLobbyList)))

(fn PlayerSetup
  (params (PlayerController :type Funderdrome%20Lobby%20Controller%20Object%20Reference) (CarNumber :type Integer) (Team :type Integer) (Driver :type Boolean))
  (bind _returnvalue (- CarNumber 1))
  (bind _lobbycarlist (Variables|Default|GetLobbyCarList))
  (bind _lobbycarlist_2 (Variables|Default|GetLobbyCarList))
  (bind _serversettingmaxteam (Variables|ServerSettings|GetServerSettingMaxTeam))
  (bind _lobbylist (Variables|Default|GetLobbyList))
  (bind _returnvalue_2 (* _returnvalue _serversettingmaxteam))
  (bind _returnvalue_3 (+ Team _returnvalue_2))
  (bind _returnvalue_4 (- _returnvalue_3 1))
  (bind _output (Utilities|Array|Get(acopy) _lobbycarlist _returnvalue_4))
  (bind (_driver _team _carnumber _cooldowntimer _gunner) (Utilities|Struct|BreakCarPlaceholder _output))
  ;[1 1 1] Check If The Desired Pos Is taken, Then Possess it.
  (if Driver
    (Utilities|IsValid _driver
      (:Is%20Not%20Valid
        (bind _structout (Utilities|Struct|SetmembersinCarPlaceholder _output PlayerController))
        (Utilities|Array|SetArrayElem _lobbycarlist _returnvalue_4 _structout)))
    (else
      (Utilities|IsValid _gunner
        (:Is%20Not%20Valid
          (bind _structout_2 (Utilities|Struct|SetmembersinCarPlaceholder _output PlayerController))
          (Utilities|Array|SetArrayElem _lobbycarlist _returnvalue_4 _structout_2)))))
  ;[1 1 1] Find Controller's Old Pos, Unpossess It.
  (bind (_array_element _array_index) (Utilities|Array|ForEachLoopwithBreak _lobbycarlist_2 :!label _label)
    (:LoopBody
      (if (== (.Driver (Utilities|Struct|BreakCarPlaceholder _array_element)) PlayerController)
        (bind _structout_3 (Utilities|Struct|SetmembersinCarPlaceholder _array_element))
        (Utilities|Array|SetArrayElem _lobbycarlist_2 _array_index _structout_3)
        (goto _label Break)
        (elif (== (.Gunner (Utilities|Struct|BreakCarPlaceholder _array_element)) PlayerController)
          (bind _structout_4 (Utilities|Struct|SetmembersinCarPlaceholder _array_element))
          (Utilities|Array|SetArrayElem _lobbycarlist_2 _array_index _structout_4)
          (goto _label Break))))
    (:Completed
      ;[1 1 1] Update It's New Pos to Lobby List, Then Boardcast It.
      (bind (_array_element_2 _array_index_2) (Utilities|Array|ForEachLoopwithBreak _lobbylist)
        (:LoopBody
          (if (== (.PlayerController (Utilities|Struct|BreakPlayerLobbyInfo _array_element_2)) PlayerController)
            (bind _structout_5 (Utilities|Struct|SetmembersinPlayerLobbyInfo _array_element_2 true Driver CarNumber Team))
            (Utilities|Array|SetArrayElem _lobbylist _array_index_2 _structout_5)))
        (:Completed
          (CallFunction|UpdateAllPlayers))))))

(fn ServerUpadeCarList
  (params (GameMode :type Game%20Modes%20Structure))
  (bind (_gamemodedisplayname _hasteam_ _maxplayers _maxteam) (Utilities|Struct|BreakGameModes GameMode))
  (Utilities|Array|Clear (Variables|Default|GetLobbyCarList))
  (Variables|ServerSettings|SetServerSettingMaxPlayer _maxplayers)
  (bind _output_get (LocalVariables|SetTempPlayer _maxplayers))
  (bind _output_get_2 (Variables|ServerSettings|SetServerSettingMaxTeam _maxteam))
  (if _hasteam_
    (Variables|ServerSettings|SetServerSettingMaxCarPerTeam (/ (/ _output_get 2) _output_get_2))
    (for _index (range 0 (- (/ _output_get 2) 1))
      (Utilities|Array|Add (Variables|Default|GetLobbyCarList) (Utilities|Struct|MakeCarPlaceholder 0 (+ (Math|Integer|%(Integer) _index (Variables|ServerSettings|GetServerSettingMaxTeam)) 1) (+ (/ _index (Variables|ServerSettings|GetServerSettingMaxTeam)) 1))))
    (else
      (Variables|ServerSettings|SetServerSettingMaxCarPerTeam (LocalVariables|GetNoTeamCarNumber))
      (for _index_2 (range 0 (- (/ _output_get 2) 1))
        (Utilities|Array|Add (Variables|Default|GetLobbyCarList) (Utilities|Struct|MakeCarPlaceholder 0 (+ _index_2 1) (LocalVariables|GetNoTeamCarNumber)))))))
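; Battle royale game mode for Funderdrome car combat, with AI enabled and every car on its own team.
; On BeginPlay it spawns an 8x8 grid of randomly outfitted cars and nav nodes, offset from the first PlayerStart.
; After a short timer it opens parachutes, readies cars and turrets, assigns controllers, starts AI and clears player death UI.
; Kill events pass through CarKillHandle and record victims in a dead list.
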(event Custom|gameStart
  (for (_array_element _array_index) (Variables|Default|GetCars)
    (Variables|/Game/TestCar/BP/FunderDromeCarBase.FunderDromeCarBase_C|SetVehicleID (.AsFunder%20Drome%20Car%20Base (Utilities|Casting|CastToFunderDromeCarBase (.Car (Utilities|Struct|BreakCarPlaceholder _array_element)))) (.CarNumber (Utilities|Struct|BreakCarPlaceholder _array_element)))
    (Default|OpenPara (.AsFunder%20Drome%20Car%20Base (Utilities|Casting|CastToFunderDromeCarBase (.Car (Utilities|Struct|BreakCarPlaceholder _array_element)))))
    (Default|CarSetup (.AsFunder%20Drome%20Car%20Base (Utilities|Casting|CastToFunderDromeCarBase (.Car (Utilities|Struct|BreakCarPlaceholder _array_element)))))
    (Default|WeaponReadyNormal (.AsFunder%20Drome%20Turret%20Base (Utilities|Casting|CastToFunderDromeTurretBase (.Turret (Utilities|Struct|BreakCarPlaceholder _array_element)))))
    (CallFunction|ControllerPosses _array_index))
  (bind _outactors (Actor|GetAllActorsOfClass "/Game/BluePrint/AIScript/FunderDromeAIController.FunderDromeAIController_C"))
  (for _array_element_2 _outactors
    (Variables|/Game/BluePrint/AIScript/FunderDromeAIController.FunderDromeAIController_C|SetAIStart _array_element_2 true))
  (bind _outactors_2 (Actor|GetAllActorsOfClass "/Game/BluePrint/AllLevels/Ultradrome_PlayerController.Ultradrome_PlayerController_C"))
  (for _array_element_3 _outactors_2
    (Default|DeathRemoveUI _array_element_3)))

(event EventBeginPlay
  (Variables|Default|SetHasAI true)
  (Variables|Default|SetFriendlyFire false)
  (CallFunction|MMOpLAYERsPAWN)
  (Utilities|Time|SetTimerbyEvent (delegate Custom|gameStart) 5.0))

(event EventTick
  (params (DeltaSeconds :type Float%20%28single-precision%29))
  (|CallParentFunction DeltaSeconds) ; This node is disabled and will not be called.\nDrag off pins to build functionality.
)

(event EventCarKillEvent
  (params (VictimID :type Integer) (Weapon :type Duke_WeaponType%20Enum :default "NewEnumerator0") (PlayerKill :type Boolean) (KillerID :type Integer))
  (bind _deadlist (Variables|Default|GetDeadList))
  (if (not (Utilities|Array|ContainsItem _deadlist VictimID))
    (bind _killedcarid (CallFunction|CarKillHandle VictimID Weapon PlayerKill KillerID))
    (Utilities|Array|AddUnique _deadlist _killedcarid)))

(fn ConstructionScript
  (|CallParentFunction))

(fn MMOpLAYERsPAWN
  (bind _returnvalue (Math|Random|RandomIntegerinRange 0 1))
  (bind _returnvalue_2 (Math|Conversions|ToByte(Integer) _returnvalue))
  (Utilities|Array|Clear (Variables|Default|GetCars))
  (Utilities|Array|Clear (Variables|Default|GetSpawnList))
  (bind _outactors (Actor|GetAllActorsOfClass "/Script/Engine.PlayerStart"))
  (Variables|Default|SetSpawnList (Utilities|Array|MakeArray (Transformation|GetActorLocation (Utilities|Array|Get(acopy) _outactors))))
  (for _index (range 0 7)
    (for _index_2 (range 0 7)
      (if (or (!= _index_2 0) (!= _index 0))
        (Utilities|Array|SetArrayElem (Variables|Default|GetSpawnList) (+ (* 8 _index) _index_2) (+ (Utilities|Array|Get(acopy) (Variables|Default|GetSpawnList)) (Math|Vector|MakeVector (* 5e+03 (Math|Conversions|ToFloat(Integer) _index_2)) (* 5e+03 (Math|Conversions|ToFloat(Integer) _index)) 0.0)) true))
      (Game|SpawnActorfromClass "/Game/BluePrint/Property/NavPointNode.NavPointNode_C" (Math|Transform|MakeTransform (+ (Utilities|Array|Get(acopy) (Variables|Default|GetSpawnList)) (Math|Vector|MakeVector (* 5e+03 (Math|Conversions|ToFloat(Integer) _index_2)) (* 5e+03 (Math|Conversions|ToFloat(Integer) _index)) 0.0))) "Undefined" 0 (+ (* 8 _index) _index_2) (+ (* 8 _index) _index_2) 0)
      (bind (_newcar _newturret) (CallFunction|RespawnCar (Math|Transform|MakeTransform (+ (Utilities|Array|Get(acopy) (Variables|Default|GetSpawnList)) (Math|Vector|MakeVector (* 5e+03 (Math|Conversions|ToFloat(Integer) _index_2)) (* 5e+03 (Math|Conversions|ToFloat(Integer) _index)) 0.0))) true (Utilities|Enum|ByteToEnumCarSetups _returnvalue_2) (Utilities|Enum|ByteToEnumDuke_WeaponType _returnvalue_2) (+ (* 8 _index) _index_2)))
      (Utilities|Array|SetArrayElem (Variables|Default|GetCars) (+ (* 8 _index) _index_2) (Utilities|Struct|MakeCarPlaceholder 0 (+ (* 8 _index) _index_2) (+ (* 8 _index) _index_2) 1.0 0 (.AsFunder%20Drome%20Car%20Base (Utilities|Casting|CastToFunderDromeCarBase _newcar)) (.AsFunder%20Drome%20Turret%20Base (Utilities|Casting|CastToFunderDromeTurretBase _newturret)) 0 0 true) true))))
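; Payload game mode for two-team FunderDrome car combat, spawning an AI-possessed payload at the start of a spline and randomly outfitted car/turret pairs at player starts.
; A countdown readies cars, then starts AI and payload.
; Kills are broadcast and queue victims for looping-timer respawn waves, which first move spawn points behind the payload along the spline, with team two parachuting from higher up.
; Airdrop pickup spawning exists, but its timer is unwired.
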(event Custom|EventCarKill
  (params (VictimID :type Integer) (Weapon :type Duke_WeaponType%20Enum) (PlayerKill :type Boolean) (KillerID :type Integer))
  (if (not (Utilities|Array|ContainsItem (Variables|Default|GetNextWaveIndex) VictimID))
    (bind (_killedcarid _killbroadcast) (CallFunction|CarKillHandle VictimID Weapon PlayerKill KillerID))
    (Utilities|Array|Add (Variables|Default|GetNextWaveIndex) _killedcarid)
    (Utilities|FlowControl|Sequence
      (:then_0
        (if (.PlayerKill (Utilities|Struct|BreakKillFeed _killbroadcast))
          (Development|PrintString (Utilities|String|Append (.VictimDriver (Utilities|Struct|BreakKillFeed _killbroadcast)) (.VictimGunner (Utilities|Struct|BreakKillFeed _killbroadcast)) (Utilities|String|EnumtoString (.WeaponType (Utilities|Struct|BreakKillFeed _killbroadcast))) (.KillerDriver (Utilities|Struct|BreakKillFeed _killbroadcast)) (.KillerGunner (Utilities|Struct|BreakKillFeed _killbroadcast))))
          (else
            (Development|PrintString (Utilities|String|Append (.VictimDriver (Utilities|Struct|BreakKillFeed _killbroadcast)) (.VictimGunner (Utilities|Struct|BreakKillFeed _killbroadcast)) (Utilities|String|ToString(Integer) (.VictimDeathCount (Utilities|Struct|BreakKillFeed _killbroadcast))) (Utilities|String|ToString(Integer) (.VictimTeam (Utilities|Struct|BreakKillFeed _killbroadcast)))))))
        (for _array_element (Variables|Default|GetPlayerList)
          (Default|BroadcastKill _array_element _killbroadcast)))
      (:then_1
        (Utilities|FlowControl|DoOnce false
          (:Completed
            (Utilities|FlowControl|Delay 15.0)
            (Utilities|Time|SetTimerbyEvent (delegate Custom|ReadyNextSpawn) 15.0 true)))))))

(event Custom|GameSet
  ;[1 1 1] CountDownStart
  (CallFunction|GameStartCountDown)
  (Utilities|FlowControl|Delay 2.0)
  (for _array_element (Variables|Default|GetCars)
    (bind _asfunder_drome_car_base (Utilities|Casting|CastToFunderDromeCarBase (.Car (Utilities|Struct|BreakCarPlaceholder _array_element))))
    (Default|CarSetup _asfunder_drome_car_base)
    (bind _asfunder_drome_turret_base (Utilities|Casting|CastToFunderDromeTurretBase (.Turret (Utilities|Struct|BreakCarPlaceholder _array_element))))
    (Default|WeaponReadyNormal _asfunder_drome_turret_base))
  (Utilities|FlowControl|Delay 5.0)
  (bind _outactors (Actor|GetAllActorsOfClass "/Game/BluePrint/AIScript/FunderDromeAIController.FunderDromeAIController_C"))
  (for _array_element_2 _outactors
    (Variables|/Game/BluePrint/AIScript/FunderDromeAIController.FunderDromeAIController_C|SetAIStart _array_element_2 true)
    (Default|PayloadInitiation (Variables|Default|GetPayload))))

(event Custom|PayloadUpdateHealth
  (params (NewHealth :type Float%20%28single-precision%29))
  (Development|PrintString (Utilities|String|ToString(Float) NewHealth)))

(event Custom|ReadyNextSpawn
  (bind _nextwaveindex (Variables|Default|GetNextWaveIndex))
  (Variables|Default|SetNextWaveTag _nextwaveindex)
  (Utilities|Array|Clear _nextwaveindex)
  (CallFunction|ReadyNextSpawnPoint)
  (CallFunction|WaveSpawn)
  (for _array_element (Variables|Default|GetNextWaveTag)
    (CallFunction|ControllerPosses _array_element))
  (Utilities|FlowControl|Delay 5.0)
  (bind _outactors (Actor|GetAllActorsOfClass "/Game/BluePrint/AIScript/FunderDromeAIController.FunderDromeAIController_C"))
  (for _array_element_2 _outactors
    (Variables|/Game/BluePrint/AIScript/FunderDromeAIController.FunderDromeAIController_C|SetAIStart _array_element_2 true)))

(event Custom|SpawnPickup
  ;[1 1 1] CountDownStart
  (CallFunction|SpawnPickUps (Transformation|GetActorLocation (Variables|Default|GetPayload))))

(event EventBeginPlay
  ;[1 1 1] NO Idea
  (Variables|Default|SetGameMode 1)
  (Variables|Default|SetMaxPlayer 16)
  (Variables|Default|SetMaxTeam 2)
  (Variables|Default|SetHasAI true)
  (|CallParentFunction)
  (EventDispatchers|BindEventtoCarKill (delegate Custom|EventCarKill))
  (bind _outactors (Actor|GetAllActorsOfClass "/Game/BluePrint/Property/PayloadMoveNode.PayloadMoveNode_C"))
  (bind _output_get (Variables|Default|SetWayPoints (Utilities|Array|Get(acopy) _outactors)))
  (bind _returnvalue (Game|SpawnActorfromClass "/Game/TestCar/BP/TestPayloadBP.TestPayloadBP_C" (Math|Transform|MakeTransform (+ (.location (Spline|GetTransformatSplinePoint (Variables|/Game/BluePrint/Property/PayloadMoveNode.PayloadMoveNode_C|GetSpline _output_get) 0 "World" false)) "0, 0,900.000000") (Math|Rotator|MakeRotator 0.0 0.0 (.Yaw (Math|Rotator|BreakRotator (.rotation (Spline|GetTransformatSplinePoint (Variables|/Game/BluePrint/Property/PayloadMoveNode.PayloadMoveNode_C|GetSpline _output_get) 0 "World" false)))))) "AlwaysSpawn" 0 0))
  (bind _output_get_2 (Variables|Default|SetPayload _returnvalue))
  (bind _returnvalue_2 (Game|SpawnActorfromClass "/Game/BluePrint/AIScript/FunderDromeAIController.FunderDromeAIController_C" (Math|Transform|MakeTransform (+ (.location (Spline|GetTransformatSplinePoint (Variables|/Game/BluePrint/Property/PayloadMoveNode.PayloadMoveNode_C|GetSpline _output_get) 0 "World" false)) "0, 0,900.000000") (Math|Rotator|MakeRotator 0.0 0.0 (.Yaw (Math|Rotator|BreakRotator (.rotation (Spline|GetTransformatSplinePoint (Variables|/Game/BluePrint/Property/PayloadMoveNode.PayloadMoveNode_C|GetSpline _output_get) 0 "World" false)))))) "AlwaysSpawn" 0 0))
  (Pawn|Possess _returnvalue_2 _output_get_2)
  (bind _outactors_2 (Actor|GetAllActorsOfClass "/Game/Cinematics/AC130Actor.AC130Actor_C"))
  (Variables|Default|SetAC130 (Utilities|Array|Get(acopy) _outactors_2))
  (bind _finished (CallFunction|GameInitSpawn))
  (if _finished
    (for (_array_element _array_index) (Variables|Default|GetCars)
      (bind _asfunder_drome_car_base (Utilities|Casting|CastToFunderDromeCarBase (.Car (Utilities|Struct|BreakCarPlaceholder _array_element))))
      (Default|OpenPara _asfunder_drome_car_base)
      (CallFunction|ControllerPosses _array_index))
    (for _array_element_2 (Variables|Default|GetPlayerList)
      (Default|DeathRemoveUI _array_element_2))
    (CallFunction|GameSet)))

(event EventTick
  (params (DeltaSeconds :type Float%20%28single-precision%29))
  (|CallParentFunction DeltaSeconds))

(fn ConstructionScript
  (|CallParentFunction))

(fn SpawnPickUps
  (params (PayloadLoc :type Vector))
  (bind _pickupdestroytimer (Variables|Default|GetPickUpDestroyTimer))
  (LocalVariables|SetSpawnTrans (Math|Transform|MakeTransform (+ PayloadLoc (Math|Vector|RotateVector "2000.000000, 0, 0" (Math|Rotator|MakeRotator 0.0 0.0 (Math|Random|RandomFloatinRange -1.8e+02 1.8e+02))) "0,0,2000.000000")))
  (Utilities|FlowControl|MultiGate true true -1
    (:Out%200
      (Game|SpawnActorfromClass "/Game/BluePrint/Property/AirDropPickup.AirDropPickup_C" (LocalVariables|GetSpawnTrans) "Undefined" 0 true "NewEnumerator0" _pickupdestroytimer))
    (:Out%201
      (Game|SpawnActorfromClass "/Game/BluePrint/Property/AirDropPickup.AirDropPickup_C" (LocalVariables|GetSpawnTrans) "Undefined" 0 false "NewEnumerator1" _pickupdestroytimer))
    (:Out%202
      (Game|SpawnActorfromClass "/Game/BluePrint/Property/AirDropPickup.AirDropPickup_C" (LocalVariables|GetSpawnTrans) "Undefined" 0 false "NewEnumerator1" _pickupdestroytimer))
    (:Out%203
      (Game|SpawnActorfromClass "/Game/BluePrint/Property/AirDropPickup.AirDropPickup_C" (LocalVariables|GetSpawnTrans) "Undefined" 0 false "NewEnumerator2" _pickupdestroytimer))
    (:Out%204
      (Game|SpawnActorfromClass "/Game/BluePrint/Property/AirDropPickup.AirDropPickup_C" (LocalVariables|GetSpawnTrans) "Undefined" 0 false "NewEnumerator2" _pickupdestroytimer))
    (:Out%205
      (Game|SpawnActorfromClass "/Game/BluePrint/Property/AirDropPickup.AirDropPickup_C" (LocalVariables|GetSpawnTrans) "Undefined" 0 false "NewEnumerator3" _pickupdestroytimer))
    (:Out%206
      (Game|SpawnActorfromClass "/Game/BluePrint/Property/AirDropPickup.AirDropPickup_C" (LocalVariables|GetSpawnTrans) "Undefined" 0 false "NewEnumerator3" _pickupdestroytimer))))

(fn GameStartAnim
  (bind _returnvalue (Sequencer|Player|CreateLevelSequencePlayer (Variables|Default|GetOpeningCinematic)))
  (Sequencer|Player|Play _returnvalue :!class /Script/MovieScene.MovieSceneSequencePlayer)
  (for _array_element (Variables|Default|GetPlayerList)
    (Default|DeathRemoveUI _array_element)))

(fn GameInitSpawn
  (bind _outactors (Actor|GetAllActorsOfClass "/Game/TestCar/BP/FunderDromePlayerStart.FunderDromePlayerStart_C"))
  (for _array_element _outactors
    (bind (_newcar _newturret) (CallFunction|RespawnCar (Transformation|GetActorTransform _array_element) true (Utilities|Enum|ByteToEnumCarSetups (Math|Conversions|ToByte(Integer) (Math|Random|RandomIntegerinRange 0 1))) (Utilities|Enum|ByteToEnumDuke_WeaponType (Math|Conversions|ToByte(Integer) (Math|Random|RandomIntegerinRange 0 3)))))
    (if (== (Variables|/Game/TestCar/BP/FunderDromePlayerStart.FunderDromePlayerStart_C|GetTeam _array_element) 1)
      (Utilities|Array|Add (Variables|Default|GetTeam1Spwan) _array_element)
      (bind _result (Math|Integer|IncrementInt (LocalVariables|GetTeamNum1))
        (:%20%20
          (Variables|/Game/TestCar/BP/FunderDromeCarBase.FunderDromeCarBase_C|SetDriverNameText (.AsFunder%20Drome%20Car%20Base (Utilities|Casting|CastToFunderDromeCarBase _newcar)) (Utilities|Text|ToText(String) (.DriverName (Utilities|Struct|BreakCarPlaceholder (.CarRef (CallFunction|GetCarIndex _result (Variables|/Game/TestCar/BP/FunderDromePlayerStart.FunderDromePlayerStart_C|GetTeam _array_element)))))))
          (Variables|/Game/TestCar/BP/FunderDromeCarBase.FunderDromeCarBase_C|SetGunnerNameText (.AsFunder%20Drome%20Car%20Base (Utilities|Casting|CastToFunderDromeCarBase _newcar)) (Utilities|Text|ToText(String) (.GunnerName (Utilities|Struct|BreakCarPlaceholder (.CarRef (CallFunction|GetCarIndex _result (Variables|/Game/TestCar/BP/FunderDromePlayerStart.FunderDromePlayerStart_C|GetTeam _array_element)))))))
          (bind _output_get (Variables|/Game/TestCar/BP/FunderDromeCarBase.FunderDromeCarBase_C|SetTeam (.AsFunder%20Drome%20Car%20Base (Utilities|Casting|CastToFunderDromeCarBase _newcar)) (.Team (Utilities|Struct|BreakCarPlaceholder (.CarRef (CallFunction|GetCarIndex _result (Variables|/Game/TestCar/BP/FunderDromePlayerStart.FunderDromePlayerStart_C|GetTeam _array_element)))))))
          (Variables|/Game/BluePrint/Turret/FunderDromeTurretBase.FunderDromeTurretBase_C|SetTeam (.AsFunder%20Drome%20Turret%20Base (Utilities|Casting|CastToFunderDromeTurretBase _newturret)) _output_get)
          (bind _output_get_2 (Variables|/Game/TestCar/BP/FunderDromeCarBase.FunderDromeCarBase_C|SetVehicleID (.AsFunder%20Drome%20Car%20Base (Utilities|Casting|CastToFunderDromeCarBase _newcar)) (.Index (CallFunction|GetCarIndex _result (Variables|/Game/TestCar/BP/FunderDromePlayerStart.FunderDromePlayerStart_C|GetTeam _array_element)))))
          (bind _output_get_3 (Variables|/Game/BluePrint/Turret/FunderDromeTurretBase.FunderDromeTurretBase_C|SetVehicleID (.AsFunder%20Drome%20Turret%20Base (Utilities|Casting|CastToFunderDromeTurretBase _newturret)) _output_get_2))
          (bind _structout (Utilities|Struct|SetmembersinCarPlaceholder (.CarRef (CallFunction|GetCarIndex _result (Variables|/Game/TestCar/BP/FunderDromePlayerStart.FunderDromePlayerStart_C|GetTeam _array_element))) (.AsFunder%20Drome%20Car%20Base (Utilities|Casting|CastToFunderDromeCarBase _newcar)) (.AsFunder%20Drome%20Turret%20Base (Utilities|Casting|CastToFunderDromeTurretBase _newturret))))
          (Utilities|Array|SetArrayElem (Variables|Default|GetCars) _output_get_3 _structout)))
      (else
        (Utilities|Array|Add (Variables|Default|GetTeam2Spwan) _array_element)
        (bind _result_2 (Math|Integer|IncrementInt (LocalVariables|GetTeamNum2))
          (:%20%20
            (Variables|/Game/TestCar/BP/FunderDromeCarBase.FunderDromeCarBase_C|SetDriverNameText (.AsFunder%20Drome%20Car%20Base (Utilities|Casting|CastToFunderDromeCarBase _newcar)) (Utilities|Text|ToText(String) (.DriverName (Utilities|Struct|BreakCarPlaceholder (.CarRef (CallFunction|GetCarIndex _result_2 (Variables|/Game/TestCar/BP/FunderDromePlayerStart.FunderDromePlayerStart_C|GetTeam _array_element)))))))
            (Variables|/Game/TestCar/BP/FunderDromeCarBase.FunderDromeCarBase_C|SetGunnerNameText (.AsFunder%20Drome%20Car%20Base (Utilities|Casting|CastToFunderDromeCarBase _newcar)) (Utilities|Text|ToText(String) (.GunnerName (Utilities|Struct|BreakCarPlaceholder (.CarRef (CallFunction|GetCarIndex _result_2 (Variables|/Game/TestCar/BP/FunderDromePlayerStart.FunderDromePlayerStart_C|GetTeam _array_element)))))))
            (bind _output_get_4 (Variables|/Game/TestCar/BP/FunderDromeCarBase.FunderDromeCarBase_C|SetTeam (.AsFunder%20Drome%20Car%20Base (Utilities|Casting|CastToFunderDromeCarBase _newcar)) (.Team (Utilities|Struct|BreakCarPlaceholder (.CarRef (CallFunction|GetCarIndex _result_2 (Variables|/Game/TestCar/BP/FunderDromePlayerStart.FunderDromePlayerStart_C|GetTeam _array_element)))))))
            (Variables|/Game/BluePrint/Turret/FunderDromeTurretBase.FunderDromeTurretBase_C|SetTeam (.AsFunder%20Drome%20Turret%20Base (Utilities|Casting|CastToFunderDromeTurretBase _newturret)) _output_get_4)
            (bind _output_get_5 (Variables|/Game/TestCar/BP/FunderDromeCarBase.FunderDromeCarBase_C|SetVehicleID (.AsFunder%20Drome%20Car%20Base (Utilities|Casting|CastToFunderDromeCarBase _newcar)) (.Index (CallFunction|GetCarIndex _result_2 (Variables|/Game/TestCar/BP/FunderDromePlayerStart.FunderDromePlayerStart_C|GetTeam _array_element)))))
            (bind _output_get_6 (Variables|/Game/BluePrint/Turret/FunderDromeTurretBase.FunderDromeTurretBase_C|SetVehicleID (.AsFunder%20Drome%20Turret%20Base (Utilities|Casting|CastToFunderDromeTurretBase _newturret)) _output_get_5))
            (bind _structout_2 (Utilities|Struct|SetmembersinCarPlaceholder (.CarRef (CallFunction|GetCarIndex _result_2 (Variables|/Game/TestCar/BP/FunderDromePlayerStart.FunderDromePlayerStart_C|GetTeam _array_element))) (.AsFunder%20Drome%20Car%20Base (Utilities|Casting|CastToFunderDromeCarBase _newcar)) (.AsFunder%20Drome%20Turret%20Base (Utilities|Casting|CastToFunderDromeTurretBase _newturret))))
            (Utilities|Array|SetArrayElem (Variables|Default|GetCars) _output_get_6 _structout_2))))))
  (return (LocalVariables|GetForceTrue)))

(fn GameStartCountDown
  (Audio|SpawnSound2D "/Game/Audio/BGM/Warlords_Cue.Warlords_Cue")
  (for _array_element (Variables|Default|GetPlayerList)
    (Default|GameReadyCountDown _array_element)))

(fn ReadyNextSpawnPoint
  (bind _payload (Variables|Default|GetPayload))
  (bind _waypoints (Variables|Default|GetWayPoints))
  (bind _returnvalue (Transformation|GetActorLocation _payload))
  (bind _spline (Variables|/Game/BluePrint/Property/PayloadMoveNode.PayloadMoveNode_C|GetSpline _waypoints))
  (bind _returnvalue_2 (Class|SplineComponent|FindTransformClosesttoWorldLocation _spline _returnvalue "World" false))
  (bind (_location _rotation) (Math|Transform|BreakTransform _returnvalue_2))
  (bind _output_get (LocalVariables|SetSpawnRot (Math|Rotator|MakeRotator 0.0 0.0 (.Yaw (Math|Rotator|BreakRotator _rotation)))))
  (LocalVariables|SetCenter (+ _location "0,0.000000,200.000000" (* (Math|Vector|GetForwardVector _output_get) -2e+03)))
  (for (_array_element _array_index) (Variables|Default|GetTeam1Spwan)
    (Transformation|SetActorLocationAndRotation _array_element (+ (LocalVariables|GetCenter) (* (Math|Vector|GetRightVector (LocalVariables|GetSpawnRot)) (+ 8e+02 (* (- _array_index 2) -8e+02)))) (LocalVariables|GetSpawnRot)))
  (for (_array_element_2 _array_index_2) (Variables|Default|GetTeam2Spwan)
    (Transformation|SetActorLocationAndRotation _array_element_2 (+ (LocalVariables|GetCenter) (* (Math|Vector|GetRightVector (LocalVariables|GetSpawnRot)) (+ 8e+02 (* (- _array_index_2 2) -8e+02))) (* (Math|Vector|GetForwardVector (LocalVariables|GetSpawnRot)) -3e+03) "0,0,2800.000000") (LocalVariables|GetSpawnRot))))

(fn WaveSpawn
  (bind _returnvalue (Math|Random|RandomIntegerinRange 0 1))
  (bind _returnvalue_2 (Math|Random|RandomIntegerinRange 0 3))
  (bind _returnvalue_3 (Math|Conversions|ToByte(Integer) _returnvalue))
  (bind _returnvalue_4 (Math|Conversions|ToByte(Integer) _returnvalue_2))
  (bind _returnvalue_5 (Utilities|Enum|ByteToEnumDuke_WeaponType _returnvalue_4))
  (bind _returnvalue_6 (Utilities|Enum|ByteToEnumCarSetups _returnvalue_3))
  (for _array_element (Variables|Default|GetNextWaveTag)
    (if (== (.Team (Utilities|Struct|BreakCarPlaceholder (Utilities|Array|Get(acopy) (Variables|Default|GetCars) _array_element))) 1)
      (bind (_newcar _newturret) (CallFunction|RespawnCar (Transformation|GetActorTransform (Utilities|Array|Get(acopy) (Variables|Default|GetTeam1Spwan) (LocalVariables|GetTeamNum1))) true _returnvalue_6 _returnvalue_5))
      (Math|Integer|IncrementInt (LocalVariables|GetTeamNum1)
        (:%20%20
          (LocalVariables|SetCar (.AsFunder%20Drome%20Car%20Base (Utilities|Casting|CastToFunderDromeCarBase _newcar)))
          (LocalVariables|SetTurret (.AsFunder%20Drome%20Turret%20Base (Utilities|Casting|CastToFunderDromeTurretBase _newturret)))
          (Variables|/Game/TestCar/BP/FunderDromeCarBase.FunderDromeCarBase_C|SetDriverNameText (LocalVariables|GetCar) (Utilities|Text|ToText(String) (.DriverName (Utilities|Struct|BreakCarPlaceholder (Utilities|Array|Get(acopy) (Variables|Default|GetCars) _array_element)))))
          (Variables|/Game/TestCar/BP/FunderDromeCarBase.FunderDromeCarBase_C|SetGunnerNameText (LocalVariables|GetCar) (Utilities|Text|ToText(String) (.GunnerName (Utilities|Struct|BreakCarPlaceholder (Utilities|Array|Get(acopy) (Variables|Default|GetCars) _array_element)))))
          (bind _output_get (Variables|/Game/TestCar/BP/FunderDromeCarBase.FunderDromeCarBase_C|SetTeam (LocalVariables|GetCar) (.Team (Utilities|Struct|BreakCarPlaceholder (Utilities|Array|Get(acopy) (Variables|Default|GetCars) _array_element)))))
          (Variables|/Game/BluePrint/Turret/FunderDromeTurretBase.FunderDromeTurretBase_C|SetTeam (LocalVariables|GetTurret) _output_get)
          (bind _output_get_2 (Variables|/Game/TestCar/BP/FunderDromeCarBase.FunderDromeCarBase_C|SetVehicleID (LocalVariables|GetCar) _array_element))
          (bind _output_get_3 (Variables|/Game/BluePrint/Turret/FunderDromeTurretBase.FunderDromeTurretBase_C|SetVehicleID (LocalVariables|GetTurret) _output_get_2))
          (bind _structout (Utilities|Struct|SetmembersinCarPlaceholder (Utilities|Array|Get(acopy) (Variables|Default|GetCars) _array_element) (LocalVariables|GetCar) (LocalVariables|GetTurret)))
          (Utilities|Array|SetArrayElem (Variables|Default|GetCars) _output_get_3 _structout)
          (Default|CarSetup (LocalVariables|GetCar))
          (Default|DriveStart (LocalVariables|GetCar))
          (Default|WeaponReadyNormal (LocalVariables|GetTurret))))
      (else
        (bind (_newcar_2 _newturret_2) (CallFunction|RespawnCar (Transformation|GetActorTransform (Utilities|Array|Get(acopy) (Variables|Default|GetTeam2Spwan) (LocalVariables|GetTeamNum2))) true _returnvalue_6 _returnvalue_5))
        (Math|Integer|IncrementInt (LocalVariables|GetTeamNum2)
          (:%20%20
            (LocalVariables|SetCar (.AsFunder%20Drome%20Car%20Base (Utilities|Casting|CastToFunderDromeCarBase _newcar_2)))
            (LocalVariables|SetTurret (.AsFunder%20Drome%20Turret%20Base (Utilities|Casting|CastToFunderDromeTurretBase _newturret_2)))
            (Variables|/Game/TestCar/BP/FunderDromeCarBase.FunderDromeCarBase_C|SetDriverNameText (LocalVariables|GetCar) (Utilities|Text|ToText(String) (.DriverName (Utilities|Struct|BreakCarPlaceholder (Utilities|Array|Get(acopy) (Variables|Default|GetCars) _array_element)))))
            (Variables|/Game/TestCar/BP/FunderDromeCarBase.FunderDromeCarBase_C|SetGunnerNameText (LocalVariables|GetCar) (Utilities|Text|ToText(String) (.GunnerName (Utilities|Struct|BreakCarPlaceholder (Utilities|Array|Get(acopy) (Variables|Default|GetCars) _array_element)))))
            (bind _output_get_4 (Variables|/Game/TestCar/BP/FunderDromeCarBase.FunderDromeCarBase_C|SetTeam (LocalVariables|GetCar) (.Team (Utilities|Struct|BreakCarPlaceholder (Utilities|Array|Get(acopy) (Variables|Default|GetCars) _array_element)))))
            (Variables|/Game/BluePrint/Turret/FunderDromeTurretBase.FunderDromeTurretBase_C|SetTeam (LocalVariables|GetTurret) _output_get_4)
            (bind _output_get_5 (Variables|/Game/TestCar/BP/FunderDromeCarBase.FunderDromeCarBase_C|SetVehicleID (LocalVariables|GetCar) _array_element))
            (bind _output_get_6 (Variables|/Game/BluePrint/Turret/FunderDromeTurretBase.FunderDromeTurretBase_C|SetVehicleID (LocalVariables|GetTurret) _output_get_5))
            (bind _structout_2 (Utilities|Struct|SetmembersinCarPlaceholder (Utilities|Array|Get(acopy) (Variables|Default|GetCars) _array_element) (LocalVariables|GetCar) (LocalVariables|GetTurret)))
            (Utilities|Array|SetArrayElem (Variables|Default|GetCars) _output_get_6 _structout_2)
            (Default|CarSetup (LocalVariables|GetCar))
            (Default|OpenPara (LocalVariables|GetCar))
            (Default|WeaponReadyNormal (LocalVariables|GetTurret))))))))
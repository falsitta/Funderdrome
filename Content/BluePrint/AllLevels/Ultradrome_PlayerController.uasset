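; Player controller for Ultradrome's team car combat, where each player is either a driver or a gunner.
; It stores role, team and car in PlayerGameState, creates the matching HUD and forwards health, ammo, killfeed, scoreboard and round results to it.
; It also drives gamepad rumble through per-weapon pulses, directional hit feedback and four continuous motor channels fed by car velocity and acceleration.
; A debug key possesses a spectator pawn or its selected pawn.
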(event Custom|BroadcastKill
  (params (killFeed :type Kill%20Feed%20Structure))
  (bind _playergamestate (Variables|Default|GetPlayerGameState))
  (bind (_isdriver _team) (Utilities|Struct|BreakPlayerGameState _playergamestate))
  ;[1 1 1] UI Update
  (if _isdriver
    (Default|AddKillfeed (Variables|Default|GetDriverUI) killFeed)
    (else
      (Default|AddKillfeed (Variables|Default|GetGunnerUI) killFeed _team))))

(event Custom|UpdatePayloadDist
  (params (Dist :type Float%20%28single-precision%29))
  (if (.isdriver (Variables|Default|GetPlayerGameState))
    _))

(event Custom|GameOver
  (Game|OpenLevel(byName) "MainMenu"))

(event Custom|StartRumble
  (Utilities|FlowControl|Sequence
    (:then_0
      (Game|Feedback|PlayDynamicForceFeedback (Variables|Default|GetRumbleStrengthLS) -1.0 false true false false))
    (:then_1
      (Game|Feedback|PlayDynamicForceFeedback (Variables|Default|GetRumbleStrengthLL) -1.0 true false false false))
    (:then_2
      (Game|Feedback|PlayDynamicForceFeedback (Variables|Default|GetRumbleStrengthRS) -1.0 false false false true))
    (:then_3
      (Game|Feedback|PlayDynamicForceFeedback (Variables|Default|GetRumbleStrengthRL) -1.0 false false true false))))

(event Custom|Weapon%20Update
  (params (OnlyAmmo :type Boolean) (Weapon :type Name) (NewAmmo :type Integer))
  (bind _gunnerui (Variables|Default|GetGunnerUI))
  ;[1 1 1] UI Update
  (if (not (.isdriver (Variables|Default|GetPlayerGameState)))
    (Utilities|IsValid _gunnerui
      (:Is%20Valid
        (Default|UpdateWeapon _gunnerui OnlyAmmo Weapon NewAmmo)))))

(event Custom|SetPlayerName
  (params (name :type String))
  (bind _output_get (Variables|Default|SetPlayerName name))
  (bind _asfunder_drome_base_mode (Utilities|Casting|CastToFunderDromeBaseMode (Game|GetGameMode))))

(event Custom|ShowLoadingScreen
  (bind _self self)
  ;[1 1 1] ShowLoadingScreen
  (Viewport|RemoveAllWidgets)
  (Utilities|IsValid (Variables|Default|GetLoadingScreenRef)
    (:Is%20Valid
      _)
    (:Is%20Not%20Valid
      (bind _returnvalue (UserInterface|CreateWidget "/Game/HUD/MainMenu/LoadingScreen.LoadingScreen_C" _self))
      (Variables|Default|SetLoadingScreenRef _returnvalue)))
  (UserInterface|Viewport|AddtoViewport (Variables|Default|GetLoadingScreenRef) 0)
  (Input|SetInputModeGameOnly _self))

(event Custom|LoadPlayerInfo
  ;[1 1 1] Start & Load Player Name
  (bind _asultradrome_game_instance (Utilities|Casting|CastToUltradrome_GameInstance (Game|GetGameInstance)))
  (CallFunction|SetPlayerName (Utilities|String|ToString(Text) (.playername (Variables|/Game/BluePrint/AllLevels/Ultradrome_GameInstance.Ultradrome_GameInstance_C|GetPlayerInfo _asultradrome_game_instance)))))

(event Custom|FireRumble
  (params (Weapon :type Duke_WeaponType%20Enum))
  (switch Utilities|FlowControl|Switch|SwitchonDuke_WeaponType Weapon
    (:NewEnumerator0
      (Game|Feedback|PlayDynamicForceFeedback 1.0 0.15 false true false true))
    (:NewEnumerator1
      (Utilities|FlowControl|Sequence
        (:then_0
          (Game|Feedback|PlayDynamicForceFeedback (stale _newtrack_4) -1.0 true false true false :!label _label))
        (:then_1
          (bind _newtrack_4 (Timeline|GrenadeTimeline PlayFromStart)
            (:Update
              (goto _label Update))
            (:Finished
              (goto _label Stop))))))
    (:NewEnumerator2
      (Game|Feedback|PlayDynamicForceFeedback 0.3 0.05 true false true false))
    (:NewEnumerator3
      (Utilities|FlowControl|Sequence
        (:then_0
          (Game|Feedback|PlayDynamicForceFeedback (stale _railgun) -1.0 true false true false :!label _label_2))
        (:then_1
          (bind _railgun (Timeline|RailgunRumbleTimeline PlayFromStart)
            (:Update
              (goto _label_2 Update))
            (:Finished
              (goto _label_2 Stop))))))))

(event Custom|GameOver%20Win
  (params (WinningTeam :type Integer))
  (CallFunction|RoundOver WinningTeam))

(event Custom|SetupUI
  (params (IsDriver :type Boolean) (Team :type Integer) (CarNumber :type Integer) (GameMode :type Integer) (MaxScore :type Integer) (MaxTeam :type Integer) (MapID :type Integer))
  (bind _self self)
  ;[1 1 1] Setup UI
  (Viewport|RemoveAllWidgets)
  (bind _structout (Utilities|Struct|SetmembersinPlayerGameState (Variables|Default|GetPlayerGameState) IsDriver Team CarNumber))
  (Utilities|FlowControl|Sequence
    (:then_0
      (if IsDriver
        (Utilities|IsValid (Variables|Default|GetDriverUI)
          (:Is%20Valid
            (if (not (UserInterface|Viewport|IsinViewport (Variables|Default|GetDriverUI)))
              (UserInterface|Viewport|AddtoViewport (stale _output_get) 0 :!label _label)
              (Default|GameModeupdate (stale _output_get) GameMode MaxScore MaxTeam MapID (Variables|Default|GetMapName))))
          (:Is%20Not%20Valid
            (bind _returnvalue (UserInterface|CreateWidget "/Game/HUD/InGameUI/DriverUI.DriverUI_C" _self Team))
            (bind _output_get (Variables|Default|SetDriverUI _returnvalue))
            (goto _label)))
        (else
          (Utilities|IsValid (Variables|Default|GetGunnerUI)
            (:Is%20Valid
              (if (not (UserInterface|Viewport|IsinViewport (Variables|Default|GetGunnerUI)))
                (UserInterface|Viewport|AddtoViewport (stale _output_get_2) 0 :!label _label_2)
                (Default|GameModeupdate (stale _output_get_2) GameMode MaxScore MaxTeam MapID (Variables|Default|GetMapName))))
            (:Is%20Not%20Valid
              (bind _returnvalue_2 (UserInterface|CreateWidget "/Game/HUD/InGameUI/TurretUI.TurretUI_C" _self Team))
              (bind _output_get_2 (Variables|Default|SetGunnerUI _returnvalue_2))
              (goto _label_2))))))
    (:then_1
      (CallFunction|SetPllayerStat _structout))))

(event Custom|Update%20CarHealth
  (params (NewHealth :type Float%20%28single-precision%29))
  (bind _driverui (Variables|Default|GetDriverUI))
  (bind _gunnerui (Variables|Default|GetGunnerUI))
  ;[1 1 1] UI Update
  (if (.isdriver (Variables|Default|GetPlayerGameState))
    (Utilities|IsValid _driverui
      (:Is%20Valid
        (Default|UpdateCarHealth _driverui NewHealth)))
    (else
      (Utilities|IsValid _gunnerui
        (:Is%20Valid
          (Default|UpdateCarHealth _gunnerui NewHealth))))))

(event Custom|ShowGameMode
  (params (GameMode :type Text) (MapName :type Text))
  (Development|PrintString (Utilities|String|ToString(Text) (Utilities|Text|FormatText "{name} : {mode}" MapName GameMode)) true true "(R=0.000000,G=0.660000,B=1.000000,A=1.000000)" 2e+01))

(event Custom|SetgameUI
  (params (UI :type Integer))
  (bind _driverui (Variables|Default|GetDriverUI))
  (bind _gunnerui (Variables|Default|GetGunnerUI))
  (if (.isdriver (Variables|Default|GetPlayerGameState))
    (switch int UI
      (:Default
        (Default|ActivateDM _driverui :!label _label))
      (:0
        (goto _label))
      (:1
        (Default|ActivateF4All _driverui))
      (:2
        (Default|ActivateCTB _driverui)))
    (else
      (switch int UI
        (:Default
          (Default|ActivateDM _gunnerui :!label _label_2))
        (:0
          (goto _label_2))
        (:1
          (Default|ActivateF4All _gunnerui))
        (:2
          (Default|ActivateCTB _gunnerui))))))

(event Custom|HitDirection
  (params (Angle :type Float%20%28single-precision%29))
  (if (> Angle 0.0)
    (Game|Feedback|PlayDynamicForceFeedback 1.0 0.1 false false true false)
    (else
      (Game|Feedback|PlayDynamicForceFeedback 1.0 0.1 true false false false))))

(event Custom|target%20hit%20blood%20screen
  (Default|TargetHitGrapeJelly (Variables|Default|GetDriverUI)))

(event Custom|GameReadyCountDown
  ;[1 1 1] UI Update
)

(event Custom|ControllerRumble
  (params (Acc :type Vector) (Vel :type Float%20%28single-precision%29) (OnGround :type Boolean))
  (bind _returnvalue (Math|Vector|VectorLength Acc))
  (bind _returnvalue_2 (/ Vel 3e+04))
  (bind _returnvalue_3 (Math|Float|Clamp(Float) _returnvalue_2 0.0 0.2))
  (Utilities|FlowControl|Sequence
    (:then_0
      (if OnGround
        (Variables|Default|SetRumbleStrengthLS _returnvalue_3)
        (Variables|Default|SetRumbleStrengthRS _returnvalue_3)
        (else
          (Variables|Default|SetRumbleStrengthLS 0.0)
          (Variables|Default|SetRumbleStrengthRS 0.0))))
    (:then_1
      (if (>= _returnvalue 2e+01)
        (if (>= _returnvalue 5e+01)
          (Variables|Default|SetRumbleStrengthLL 0.5)
          (Variables|Default|SetRumbleStrengthRL 0.5)
          (else
            (Variables|Default|SetRumbleStrengthLL 0.5)
            (Variables|Default|SetRumbleStrengthRL 0.0)))
        (else
          (Variables|Default|SetRumbleStrengthLL 0.0)
          (Variables|Default|SetRumbleStrengthRL 0.0))))))

(event Custom|UpdatePayloadHealth
  (params (NewHealth :type Float%20%28single-precision%29))
  (Development|PrintString (Utilities|String|ToString(Float) NewHealth) true true "(R=0.000000,G=0.660000,B=1.000000,A=1.000000)" 1.0)
  (if (.isdriver (Variables|Default|GetPlayerGameState))
    _))

(event Custom|Death%20removeUI
  (Viewport|RemoveAllWidgets))

(event Custom|Aquire%20Player%20Name
  (bind _asultradrome_game_instance (Utilities|Casting|CastToUltradrome_GameInstance (Game|GetGameInstance)))
  (CallFunction|SetPlayerName (Utilities|String|ToString(Text) (.playername (Variables|/Game/BluePrint/AllLevels/Ultradrome_GameInstance.Ultradrome_GameInstance_C|GetPlayerInfo _asultradrome_game_instance)))))

(event Custom|SetPllayerStat
  (params (State :type Player%20Game%20State%20Structure))
  (Variables|Default|SetPlayerGameState State))

(event Custom|Round%20Over
  (params (WinningTeam :type Integer))
  (bind _playergamestate (Variables|Default|GetPlayerGameState))
  (bind _returnvalue (== WinningTeam (.team _playergamestate)))
  (if (.isdriver _playergamestate)
    (Default|WinorLose (Variables|Default|GetDriverUI) _returnvalue)
    (else
      (Default|WinorLose (Variables|Default|GetGunnerUI) _returnvalue))))

(event Custom|AttackRumble
  (params (AttackAngle :type Float%20%28single-precision%29))
  (if (> (stale Custom|HitDirection Angle) 0.0)
    (Game|Feedback|PlayDynamicForceFeedback 1.0 0.1 false false true false)
    (else
      (Game|Feedback|PlayDynamicForceFeedback 1.0 0.1 true false false false))))

(event Custom|target%20hit
  ;[1 1 1] UI Update
  (Default|TargetHit (Variables|Default|GetGunnerUI)))

(event EventBeginPlay
  (Variables|Default|SetbForceFeedbackEnabled true))

(event EventTick
  (params (DeltaSeconds :type Float%20%28single-precision%29))
  (Utilities|FlowControl|Sequence
    (:then_0
      (Game|Feedback|PlayDynamicForceFeedback (Variables|Default|GetRumbleStrengthLS) -1.0 false true false false) ; enters at Update
    )
    (:then_1
      (Game|Feedback|PlayDynamicForceFeedback (Variables|Default|GetRumbleStrengthRS) -1.0 false false false true) ; enters at Update
    )
    (:then_2
      (Game|Feedback|PlayDynamicForceFeedback (Variables|Default|GetRumbleStrengthLL) -1.0 true false false false) ; enters at Update
    )
    (:then_3
      (Game|Feedback|PlayDynamicForceFeedback (Variables|Default|GetRumbleStrengthRL) -1.0 false false true false) ; enters at Update
    )))

(event Input|ActionEvents|InputActionToggleScoreboard
  (params (Key :type Key%20Structure :default "AnyKey"))
  (bind _playergamestate (Variables|Default|GetPlayerGameState))
  (bind _gunnerui (Variables|Default|GetGunnerUI))
  (bind _driverui (Variables|Default|GetDriverUI))
  (:Pressed
    (if (.isdriver _playergamestate)
      (Default|ToggleScoreboard(UI) _driverui)
      (else
        (Default|ToggleScoreboard(UI) _gunnerui))))
  (:Released
    (if (.isdriver _playergamestate)
      (Default|HideScoreboard(UI) _driverui)
      (else
        (Default|HideScoreboard(UI) _gunnerui)))))

(event Input|ActionEvents|InputActionToggleMiniMap
  (params (Key :type Key%20Structure :default "AnyKey"))
  (:Pressed
    (if (.isdriver (Variables|Default|GetPlayerGameState))
      (Default|ToggleMiniMap (Variables|Default|GetDriverUI))
      (else
        (Default|ToggleMiniMap (Variables|Default|GetGunnerUI))))))

(event Input|ActionEvents|InputActionDebugKey
  (params (Key :type Key%20Structure :default "AnyKey"))
  (bind _returnvalue (Game|GetPlayerCameraManager 0))
  (bind _returnvalue_2 (Transformation|GetActorTransform _returnvalue))
  (bind (_location _rotation) (Math|Transform|BreakTransform _returnvalue_2))
  (bind (_roll _pitch _yaw) (Math|Rotator|BreakRotator _rotation))
  ;[1 1 1] Debug Func
  (:Pressed
    (Utilities|FlowControl|DoOnce false :!label _label
      (:Completed
        (bind _asmy_spec_pawn (Utilities|Casting|CastToMySpecPawn (Pawn|GetControlledPawn))
          (:then
            (Utilities|IsValid (Variables|/Game/BluePrint/MySpecPawn.MySpecPawn_C|GetPawnSelected _asmy_spec_pawn)
              (:Is%20Valid
                (Pawn|Possess (Variables|/Game/BluePrint/MySpecPawn.MySpecPawn_C|GetPawnSelected _asmy_spec_pawn)))))
          (:CastFailed
            (bind _returnvalue_3 (Game|SpawnActorfromClass "/Game/BluePrint/MySpecPawn.MySpecPawn_C" (Math|Transform|MakeTransform _location (Math|Rotator|MakeRotator 0.0 _pitch _yaw)) "AlwaysSpawn" 0 0))
            (Pawn|Possess _returnvalue_3))))))
  (:Released
    (goto _label Reset)))

(fn ConstructionScript)
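; Base game mode for FunderDrome team car combat, where each car has a driver and a turret gunner.
; A Cars placeholder array indexed by team and car number seats players carried over from the lobby through a timed queue.
; Helpers spawn car-turret pairs, possess them with players or optional AI, and fire projectiles.
; Kills update records, spawn death cams and wrecks, and broadcast a feed; match end server-travels everyone to the lobby.
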(event Custom|DamageNotify
  (params (Instigator :type Actor%20Object%20Reference))
  (bind _asfunder_drome_turret_base (Utilities|Casting|CastToFunderDromeTurretBase Instigator))
  (Default|TargetHit _asfunder_drome_turret_base))

(event Custom|EventCarKilled
  (params (VictimID :type Integer) (Weapon :type Duke_WeaponType%20Enum) (PlayerKill :type Boolean) (KillerID :type Integer))
  (Default|CallCarKill VictimID Weapon PlayerKill KillerID))

(event Custom|CarKilled
  (params (VictimID :type Integer) (Weapon :type Duke_WeaponType%20Enum) (PlayerKill :type Boolean) (Killer :type Integer))
  (bind _killbroadcast (CallFunction|CarKillHandle VictimID Weapon PlayerKill Killer))
  (for _array_element (Variables|Default|GetPlayerList)
    (Default|BroadcastKill _array_element _killbroadcast)))

(event Custom|EndOfMatch
  (params (WinningTeam :type Integer) (WinLocation :type Vector))
  ;[1 1 1] End Of Match Spawn Spectator Pawn
  (Variables|Default|SetGameModeReady false)
  (bind _outactors (Actor|GetAllActorsOfClass "/Game/BluePrint/AIScript/FunderDromeAIController.FunderDromeAIController_C"))
  (for _array_element _outactors
    (Pawn|UnPossess _array_element)
    (Actor|DestroyActor _array_element))
  (bind _outactors_2 (Actor|GetAllActorsOfClass "/Game/BluePrint/Turret/FunderDromeTurretBase.FunderDromeTurretBase_C"))
  (for _array_element_2 _outactors_2
    (Variables|/Game/BluePrint/Turret/FunderDromeTurretBase.FunderDromeTurretBase_C|SetFireing _array_element_2 false))
  (for _array_element_3 (Variables|Default|GetPlayerList)
    (bind _returnvalue (Game|SpawnActorfromClass "/Game/BluePrint/DeathSpecPawn.DeathSpecPawn_C" (Math|Transform|MakeTransform WinLocation "0, 0, 0" "1,1,1.000000") "Undefined" 0 0))
    (Pawn|Possess _array_element_3 _returnvalue)
    (Default|GameOverWin _array_element_3 WinningTeam))
  ;[1 1 1] GameOver Travel to Lobby
  (Utilities|FlowControl|Delay 2e+01)
  (for _array_element_4 (Variables|Default|GetPlayerList)
    (Input|SetInputModeGameOnly _array_element_4)
    (Viewport|RemoveAllWidgets)
    (Default|ShowLoadingScreen _array_element_4))
  (Development|ExecuteConsoleCommand (Utilities|String|Append "servertravel " "/Game/Maps/" "Lobby" "?game=/Game/MyBluePrint/AllLevels/" "FunderDromeLobbyMode.FunderDromeLobbyMode_C") (Game|GetPlayerController 0)))

(event Custom|HealthUpdateForPlayer
  (params (ID :type Integer) (Health :type Float%20%28single-precision%29))
  (bind _cars (Variables|Default|GetCars))
  (bind _item (Utilities|Array|Get(acopy) _cars ID))
  (bind (_driver _team _carnumber _cooldowntimer _gunner) (Utilities|Struct|BreakCarPlaceholder _item))
  (bind _asultradrome_player_controller (Utilities|Casting|CastToUltradrome_PlayerController _driver)
    (:then
      (Default|UpdateCarHealth _asultradrome_player_controller Health))
    (:CastFailed
      _))
  (bind _asultradrome_player_controller_2 (Utilities|Casting|CastToUltradrome_PlayerController _gunner))
  (Default|UpdateCarHealth _asultradrome_player_controller_2 0.0))

(event Custom|SetQueuePlayerToList
  ;[1 1 1] Init
  (CallFunction|ClearQueue))

(event EventOnSwapPlayerControllers
  (params (OldPC :type Player%20Controller%20Object%20Reference) (NewPC :type Player%20Controller%20Object%20Reference))
  (bind _asultradrome_player_controller (Utilities|Casting|CastToUltradrome_PlayerController NewPC))
  ;[1 1 1] TransferPlayer
  (bind _asfunderdrome_lobby_controller (Utilities|Casting|CastToFunderdromeLobbyController OldPC))
  (Variables|/Game/BluePrint/AllLevels/Ultradrome_PlayerController.Ultradrome_PlayerController_C|SetPlayerGameState _asultradrome_player_controller (Utilities|Struct|MakePlayerGameState (.isdriver (Variables|/Game/BluePrint/AllLevels/FunderdromeLobbyController.FunderdromeLobbyController_C|GetLobbyInfo _asfunderdrome_lobby_controller)) (.team (Variables|/Game/BluePrint/AllLevels/FunderdromeLobbyController.FunderdromeLobbyController_C|GetLobbyInfo _asfunderdrome_lobby_controller)) (.carnumber (Variables|/Game/BluePrint/AllLevels/FunderdromeLobbyController.FunderdromeLobbyController_C|GetLobbyInfo _asfunderdrome_lobby_controller)) 0 0 true))
  (Utilities|Array|AddUnique (Variables|Default|GetPlayerList) _asultradrome_player_controller)
  (Utilities|Array|AddUnique (Variables|Default|GetQueuePlayers) _asultradrome_player_controller))

(event EventPostLogin
  (params (NewPlayer :type Player%20Controller%20Object%20Reference))
  (bind _asultradrome_player_controller (Utilities|Casting|CastToUltradrome_PlayerController NewPlayer))
  (Utilities|Array|AddUnique (Variables|Default|GetPlayerList) _asultradrome_player_controller))

(event EventBeginPlay
  ;[1 1 1] Init
  (Variables|Default|SetColorList (Variables|/Game/BluePrint/AllLevels/Ultradrome_GameInstance.Ultradrome_GameInstance_C|GetColorList (.AsUltradrome%20Game%20Instance (Utilities|Casting|CastToUltradrome_GameInstance (Game|GetGameInstance)))))
  (CallFunction|GameModeInit)
  (CallFunction|ClearQueue)
  (Utilities|Time|SetTimerbyEvent (delegate Custom|SetQueuePlayerToList) 2.0 true))

(event EventTick
  (params (DeltaSeconds :type Float%20%28single-precision%29))
  (Variables|Default|SetDeltaTime DeltaSeconds))

(event EventOnLogout
  (params (ExitingController :type Controller%20Object%20Reference)))

(fn ConstructionScript)

(fn WeaponFired
  (params (Turret :type Pawn%20Object%20Reference) (WeaponType :type Duke_WeaponType%20Enum) (MuzzleLocation :type Vector) (Forward :type Vector))
  (bind _returnvalue (Math|Conversions|RotationFromXVector Forward))
  (bind _returnvalue_2 (Math|Transform|MakeTransform MuzzleLocation _returnvalue))
  (switch Utilities|FlowControl|Switch|SwitchonDuke_WeaponType WeaponType
    (:NewEnumerator1
      (Game|SpawnActorfromClass "/Game/BluePrint/Turret/Duke_Grenade.Duke_Grenade_C" _returnvalue_2 "AlwaysSpawn" 0 Turret))
    (:NewEnumerator2
      (Game|SpawnActorfromClass "/Game/BluePrint/Turret/Duke_Plasma.Duke_Plasma_C" _returnvalue_2 "AlwaysSpawn" 0 Turret))
    (:NewEnumerator3
      (Game|SpawnActorfromClass "/Game/BluePrint/Turret/Duke_Railgun.Duke_Railgun_C" _returnvalue_2 "AlwaysSpawn" 0 Turret))))

(fn RespawnCar
  (params (Transform :type Transform) (DayTime :type Boolean) (CarSetup :type CarSetups%20Enum) (TurretSetup :type Duke_WeaponType%20Enum) (Team :type Integer))
  (bind _returnvalue (Game|SpawnActorfromClass "/Game/TestCar/BP/FunderDromeCarBase.FunderDromeCarBase_C" Transform "AlwaysSpawn" 0 DayTime Team))
  (LocalVariables|SetCar _returnvalue)
  (if (Utilities|Enum|Equal(Enum) CarSetup "NewEnumerator0")
    (Components|StaticMesh|SetStaticMesh (Variables|/Game/TestCar/BP/FunderDromeCarBase.FunderDromeCarBase_C|GetProxy (LocalVariables|GetCar)) "/Game/Models/Models/MilitaryJeep_2.MilitaryJeep_2")
    (Transformation|SetRelativeScale3D (Variables|/Game/TestCar/BP/FunderDromeCarBase.FunderDromeCarBase_C|GetProxy (LocalVariables|GetCar)) "1.750000,1.750000,1.750000"))
  (bind _returnvalue_2 (Game|SpawnActorfromClass "/Game/BluePrint/Turret/FunderDromeTurretBase.FunderDromeTurretBase_C" Transform "AlwaysSpawn" 0 TurretSetup 0))
  (bind _output_get (LocalVariables|SetTurret _returnvalue_2))
  (Default|TurretSetupServer _output_get)
  (Transformation|AttachComponentToComponent _returnvalue_2 (Variables|/Game/TestCar/BP/FunderDromeCarBase.FunderDromeCarBase_C|GetProxy (LocalVariables|GetCar)) "TurretSocket" "SnapToTarget" "KeepWorld" "KeepWorld" true)
  (return (LocalVariables|GetCar) (LocalVariables|GetTurret)))

(fn CheckforAvailablePawns
  (params (Controller :type Ultradrome%20Player%20Controller%20Object%20Reference))
  (bind (_array_element _array_index) (Utilities|Array|ForEachLoopwithBreak (Variables|Default|GetCars) :!label _label)
    (:LoopBody
      (if (.ExistInGame (Utilities|Struct|BreakCarPlaceholder _array_element))
        (if (Class|KismetMathLibrary|XORBoolean (Utilities|IsValid (.Driver (Utilities|Struct|BreakCarPlaceholder _array_element))) (Utilities|IsValid (.Gunner (Utilities|Struct|BreakCarPlaceholder _array_element))))
          (if (Utilities|IsValid (.Driver (Utilities|Struct|BreakCarPlaceholder _array_element)))
            (Utilities|Struct|SetmembersinCarPlaceholder _array_element Controller)
            (LocalVariables|SetFound_0 true)
            (LocalVariables|SetCarIndex_0 _array_index)
            (LocalVariables|SetDriver_0 true)
            (goto _label Break)
            (elif (Utilities|IsValid (.Gunner (Utilities|Struct|BreakCarPlaceholder _array_element)))
              (Utilities|Struct|SetmembersinCarPlaceholder _array_element Controller)
              (LocalVariables|SetFound_0 true)
              (LocalVariables|SetCarIndex_0 _array_index)
              (LocalVariables|SetDriver_0 false)
              (goto _label Break))))))
    (:Completed
      (return (LocalVariables|GetFound_0) (LocalVariables|GetCarIndex_0) (LocalVariables|GetDriver_0)))))

(fn SetPlayerstoPlaceholders
  (params (PlayerController :type Ultradrome%20Player%20Controller%20Object%20Reference))
  (bind _playergamestate (Variables|/Game/BluePrint/AllLevels/Ultradrome_PlayerController.Ultradrome_PlayerController_C|GetPlayerGameState PlayerController))
  (bind _playerstate (Variables|/Script/Engine.Controller|GetPlayerState PlayerController))
  (bind _cars (Variables|Default|GetCars))
  (bind _cars_2 (Variables|Default|GetCars))
  (bind _cars_3 (Variables|Default|GetCars))
  (bind (_isdriver _team _carnumber _killcountthismatch _deathcountthismatch _transferedplayer) (Utilities|Struct|BreakPlayerGameState _playergamestate))
  (bind _asultradrome_player_state (Utilities|Casting|CastToUltradrome_PlayerState _playerstate))
  (bind (_index _carref) (CallFunction|GetCarIndex _carnumber _team))
  (bind _displayname (Variables|/Game/BluePrint/AllLevels/Ultradrome_PlayerState.Ultradrome_PlayerState_C|GetDisplayName _asultradrome_player_state))
  (if _transferedplayer
    (if _isdriver
      (bind _structout (Utilities|Struct|SetmembersinCarPlaceholder _carref PlayerController _displayname true))
      (Utilities|Array|SetArrayElem _cars _index _structout)
      (else
        (bind _structout_2 (Utilities|Struct|SetmembersinCarPlaceholder _carref PlayerController _displayname true))
        (Utilities|Array|SetArrayElem _cars _index _structout_2)))
    (return)
    (else
      (bind (_array_element _array_index) (Utilities|Array|ForEachLoopwithBreak _cars_3 :!label _label)
        (:LoopBody
          (if (Class|KismetMathLibrary|XORBoolean (Utilities|IsValid (.Driver (Utilities|Struct|BreakCarPlaceholder _array_element))) (Utilities|IsValid (.Gunner (Utilities|Struct|BreakCarPlaceholder _array_element))))
            (if (Utilities|IsValid (.Driver (Utilities|Struct|BreakCarPlaceholder _array_element)))
              (bind _structout_3 (Utilities|Struct|SetmembersinCarPlaceholder _array_element PlayerController _displayname))
              (Utilities|Array|SetArrayElem _cars_2 _array_index _structout_3)
              (goto _label Break)
              (elif (Utilities|IsValid (.Gunner (Utilities|Struct|BreakCarPlaceholder _array_element)))
                (bind _structout_4 (Utilities|Struct|SetmembersinCarPlaceholder _array_element PlayerController _displayname))
                (Utilities|Array|SetArrayElem _cars_2 _array_index _structout_4)
                (goto _label Break)))))
        (:Completed
          (bind (_array_element_2 _array_index_2) (Utilities|Array|ForEachLoopwithBreak _cars_3 :!label _label_2)
            (:LoopBody
              (if (.ExistInGame (Utilities|Struct|BreakCarPlaceholder _array_element_2))
                (bind _structout_5 (Utilities|Struct|SetmembersinCarPlaceholder _array_element_2 PlayerController _displayname true))
                (Utilities|Array|SetArrayElem (Variables|Default|GetCars) _array_index_2 _structout_5)
                (goto _label_2 Break)))
            (:Completed
              (return))))))))

(fn GameModeInit
  (bind _maxplayer (Variables|Default|GetMaxPlayer))
  (bind _maxteam (Variables|Default|GetMaxTeam))
  (if (== (Math|Integer|%(Integer) _maxplayer (Variables|Default|GetMaxTeam)) 0)
    (for _index (range 0 (- (/ _maxplayer 2) 1))
      (Utilities|Array|Add (Variables|Default|GetCars) (Utilities|Struct|MakeCarPlaceholder 0 (+ (Math|Integer|%(Integer) _index _maxteam) 1) (+ (/ _index _maxteam) 1) 1.0 0 0 0 0 0 false (Utilities|String|Append "Driver" (Utilities|String|ToString(Integer) (+ (/ _index _maxteam) 1))) "(R=0.000000,G=0.000000,B=0.000000,A=0.000000)" (Utilities|String|Append "Gunner" (Utilities|String|ToString(Integer) (+ (/ _index _maxteam) 1))))))
    (Variables|Default|SetGameModeReady true)
    (else
      (CallFunction|EndOfMatch 0 "0, 0, 0")))
  (return))

(fn ClearQueue
  (bind _queueplayers (Variables|Default|GetQueuePlayers))
  (for _array_element _queueplayers
    (CallFunction|SetPlayerstoPlaceholders _array_element)
    (Utilities|Array|RemoveItem _queueplayers _array_element)))

(fn ControllerPosses
  (params (Index :type Integer))
  (bind _cars (Variables|Default|GetCars))
  (bind _item (Utilities|Array|Get(acopy) _cars Index))
  (bind (_driver _team _carnumber _cooldowntimer _gunner _car _turret) (Utilities|Struct|BreakCarPlaceholder _item))
  (if (Utilities|IsValid _driver)
    (Pawn|Possess _driver _car)
    (Default|SetupUI (.AsUltradrome%20Player%20Controller (Utilities|Casting|CastToUltradrome_PlayerController _driver)) true _team _carnumber (Variables|Default|GetGameMode))
    (elif (Variables|Default|GetHasAI)
      (bind _returnvalue (Game|SpawnActorfromClass "/Game/BluePrint/AIScript/FunderDromeAIController.FunderDromeAIController_C" (Math|Transform|MakeTransform "0, 0, 0") "AlwaysSpawn" 0 0))
      (Pawn|Possess _returnvalue _car)
      (bind _structout (Utilities|Struct|SetmembersinCarPlaceholder _item _returnvalue))
      (Utilities|Array|SetArrayElem _cars Index _structout)))
  (if (Utilities|IsValid _gunner)
    (Pawn|Possess _gunner _turret)
    (Default|SetupUI (.AsUltradrome%20Player%20Controller (Utilities|Casting|CastToUltradrome_PlayerController _gunner)) false _team _carnumber (Variables|Default|GetGameMode))
    (elif (Variables|Default|GetHasAI)
      (bind _returnvalue_2 (Game|SpawnActorfromClass "/Game/BluePrint/AIScript/FunderDromeAIController.FunderDromeAIController_C" (Math|Transform|MakeTransform "0, 0, 0") "AlwaysSpawn" 0 0))
      (Pawn|Possess _returnvalue_2 _turret)
      (bind _structout_2 (Utilities|Struct|SetmembersinCarPlaceholder _item _returnvalue_2))
      (Utilities|Array|SetArrayElem _cars Index _structout_2)))
  (return))

(fn GetCarIndex
  (params (CarNumber :type Integer) (team :type Integer))
  (bind _returnvalue (- CarNumber 1))
  (bind _returnvalue_2 (- team 1))
  (bind _maxteam (Variables|Default|GetMaxTeam))
  (bind _returnvalue_3 (* _returnvalue _maxteam))
  (bind _returnvalue_4 (+ _returnvalue_2 _returnvalue_3))
  (return _returnvalue_4 (Utilities|Array|Get(acopy) (Variables|Default|GetCars) _returnvalue_4)))

(fn WeaponPickup
  (params (Weapon :type Duke_WeaponType%20Enum) (Car :type Integer))
  (Default|WeaponPickupServer (.AsFunder%20Drome%20Turret%20Base (Utilities|Casting|CastToFunderDromeTurretBase (.Turret (Utilities|Struct|BreakCarPlaceholder (Utilities|Array|Get(acopy) (Variables|Default|GetCars) Car))))) Weapon))

(fn CarKillHandle
  (params (VictimID :type Integer) (Weapon :type Duke_WeaponType%20Enum) (PlayerKill :type Boolean) (KillerID :type Integer))
  (bind _cars (Variables|Default|GetCars))
  (bind _item (Utilities|Array|Get(acopy) _cars KillerID))
  (bind (_driver _team _carnumber _cooldowntimer _gunner _car _turret _kills _death _needrespawn _drivername _drivercolor _gunnername) (Utilities|Struct|BreakCarPlaceholder _item))
  (LocalVariables|SetTempID VictimID)
  (LocalVariables|SetTempFeed (Utilities|Struct|MakeKillFeed PlayerKill))
  (bind _output_get (LocalVariables|SetTempHolder (Utilities|Array|Get(acopy) _cars (LocalVariables|GetTempID))))
  (bind _output_get_2 (LocalVariables|SetTempLoc (Transformation|GetActorLocation (.Car (Utilities|Struct|BreakCarPlaceholder _output_get)))))
  (LocalVariables|SetKillLoc (Math|Transform|MakeTransform _output_get_2 "0,0.000000, 0"))
  (if PlayerKill
    ;[1 1 1] Killer Info
    (bind _structout (Utilities|Struct|SetmembersinKillFeed (LocalVariables|GetTempFeed) true _drivername _gunnername Weapon (+ _kills 1) _team (Utilities|Array|Get(acopy) (Variables|Default|GetScores) _team)))
    (LocalVariables|SetTempFeed _structout)
    (bind _structout_2 (Utilities|Struct|SetmembersinCarPlaceholder _item (+ (.Kills (Utilities|Struct|BreakCarPlaceholder _item)) 1)))
    (Utilities|Array|SetArrayElem _cars KillerID _structout_2)
    (Default|TargetKill (.AsFunder%20Drome%20Turret%20Base (Utilities|Casting|CastToFunderDromeTurretBase _turret))))
  (bind _returnvalue (Game|SpawnActorfromClass "/Game/BluePrint/DeathSpecPawn.DeathSpecPawn_C" (LocalVariables|GetKillLoc) "AlwaysSpawn" 0 0))
  (Variables|/Game/BluePrint/DeathSpecPawn.DeathSpecPawn_C|SetDeathCam _returnvalue true)
  (Utilities|IsValid (.Driver (Utilities|Struct|BreakCarPlaceholder (LocalVariables|GetTempHolder)))
    (:Is%20Valid
      (bind _asultradrome_player_controller (Utilities|Casting|CastToUltradrome_PlayerController (.Driver (Utilities|Struct|BreakCarPlaceholder (LocalVariables|GetTempHolder))))
        (:then
          (Pawn|Possess _asultradrome_player_controller _returnvalue))
        (:CastFailed
          (Actor|DestroyActor _returnvalue :!label _label)
          (Actor|DestroyActor (.Driver (Utilities|Struct|BreakCarPlaceholder (LocalVariables|GetTempHolder)))))))
    (:Is%20Not%20Valid
      (goto _label)))
  (bind _returnvalue_2 (Game|SpawnActorfromClass "/Game/BluePrint/DeathSpecPawn.DeathSpecPawn_C" (LocalVariables|GetKillLoc) "AlwaysSpawn" 0 0))
  (Variables|/Game/BluePrint/DeathSpecPawn.DeathSpecPawn_C|SetDeathCam _returnvalue_2 true)
  (Utilities|IsValid (.Gunner (Utilities|Struct|BreakCarPlaceholder (LocalVariables|GetTempHolder)))
    (:Is%20Valid
      (bind _asultradrome_player_controller_2 (Utilities|Casting|CastToUltradrome_PlayerController (.Gunner (Utilities|Struct|BreakCarPlaceholder (LocalVariables|GetTempHolder))))
        (:then
          (Pawn|Possess _asultradrome_player_controller_2 _returnvalue_2))
        (:CastFailed
          (Actor|DestroyActor _returnvalue_2 :!label _label_2)
          (Actor|DestroyActor (.Gunner (Utilities|Struct|BreakCarPlaceholder (LocalVariables|GetTempHolder)))))))
    (:Is%20Not%20Valid
      (goto _label_2)))
  (Game|SpawnActorfromClass "/Game/BluePrint/Vehicle/DestroiedCar.DestroiedCar_C" (LocalVariables|GetKillLoc) "Undefined" 0 0)
  (Actor|DestroyActor (.Car (Utilities|Struct|BreakCarPlaceholder (LocalVariables|GetTempHolder))))
  (bind _structout_3 (Utilities|Struct|SetmembersinKillFeed (LocalVariables|GetTempFeed) (.DriverName (Utilities|Struct|BreakCarPlaceholder (LocalVariables|GetTempHolder))) (.GunnerName (Utilities|Struct|BreakCarPlaceholder (LocalVariables|GetTempHolder))) (+ (.Death (Utilities|Struct|BreakCarPlaceholder (LocalVariables|GetTempHolder))) 1) (.Team (Utilities|Struct|BreakCarPlaceholder (LocalVariables|GetTempHolder))) (Utilities|Array|Get(acopy) (Variables|Default|GetScores) (.Team (Utilities|Struct|BreakCarPlaceholder (LocalVariables|GetTempHolder)))) (LocalVariables|GetTempLoc)))
  (LocalVariables|SetTempFeed _structout_3)
  (return (LocalVariables|GetTempID) (LocalVariables|GetTempFeed)))
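; Player controller for the Funderdrome lobby, linking each player's lobby menu to the lobby game mode.
; It creates and shows the Lobby_UI widget with UI-only input, and forwards team, car and driver requests to FunderDromeLobbyMode.
; Player list updates cache the list, find this controller's own slot to store as LobbyInfo, and refresh the menu.
; Map and game mode changes are also passed to the menu.
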(event Custom|ShowLobbyMenu
  ;[1 1 1] Show Lobby Menu
  (Utilities|IsValid (Variables|Default|GetLobbyMenu)
    (:Is%20Valid
      _)
    (:Is%20Not%20Valid
      (bind _returnvalue (UserInterface|CreateWidget "/Game/HUD/InGameMenu/Lobby_UI.Lobby_UI_C" self))
      (Variables|Default|SetLobbyMenu _returnvalue)))
  (UserInterface|Viewport|AddtoViewport (Variables|Default|GetLobbyMenu) 0)
  (Variables|Default|SetbShowMouseCursor true)
  (Input|SetInputModeUIOnly self (Variables|Default|GetLobbyMenu) "DoNotLock"))

(event Custom|UpdateUIPlayers
  (params (List :type Array%20of%20Player%20Lobby%20Info%20Structures))
  ;[1 1 1] Update All Player Info
  (Default|RefreshPlayerInfo (Variables|Default|GetLobbyMenu) List))

(event Custom|PlayerChangePosition
  (params (Team :type Integer) (Car :type Integer) (Driver? :type Boolean))
  ;[1 1 1] Player Apply For A New Position
  (bind _asfunder_drome_lobby_mode (Utilities|Casting|CastToFunderDromeLobbyMode (Game|GetGameMode)))
  (Default|PlayerSetup _asfunder_drome_lobby_mode self Car Team Driver?))

(event Custom|UpdatePlayers
  (params (PlayerList :type Array%20of%20Player%20Lobby%20Info%20Structures))
  ;[1 1 1] Update All Player Info
  (Variables|Default|SetLobbyPlayerList PlayerList)
  (Utilities|FindSelfinList (Variables|Default|GetLobbyPlayerList)
    (:finished
      (CallFunction|UpdateUIPlayers (Variables|Default|GetLobbyPlayerList)))))

(event Custom|UpdateServerSettings
  (params (MapName :type String) (GameMode :type Game%20Modes%20Structure))
  (bind _lobbymenu (Variables|Default|GetLobbyMenu))
  ;[1 1 1] ServerSettingsUpdate
  (Utilities|IsValid _lobbymenu ; I have no idea why I should check if this thing exists here.
    (:Is%20Valid
      (Default|UpdateServerSettings _lobbymenu MapName GameMode))))

(event EventTick
  (params (DeltaSeconds :type Float%20%28single-precision%29)))

(event Input|KeyboardEvents|F
  (params (Key :type Key%20Structure))
  (:Pressed
    (Default|TestFunction (Variables|Default|GetLobbyMenu))))

(fn ConstructionScript
  (|CallParentFunction))
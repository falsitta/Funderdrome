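; Game mode for Funderdrome two-team deathmatch: kills score for the opposing team until one reaches the 100-point limit.
; GamePrep splits shuffled SpawnZones between teams and queues every car; killed cars rejoin their team's waiting list.
; A looping timer respawns waiting cars in waves, in groups sized by queue length, then re-possesses them and starts AI.
; Another timer insertion-sorts zones by distance to the average car position, favouring spawns near the action.
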(event Custom|HotSpotUpdate
  (CallFunction|UpdateHotSpot))

(event Custom|WaveSpawnEvent
  (CallFunction|WaveSpawn)
  (Utilities|FlowControl|Delay 0.2)
  (bind _outactors (Actor|GetAllActorsOfClass "/Game/BluePrint/AIScript/FunderDromeAIController.FunderDromeAIController_C"))
  (for _array_element _outactors
    (Variables|/Game/BluePrint/AIScript/FunderDromeAIController.FunderDromeAIController_C|SetAIStart _array_element true)))

(event EventBeginPlay
  (Variables|Default|SetHasAI true)
  (Variables|Default|SetFriendlyFire false)
  (|CallParentFunction)
  (CallFunction|GamePrep)
  (CallFunction|WaveSpawn)
  (for (_ _array_index) (Variables|Default|GetCars)
    (CallFunction|ControllerPosses _array_index))
  (Variables|Default|SetStarted true)
  ;[1 1 1] Start CountDown
  (for _array_element (Variables|Default|GetPlayerList)
    (Default|DeathRemoveUI _array_element))
  (Utilities|FlowControl|Delay 5.0)
  (bind _outactors (Actor|GetAllActorsOfClass "/Game/BluePrint/AIScript/FunderDromeAIController.FunderDromeAIController_C"))
  (for _array_element_2 _outactors
    (Variables|/Game/BluePrint/AIScript/FunderDromeAIController.FunderDromeAIController_C|SetAIStart _array_element_2 true))
  (Utilities|Time|SetTimerbyEvent (delegate Custom|WaveSpawnEvent) 1e+01 true)
  (Utilities|Time|SetTimerbyEvent (delegate Custom|HotSpotUpdate) 5.0 true))

(event EventTick
  (params (DeltaSeconds :type Float%20%28single-precision%29))
  (|CallParentFunction DeltaSeconds) ; This node is disabled and will not be called.\nDrag off pins to build functionality.
)

(event EventCarKillEvent
  (params (VictimID :type Integer) (Weapon :type Duke_WeaponType%20Enum :default "NewEnumerator0") (PlayerKill :type Boolean) (KillerID :type Integer))
  (bind _scores (Variables|Default|GetScores))
  (if (not (Variables|Default|GetGameEnd?))
    (bind (_killedcarid _killbroadcast) (CallFunction|CarKillHandle VictimID Weapon PlayerKill KillerID))
    (if (== (.VictimTeam (Utilities|Struct|BreakKillFeed _killbroadcast)) 1)
      (Utilities|Array|AddUnique (Variables|Default|GetTeam1Waiting) _killedcarid)
      (bind _result (Math|Integer|IncrementInt (Utilities|Array|Get(acopy) _scores 1))
        (:%20%20
          (Development|PrintString (Utilities|String|Append "Team2 Score" (Utilities|String|ToString(Integer) _result)))
          (if (>= _result 100)
            (CallFunction|EndOfMatch 2 "0, 0, 0"))))
      (else
        (Utilities|Array|AddUnique (Variables|Default|GetTeam2Waiting) _killedcarid)
        (bind _result_2 (Math|Integer|IncrementInt (Utilities|Array|Get(acopy) _scores))
          (:%20%20
            (Development|PrintString (Utilities|String|Append "Team1 Score" (Utilities|String|ToString(Integer) _result_2)))
            (if (>= _result_2 100)
              (CallFunction|EndOfMatch 1 "0, 0, 0"))))))))

(fn ConstructionScript
  (|CallParentFunction))

(fn GameReadySpawn)

(fn GamePrep
  (bind _outactors (Actor|GetAllActorsOfClass "/Game/BluePrint/Property/SpawnZone.SpawnZone_C"))
  (bind _output_get (Variables|Default|SetSpawnZones _outactors))
  (if (< (Utilities|Array|Length _output_get) 8)
    (Development|PrintString "GameModeError!! Not enough Spawn Zones!!")
    (CallFunction|EndOfMatch 0 "0, 0, 0")
    (else
      (Utilities|Array|Shuffle _output_get)
      (for _array_element (Variables|Default|GetSpawnZones)
        (bind _isa (Utilities|FlowControl|FlipFlop)
          (:A
            _)
          (:B
            _))
        (Variables|/Game/BluePrint/Property/SpawnZone.SpawnZone_C|Setteam _array_element (Math|Integer|SelectInt 1 2 _isa)))
      (for (_array_element_2 _array_index) (Variables|Default|GetCars)
        (if (== (.Team (Utilities|Struct|BreakCarPlaceholder _array_element_2)) 1)
          (Utilities|Array|AddUnique (Variables|Default|GetTeam1Waiting) _array_index)
          (else
            (Utilities|Array|AddUnique (Variables|Default|GetTeam2Waiting) _array_index)))))))

(fn SpawnZoneSpawn
  (params (Cars :type Array%20of%20Integers) (Team :type Integer) (Zone :type Integer))
  (LocalVariables|SetNewCars Cars)
  (LocalVariables|SetTeamNum Team)
  (bind _output_get (LocalVariables|SetShuffle (Variables|/Game/BluePrint/Property/SpawnZone.SpawnZone_C|GetStarts (Utilities|Array|Get(acopy) (Variables|Default|GetSpawnZones) Zone))))
  (Utilities|Array|Shuffle _output_get)
  (for (_array_element _array_index) (LocalVariables|GetNewCars)
    (bind (_newcar _newturret) (CallFunction|RespawnCar (Transformation|GetWorldTransform (Utilities|Array|Get(acopy) (LocalVariables|GetShuffle) _array_index)) true (Utilities|Enum|ByteToEnumCarSetups (Math|Conversions|ToByte(Integer) (- (LocalVariables|GetTeamNum) 1))) (Utilities|Enum|ByteToEnumDuke_WeaponType (Math|Conversions|ToByte(Integer) (Math|Random|RandomIntegerinRange 0 1))) (LocalVariables|GetTeamNum)))
    (LocalVariables|SetCar (.AsFunder%20Drome%20Car%20Base (Utilities|Casting|CastToFunderDromeCarBase _newcar)))
    (LocalVariables|SetTurret (.AsFunder%20Drome%20Turret%20Base (Utilities|Casting|CastToFunderDromeTurretBase _newturret)))
    (Variables|/Game/TestCar/BP/FunderDromeCarBase.FunderDromeCarBase_C|SetDriverNameText (LocalVariables|GetCar) (Utilities|Text|ToText(String) (.DriverName (Utilities|Struct|BreakCarPlaceholder (Utilities|Array|Get(acopy) (Variables|Default|GetCars) _array_element)))))
    (Variables|/Game/TestCar/BP/FunderDromeCarBase.FunderDromeCarBase_C|SetGunnerNameText (LocalVariables|GetCar) (Utilities|Text|ToText(String) (.GunnerName (Utilities|Struct|BreakCarPlaceholder (Utilities|Array|Get(acopy) (Variables|Default|GetCars) _array_element)))))
    (bind _output_get_2 (Variables|/Game/TestCar/BP/FunderDromeCarBase.FunderDromeCarBase_C|SetVehicleID (LocalVariables|GetCar) _array_element))
    (bind _output_get_3 (Variables|/Game/BluePrint/Turret/FunderDromeTurretBase.FunderDromeTurretBase_C|SetVehicleID (LocalVariables|GetTurret) _output_get_2))
    (bind _structout (Utilities|Struct|SetmembersinCarPlaceholder (Utilities|Array|Get(acopy) (Variables|Default|GetCars) _array_element) (LocalVariables|GetCar) (LocalVariables|GetTurret)))
    (Utilities|Array|SetArrayElem (Variables|Default|GetCars) _output_get_3 _structout)
    (Default|CarSetup (LocalVariables|GetCar))
    (Default|DriveStart (LocalVariables|GetCar))
    (Default|WeaponReadyNormal (LocalVariables|GetTurret))))

(fn WaveSpawn
  (bind _nextlist (LocalVariables|GetNextList))
  (bind _nextlist_2 (LocalVariables|GetNextList))
  (bind _team1waiting (Variables|Default|GetTeam1Waiting))
  (bind _team2waiting (Variables|Default|GetTeam2Waiting))
  (LocalVariables|Setteam 0)
  (LocalVariables|SetTeamTemp _team1waiting)
  (Utilities|Array|Clear _team1waiting)
  (while (< (LocalVariables|Getteam) 2)
    (Math|Integer|IncrementInt (LocalVariables|Getteam)
      (:%20%20
        (Utilities|Array|Clear (LocalVariables|GetNextList))
        (if (< (Utilities|Array|Length (LocalVariables|GetTeamTemp)) 20)
          (if (< (Utilities|Array|Length (LocalVariables|GetTeamTemp)) 8)
            (LocalVariables|SetMethod 3)
            (else
              (LocalVariables|SetMethod 4)))
          (else
            (LocalVariables|SetMethod 7)))
        (while (or (> (Utilities|Array|Length (LocalVariables|GetTeamTemp)) 0) (> (Utilities|Array|Length (LocalVariables|GetNextList)) 0))
          (Utilities|Array|AddUnique _nextlist (Utilities|Array|Get(acopy) (LocalVariables|GetTeamTemp)))
          (Utilities|Array|RemoveIndex (LocalVariables|GetTeamTemp))
          (if (or (== (Utilities|Array|Length _nextlist) (LocalVariables|GetMethod)) (== (Utilities|Array|Length (LocalVariables|GetTeamTemp)) 0))
            (LocalVariables|Setcounter 0)
            (LocalVariables|SetFound false)
            (while (not (LocalVariables|GetFound))
              (bind (_array_element _array_index) (Utilities|Array|ForEachLoopwithBreak (Variables|Default|GetSpawnZones) :!label _label)
                (:LoopBody
                  (if (and (== (Variables|/Game/BluePrint/Property/SpawnZone.SpawnZone_C|Getteam _array_element) (LocalVariables|Getteam)) (Variables|/Game/BluePrint/Property/SpawnZone.SpawnZone_C|Getavailable _array_element))
                    (LocalVariables|SetZone _array_index)
                    (Variables|/Game/BluePrint/Property/SpawnZone.SpawnZone_C|Setavailable _array_element false)
                    (LocalVariables|SetFound true)
                    (goto _label Break)))))
            (CallFunction|SpawnZoneSpawn _nextlist_2 (LocalVariables|Getteam) (LocalVariables|GetZone))
            (if (Variables|Default|GetStarted)
              (for _array_element_2 _nextlist_2
                (CallFunction|ControllerPosses _array_element_2)))
            (Utilities|Array|Clear _nextlist_2)))
        (if (== (LocalVariables|Getteam) 1)
          (LocalVariables|SetTeamTemp _team2waiting)
          (Utilities|Array|Clear _team2waiting))))))

(fn UpdateHotSpot
  (bind _outactors (Actor|GetAllActorsOfClass "/Game/TestCar/BP/FunderDromeCarBase.FunderDromeCarBase_C"))
  (bind _returnvalue (Class|GameplayStatics|GetActorArrayAverageLocation _outactors))
  (Variables|Default|SetHotSpot _returnvalue)
  (for (_array_element _array_index) (Variables|Default|GetSpawnZones)
    (LocalVariables|SetThis _array_element)
    (LocalVariables|SetStepper _array_index)
    (LocalVariables|SetCDist (Math|Vector|VectorLength (- (Transformation|GetActorLocation (LocalVariables|GetThis)) (Variables|Default|GetHotSpot))))
    (while (and (> (Math|Vector|VectorLength (- (Transformation|GetActorLocation (Utilities|Array|Get(acopy) (LocalVariables|GetNewList) (- (LocalVariables|GetStepper) 1))) (Variables|Default|GetHotSpot))) (LocalVariables|GetCDist)) (> (LocalVariables|GetStepper) 0))
      (Math|Integer|DecrementInt (LocalVariables|GetStepper)))
    (Utilities|Array|Insert (LocalVariables|GetNewList) (LocalVariables|GetThis) (LocalVariables|GetStepper)))
  (Variables|Default|SetSpawnZones (LocalVariables|GetNewList)))
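; Player controller for menus that turns movement axis input into cursor moves on the main menu.
; MoveForward and MoveRight values beyond a 0.5 dead zone call directional cursor functions on the MainMenu held by Ultradrome_GameInstance.
; The horizontal mapping is reversed, with positive MoveRight moving the cursor left.
; Calls repeat on every axis event past the threshold, with no debounce in this controller.
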(event Input|AxisEvents|InputAxisMoveForward
  (params (AxisValue :type Float%20%28single-precision%29))
  (if (> AxisValue 0.5)
    (Default|MoveCursorUp (Variables|/Game/BluePrint/AllLevels/Ultradrome_GameInstance.Ultradrome_GameInstance_C|GetMainMenu (.AsUltradrome%20Game%20Instance (Utilities|Casting|CastToUltradrome_GameInstance (Game|GetGameInstance)))))))

(event Input|AxisEvents|InputAxisMoveForward
  (params (AxisValue :type Float%20%28single-precision%29))
  (if (< AxisValue -0.5)
    (Default|MoveCursorDown (Variables|/Game/BluePrint/AllLevels/Ultradrome_GameInstance.Ultradrome_GameInstance_C|GetMainMenu (.AsUltradrome%20Game%20Instance (Utilities|Casting|CastToUltradrome_GameInstance (Game|GetGameInstance)))))))

(event Input|AxisEvents|InputAxisMoveRight
  (params (AxisValue :type Float%20%28single-precision%29))
  (if (> AxisValue 0.5)
    (Default|MoveCursorLeft (Variables|/Game/BluePrint/AllLevels/Ultradrome_GameInstance.Ultradrome_GameInstance_C|GetMainMenu (.AsUltradrome%20Game%20Instance (Utilities|Casting|CastToUltradrome_GameInstance (Game|GetGameInstance)))))))

(event Input|AxisEvents|InputAxisMoveRight
  (params (AxisValue :type Float%20%28single-precision%29))
  (if (< AxisValue -0.5)
    (Default|MoveCursorRight (Variables|/Game/BluePrint/AllLevels/Ultradrome_GameInstance.Ultradrome_GameInstance_C|GetMainMenu (.AsUltradrome%20Game%20Instance (Utilities|Casting|CastToUltradrome_GameInstance (Game|GetGameInstance)))))))

(fn ConstructionScript)
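; Player state for Ultradrome that sets the player's display name and registers it with the game mode.
; On BeginPlay it reads the name from the game instance's PlayerInfo and passes it, with player controller 0, to PlayerInfoServerUpdate.
; That event stores DisplayName, forwards it and the controller to FunderDromeBaseMode via CallNameUpdate, then prints the name.
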(event Custom|AquireName
  (bind _asultradrome_game_instance (Utilities|Casting|CastToUltradrome_GameInstance (Game|GetGameInstance)))
  (CallFunction|PlayerInfoServerUpdate (Utilities|String|ToString(Text) (.playername (Variables|/Game/BluePrint/AllLevels/Ultradrome_GameInstance.Ultradrome_GameInstance_C|GetPlayerInfo _asultradrome_game_instance))) (Game|GetPlayerController 0)))

(event Custom|PlayerInfoServerUpdate
  (params (Name :type String) (controllerRef :type Player%20Controller%20Object%20Reference))
  (bind _output_get (Variables|Default|SetDisplayName Name))
  (bind _asfunder_drome_base_mode (Utilities|Casting|CastToFunderDromeBaseMode (Game|GetGameMode)))
  (Default|CallNameUpdate _asfunder_drome_base_mode _output_get controllerRef)
  (Development|PrintString (Variables|Default|GetDisplayName)))

(event EventBeginPlay
  (CallFunction|AquireName))

(event EventTick
  (params (DeltaSeconds :type Float%20%28single-precision%29)))

(fn ConstructionScript)
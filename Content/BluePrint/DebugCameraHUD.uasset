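; Debug HUD for a car that draws motion vectors and per-wheel readouts on screen.
; CarIndication stores forward speed and scaled forward, velocity and force vectors, drawn as colored lines from screen center.
; UpdateNumber caches three values and a screen position per wheel, drawn as stacked text tinted green to red by the first value.
; FR and RL second and third values draw at each other's positions, and RR3's input overwrites RR2.
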(event Custom|CarIndication
  (params (Velocity :type Vector%202D%20Structure) (force :type Vector%202D%20Structure) (Forward :type Vector%202D%20Structure) (FVelocity :type Float%20%28single-precision%29))
  (bind _data (Variables|Default|GetData))
  (Variables|Default|SetForwardVelocity FVelocity)
  (Utilities|Array|SetArrayElem _data 0 (* Forward 1e+02))
  (Utilities|Array|SetArrayElem _data 1 (/ Velocity 4e+01) true)
  (Utilities|Array|SetArrayElem _data 2 (/ force 4e+01) true))

(event Custom|UpdateNumber
  (params (FL1 :type Float%20%28single-precision%29) (FL2 :type Float%20%28single-precision%29) (FL3 :type Float%20%28single-precision%29) (FLPos :type Vector%202D%20Structure) (FR1 :type Float%20%28single-precision%29) (FR2 :type Float%20%28single-precision%29) (FR3 :type Float%20%28single-precision%29) (FRPos :type Vector%202D%20Structure) (RL1 :type Float%20%28single-precision%29) (RL2 :type Float%20%28single-precision%29) (RL3 :type Float%20%28single-precision%29) (RLPos :type Vector%202D%20Structure) (RR1 :type Float%20%28single-precision%29) (RR2 :type Float%20%28single-precision%29) (RR3 :type Float%20%28single-precision%29) (RRPos :type Vector%202D%20Structure))
  (Variables|Default|SetFL1 FL1)
  (Variables|Default|SetFL2 FL2)
  (Variables|Default|SetFL3 FL3)
  (Variables|Default|SetFLPos FLPos)
  (Variables|Default|SetFR1 FR1)
  (Variables|Default|SetFR2 FR2)
  (Variables|Default|SetFR3 FR3)
  (Variables|Default|SetFRPos FRPos)
  (Variables|Default|SetRL1 RL1)
  (Variables|Default|SetRL2 RL2)
  (Variables|Default|SetRL3 RL3)
  (Variables|Default|SetRLPos RLPos)
  (Variables|Default|SetRR1 RR1)
  (Variables|Default|SetRR2 RR2)
  (Variables|Default|SetRR2 RR3)
  (Variables|Default|SetRRPos RRPos))

(event EventBeginPlay)

(event EventActorBeginOverlap
  (params (OtherActor :type Actor%20Object%20Reference)))

(event EventTick
  (params (DeltaSeconds :type Float%20%28single-precision%29)))

(event EventDrawHUD
  (params (SizeX :type Integer) (SizeY :type Integer))
  (bind _fl1 (Variables|Default|GetFL1))
  (bind _fr1 (Variables|Default|GetFR1))
  (bind _rl1 (Variables|Default|GetRL1))
  (bind _rr1 (Variables|Default|GetRR1))
  (bind _flpos (Variables|Default|GetFLPos))
  (bind _frpos (Variables|Default|GetFRPos))
  (bind _rlpos (Variables|Default|GetRLPos))
  (bind _rrpos (Variables|Default|GetRRPos))
  (bind _data (Variables|Default|GetData))
  (bind _returnvalue (Math|Color|Lerp(LinearColor) "(R=0.000000,G=1.000000,B=0.000000,A=1.000000)" "(R=1.000000,G=0.000000,B=0.000000,A=1.000000)" _fl1))
  (bind _returnvalue_2 (Math|Color|Lerp(LinearColor) "(R=0.000000,G=1.000000,B=0.000000,A=1.000000)" "(R=1.000000,G=0.000000,B=0.000000,A=1.000000)" _fr1))
  (bind _returnvalue_3 (Math|Color|Lerp(LinearColor) "(R=0.000000,G=1.000000,B=0.000000,A=1.000000)" "(R=1.000000,G=0.000000,B=0.000000,A=1.000000)" _rl1))
  (bind _returnvalue_4 (Math|Color|Lerp(LinearColor) "(R=0.000000,G=1.000000,B=0.000000,A=1.000000)" "(R=1.000000,G=0.000000,B=0.000000,A=1.000000)" _rr1))
  (bind _output_get (Variables|Default|SetScreenCenter (Math|Vector2D|MakeVector2D (Math|Conversions|ToFloat(Integer) (/ SizeX 2)) (Math|Conversions|ToFloat(Integer) (/ SizeY 2)))))
  (Class|HUD|DrawLine (.X (Math|Vector2D|BreakVector2D _output_get)) (.Y (Math|Vector2D|BreakVector2D _output_get)) (.x (+ _output_get (Utilities|Array|Get(acopy) _data))) (.y (+ _output_get (Utilities|Array|Get(acopy) _data))) "(R=1.000000,G=1.000000,B=0.000000,A=1.000000)" 0.0)
  (Class|HUD|DrawLine (.X (Math|Vector2D|BreakVector2D _output_get)) (.Y (Math|Vector2D|BreakVector2D _output_get)) (.x (+ _output_get (Utilities|Array|Get(acopy) _data 1))) (.y (+ _output_get (Utilities|Array|Get(acopy) _data 1))) "(R=1.000000,G=0.000000,B=0.000000,A=1.000000)" 0.0)
  (Class|HUD|DrawLine (.X (Math|Vector2D|BreakVector2D _output_get)) (.Y (Math|Vector2D|BreakVector2D _output_get)) (.x (+ _output_get (Utilities|Array|Get(acopy) _data 2))) (.y (+ _output_get (Utilities|Array|Get(acopy) _data 2))) "(R=0.000000,G=1.000000,B=0.000000,A=1.000000)" 0.0)
  (HUD|DrawText (Utilities|String|ToString(Float) (Variables|Default|GetForwardVelocity)) "(R=1.000000,G=0.000000,B=0.129783,A=1.000000)" (.X (Math|Vector2D|BreakVector2D _output_get)) (.Y (Math|Vector2D|BreakVector2D _output_get)) 0 1.0 false)
  (HUD|DrawText (Utilities|String|ToString(Text) (Utilities|Text|ToText(Float) _fl1 "HalfToEven" false 1 324 0 2)) _returnvalue (.x _flpos) (.y _flpos) 0 1.0 false)
  (HUD|DrawText (Utilities|String|ToString(Text) (Utilities|Text|ToText(Float) (Variables|Default|GetFL2) "HalfToEven" false 1 324 0 2)) _returnvalue (.x _flpos) (+ (.y _flpos) 11.0) 0 1.0 false)
  (HUD|DrawText (Utilities|String|ToString(Text) (Utilities|Text|ToText(Float) (Variables|Default|GetFL3) "HalfToEven" false 1 324 0 2)) _returnvalue (.x _flpos) (+ (.y _flpos) 22.0) 0 1.0 false)
  (HUD|DrawText (Utilities|String|ToString(Text) (Utilities|Text|ToText(Float) _fr1 "HalfToEven" false 1 324 0 2)) _returnvalue_2 (.x _frpos) (.y _frpos) 0 1.0 false)
  (HUD|DrawText (Utilities|String|ToString(Text) (Utilities|Text|ToText(Float) (Variables|Default|GetRL2) "HalfToEven" false 1 324 0 2)) _returnvalue_2 (.x _frpos) (+ (.y _frpos) 11.0) 0 1.0 false)
  (HUD|DrawText (Utilities|String|ToString(Text) (Utilities|Text|ToText(Float) (Variables|Default|GetRL3) "HalfToEven" false 1 324 0 2)) _returnvalue_2 (.x _frpos) (+ (.y _frpos) 22.0) 0 1.0 false)
  (HUD|DrawText (Utilities|String|ToString(Text) (Utilities|Text|ToText(Float) _rl1 "HalfToEven" false 1 324 0 2)) _returnvalue_3 (.x _rlpos) (.y _rlpos) 0 1.0 false)
  (HUD|DrawText (Utilities|String|ToString(Text) (Utilities|Text|ToText(Float) (Variables|Default|GetFR2) "HalfToEven" false 1 324 0 2)) _returnvalue_3 (.x _rlpos) (+ (.y _rlpos) 11.0) 0 1.0 false)
  (HUD|DrawText (Utilities|String|ToString(Text) (Utilities|Text|ToText(Float) (Variables|Default|GetFR3) "HalfToEven" false 1 324 0 2)) _returnvalue_3 (.x _rlpos) (+ (.y _rlpos) 22.0) 0 1.0 false)
  (HUD|DrawText (Utilities|String|ToString(Text) (Utilities|Text|ToText(Float) _rr1 "HalfToEven" false 1 324 0 2)) _returnvalue_4 (.x _rrpos) (.y _rrpos) 0 1.0 false)
  (HUD|DrawText (Utilities|String|ToString(Text) (Utilities|Text|ToText(Float) (Variables|Default|GetRR2) "HalfToEven" false 1 324 0 2)) _returnvalue_4 (.x _rrpos) (+ (.y _rrpos) 11.0) 0 1.0 false)
  (HUD|DrawText (Utilities|String|ToString(Text) (Utilities|Text|ToText(Float) (Variables|Default|GetRR3) "HalfToEven" false 1 324 0 2)) _returnvalue_4 (.x _rrpos) (+ (.y _rrpos) 22.0) 0 1.0 false))

(fn ConstructionScript)
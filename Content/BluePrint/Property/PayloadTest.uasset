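; Payload actor for the FunderDrome payload mode that travels along a path's spline once set up and started.
; Tick advances it by speed along the spline, while its kill zone damages overlapping actors tagged Vehicle.
; While moving, damage instigated by team 2 turrets sets health to damage minus current health and reports it to the game mode.
; At zero or below, it ends the match for team 2.
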(event OnComponentBeginOverlap(Killzone)
  (params (OverlappedComponent :type Primitive%20Component%20Object%20Reference) (OtherActor :type Actor%20Object%20Reference) (OtherComp :type Primitive%20Component%20Object%20Reference) (OtherBodyIndex :type Integer) (bFromSweep :type Boolean) (SweepResult :type Hit%20Result%20Structure%20%28by%20ref%29))
  (if (Actor|ActorHasTag OtherActor "Vehicle")
    (Game|Damage|ApplyDamage OtherActor (Variables|Default|GetCoolDamage) 0 0)))

(event Custom|PayloadSetup
  (params (Path :type Payload%20Move%20Node%20Object%20Reference))
  (bind _output_get (Variables|Default|SetMovepath Path))
  (Variables|Default|SetPathLength (Spline|GetSplineLength (Variables|/Game/BluePrint/Property/PayloadMoveNode.PayloadMoveNode_C|GetSpline _output_get)))
  (Transformation|SetWorldTransform (Variables|Default|GetScene) (Math|Transform|MakeTransform (Spline|GetLocationatDistanceAlongSpline (Variables|/Game/BluePrint/Property/PayloadMoveNode.PayloadMoveNode_C|GetSpline _output_get) 0.0 "World") (Spline|GetRotationatDistanceAlongSpline (Variables|/Game/BluePrint/Property/PayloadMoveNode.PayloadMoveNode_C|GetSpline _output_get) 0.0 "World")) false false)
  (Variables|Default|SetHealth (Variables|Default|GetMaxHealth))
  (Variables|Default|SetMoving false)
  (Variables|Default|SetReady true))

(event Custom|StartMoving
  (Variables|Default|SetMoving true))

(event EventBeginPlay
  (bind _asfunder_drome_payload_mode (Utilities|Casting|CastToFunderDromePayloadMode (Game|GetGameMode)))
  (Variables|Default|SetGamemodeRef _asfunder_drome_payload_mode))

(event Collision|EventActorBeginOverlap
  (params (OtherActor :type Actor%20Object%20Reference)))

(event EventTick
  (params (DeltaSeconds :type Float%20%28single-precision%29))
  (bind _movepath (Variables|Default|GetMovepath))
  (bind _spline (Variables|/Game/BluePrint/Property/PayloadMoveNode.PayloadMoveNode_C|GetSpline _movepath))
  (if (and (Variables|Default|GetReady) (Variables|Default|GetMoving))
    (Variables|Default|SetMovedDistance (+ (* DeltaSeconds (Variables|Default|GetMovementSpeed)) (Variables|Default|GetMovedDistance)))
    (Transformation|SetWorldTransform (Variables|Default|GetScene) (Math|Transform|MakeTransform (Spline|GetLocationatDistanceAlongSpline _spline (Variables|Default|GetMovedDistance) "World") (Spline|GetRotationatDistanceAlongSpline _spline (Variables|Default|GetMovedDistance) "World")) false false)))

(event Game|Damage|EventAnyDamage
  (params (Damage :type Float%20%28single-precision%29) (DamageType :type Damage%20Type%20Object%20Reference) (InstigatedBy :type Controller%20Object%20Reference) (DamageCauser :type Actor%20Object%20Reference))
  (if (and (Variables|Default|GetReady) (Variables|Default|GetMoving))
    (bind _asfunder_drome_turret_base (Utilities|Casting|CastToFunderDromeTurretBase (Game|GetInstigator DamageCauser)))
    (if (== (Variables|/Game/BluePrint/Turret/FunderDromeTurretBase.FunderDromeTurretBase_C|GetTeam _asfunder_drome_turret_base) 2)
      (bind _output_get (Variables|Default|SetHealth (- Damage (Variables|Default|GetHealth))))
      (Default|PayloadUpdateHealth (Variables|Default|GetGamemodeRef) _output_get)
      (if (<= _output_get 0.0)
        (Default|EndOfMatch (Variables|Default|GetGamemodeRef) 2 (Transformation|GetActorLocation))))))

(fn ConstructionScript)
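; Air drop pickup actor that grants either health or one of three weapons (Grenade Launcher, Plasma Gun, Railgun) to cars.
; BeginPlay shows the matching mesh, while Tick bobs it on a sine wave, spins it and counts down to self-destruction.
; Overlap with a FunderDromeCarBase calls its WeaponPickup and destroys the actor, but health is only taken below max.
; Disconnected FunderDromeVehicle nodes remain unused.
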(event Collision|EventActorBeginOverlap
  (params (OtherActor :type Actor%20Object%20Reference))
  (bind _ishealthpickup (Variables|Default|GetIsHealthPickup))
  (bind _asfunder_drome_car_base (Utilities|Casting|CastToFunderDromeCarBase OtherActor))
  (if _ishealthpickup
    (if (< (Variables|/Game/TestCar/BP/FunderDromeCarBase.FunderDromeCarBase_C|GetHealth _asfunder_drome_car_base) (Variables|/Game/TestCar/BP/FunderDromeCarBase.FunderDromeCarBase_C|GetMaxHealth _asfunder_drome_car_base))
      (Default|WeaponPickup _asfunder_drome_car_base (Variables|Default|GetWeaponType) _ishealthpickup (Variables|Default|GetPickUpHealth) (Transformation|GetActorLocation) :!label _label)
      (Actor|DestroyActor))
    (else
      (goto _label))))

(event EventBeginPlay
  (if (Variables|Default|GetIsHealthPickup)
    (Rendering|SetVisibility (Variables|Default|GetHealthPick) true true)
    (else
      (switch Utilities|FlowControl|Switch|SwitchonDuke_WeaponType (Variables|Default|GetWeaponType)
        (:NewEnumerator1
          (Rendering|SetVisibility (Variables|Default|GetGrenadePick) true true))
        (:NewEnumerator2
          (Rendering|SetVisibility (Variables|Default|GetPlasmaPick) true true))
        (:NewEnumerator3
          (Rendering|SetVisibility (Variables|Default|GetRailPick) true true))))))

(event EventTick
  (params (DeltaSeconds :type Float%20%28single-precision%29))
  (bind _animoffest (Variables|Default|GetanimOffest))
  (Utilities|FlowControl|Sequence
    (:then_0
      (Variables|Default|SetAnimTimer (.Remainder (Math|Float|Division(WholeandRemainder) (+ (Variables|Default|GetAnimTimer) DeltaSeconds) 3.6e+02)))
      (Transformation|SetRelativeLocation _animoffest (Math|Vector|MakeVector 0.0 0.0 (+ (* (Math|Trig|Sin(Degrees) (* (Variables|Default|GetAnimTimer) (Variables|Default|GetFloatTimerMultiplier))) (Variables|Default|GetFloatMultiplier)) (Variables|Default|GetFloatOffset))) false false)
      (Transformation|AddLocalRotation _animoffest (Math|Rotator|MakeRotator 0.0 0.0 (* DeltaSeconds (Variables|Default|GetRotMultiplier))) false false))
    (:then_1
      (bind _output_get (Variables|Default|SetDestroyTimer (- (Variables|Default|GetDestroyTimer) DeltaSeconds)))
      (if (<= _output_get 0.0)
        (Actor|DestroyActor)))))

(fn ConstructionScript)
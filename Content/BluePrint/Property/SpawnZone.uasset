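; SpawnZone is a spawn area for FunderDrome cars that tracks whether it is available.
; On the server, a two-second looping timer marks it unavailable while any FunderDromeCarBase overlaps its sphere, regardless of team.
; The construction script sizes the sphere from Range and gathers nine start references into Starts.
; An overlap-counting variant that filters by opposing team remains in the graph, disconnected.
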(event OnComponentBeginOverlap(Sphere)
  (params (OverlappedComponent :type Primitive%20Component%20Object%20Reference) (OtherActor :type Actor%20Object%20Reference) (OtherComp :type Primitive%20Component%20Object%20Reference) (OtherBodyIndex :type Integer) (bFromSweep :type Boolean) (SweepResult :type Hit%20Result%20Structure%20%28by%20ref%29)))

(event OnComponentEndOverlap(Sphere)
  (params (OverlappedComponent :type Primitive%20Component%20Object%20Reference) (OtherActor :type Actor%20Object%20Reference) (OtherComp :type Primitive%20Component%20Object%20Reference) (OtherBodyIndex :type Integer)))

(event Custom|checkoverlap
  (Variables|Default|Setavailable (not (> (Utilities|Array|Length (Collision|GetOverlappingActors (Variables|Default|GetSphere) "/Game/TestCar/BP/FunderDromeCarBase.FunderDromeCarBase_C" :!class /Script/Engine.PrimitiveComponent)) 0))))

(event EventBeginPlay
  (if (Networking|IsServer)
    (Utilities|Time|SetTimerbyEvent (delegate Custom|checkoverlap) 2.0 true)))

(event Collision|EventActorBeginOverlap
  (params (OtherActor :type Actor%20Object%20Reference)))

(event EventTick
  (params (DeltaSeconds :type Float%20%28single-precision%29)))

(fn ConstructionScript
  (Components|Sphere|SetSphereRadius (Variables|Default|GetSphere) (Variables|Default|Getrange) false)
  (Variables|Default|SetStarts (Utilities|Array|MakeArray (Variables|Default|Getstart1) (Variables|Default|Getstart2) (Variables|Default|Getstart3) (Variables|Default|Getstart4) (Variables|Default|Getstart5) (Variables|Default|Getstart6) (Variables|Default|Getstart7) (Variables|Default|Getstart8) (Variables|Default|Getstart9))))
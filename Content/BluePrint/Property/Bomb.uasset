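; Bomb actor, apparently a tug-of-war objective that damage pushes along the line between Red and Blue bases.
; UpdatePosition shifts it by clamped accumulated damage, then resets the total and records its offset from Blue's edge.
; Base setup, damage tallying, timers and server-physics sync with velocity extrapolation are all disconnected.
; BeginPlay, Hit and RadialDamage are empty, Tick only stores delta time, and SyncData copies Data and flags it dirty.
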(event Custom|SyncLocation
  (Variables|Default|SetDirty true))

(event Custom|SyncData
  (Variables|Default|SetServerData (Variables|Default|GetData))
  (CallFunction|SyncLocation))

(event Custom|UpdatePosition
  (bind _returnvalue (Transformation|GetActorLocation))
  (bind _bluesideedge (Variables|Default|GetBlueSideEdge))
  (Transformation|AddActorWorldOffset (* (/ (Variables|Default|GetBaseDistance) 1e+02) (Math|Float|Clamp(Float) (/ (Variables|Default|GetDamageThisTick) 1.4e+04) -0.5 0.5)))
  (Variables|Default|SetCurrent%20distance (- (Math|Vector|MakeVector (.x _returnvalue) (.y _returnvalue) 0.0) (Math|Vector|MakeVector (.x _bluesideedge) (.y _bluesideedge) 0.0)))
  (Variables|Default|SetDamageThisTick 0.0))

(event EventBeginPlay)

(event EventActorBeginOverlap
  (params (OtherActor :type Actor%20Object%20Reference)))

(event EventTick
  (params (DeltaSeconds :type Float%20%28single-precision%29))
  (Variables|Default|SetDeltatime DeltaSeconds))

(event Collision|EventHit
  (params (MyComp :type Primitive%20Component%20Object%20Reference) (Other :type Actor%20Object%20Reference) (OtherComp :type Primitive%20Component%20Object%20Reference) (bSelfMoved :type Boolean) (HitLocation :type Vector :default "0, 0, 0") (HitNormal :type Vector :default "0, 0, 0") (NormalImpulse :type Vector :default "0, 0, 0") (Hit :type Hit%20Result%20Structure%20%28by%20ref%29)))

(event Game|Damage|EventRadialDamage
  (params (DamageReceived :type Float%20%28single-precision%29) (DamageType :type Damage%20Type%20Object%20Reference) (Origin :type Vector :default "0, 0, 0") (HitInfo :type Hit%20Result%20Structure%20%28by%20ref%29) (InstigatedBy :type Controller%20Object%20Reference) (DamageCauser :type Actor%20Object%20Reference)))

(fn ConstructionScript)
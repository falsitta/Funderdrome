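; NavNodeBP is a hand-placed navigation node that links to other nodes under a shared NavManager.
; Its construction script finds the manager if unset, snaps the node to ground with a vertical trace, flags an error on a miss, then has the manager redraw links.
; DrawDebugLine builds line components to each linked node, and UpdateMap shows the floored Dist value as text.
; Tick is disabled at BeginPlay.
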(event EventBeginPlay
  (Actor|Tick|SetActorTickEnabled false))

(event Collision|EventActorBeginOverlap
  (params (OtherActor :type Actor%20Object%20Reference)))

(event EventTick
  (params (DeltaSeconds :type Float%20%28single-precision%29)))

(fn ConstructionScript
  (bind _returnvalue (Transformation|GetActorLocation))
  (bind _groundcorrection (Variables|Default|GetGroundCorrection))
  (Utilities|IsValid (Variables|Default|GetManager)
    (:Is%20Valid
      _)
    (:Is%20Not%20Valid
      (bind _outactors (Actor|GetAllActorsOfClass "/Game/BluePrint/AIScript/NavManager.NavManager_C"))
      (Variables|Default|SetManager (Utilities|Array|Get(acopy) _outactors))))
  (bind (_outhit _returnvalue_2) (Collision|LineTraceByChannel (+ _returnvalue (Math|Vector|MakeVector 0.0 0.0 _groundcorrection)) (+ _returnvalue (Math|Vector|MakeVector 0.0 0.0 (- 0.0 _groundcorrection))) "TraceTypeQuery1" false 0 "ForOneFrame" true "(R=1.000000,G=0.000000,B=0.000000,A=1.000000)" "(R=0.000000,G=1.000000,B=0.000000,A=1.000000)" 1.0))
  (if _returnvalue_2
    (Variables|Default|SetError false)
    (Transformation|SetActorLocation (.Location (Collision|BreakHitResult _outhit)) false false)
    (else
      (Variables|Default|SetError true)))
  (Default|RedrawLines (Variables|Default|GetManager)))

(fn DrawDebugLine
  (bind _groundoffset (Variables|Default|GetGroundOffset))
  (Utilities|Array|Clear (Variables|Default|GetDebugLines))
  (for _array_element (Variables|Default|GetLinkedNodes)
    (bind _returnvalue (AddComponent|AddDebugLine))
    (Variables|/Script/MyFunderDrome.DebugLine|SetStart _returnvalue (+ (Transformation|GetActorLocation _array_element) _groundoffset))
    (Variables|/Script/MyFunderDrome.DebugLine|SetEnd _returnvalue (+ (Transformation|GetActorLocation) _groundoffset))
    (Class|DebugLine|RedrawLine _returnvalue)
    (Utilities|Array|AddUnique (Variables|Default|GetDebugLines) _returnvalue)))

(fn UpdateMap
  (Rendering|Components|TextRender|SetText (Variables|Default|GetTextRender) (Utilities|Text|ToText(Integer) (Math|Float|Floor (Variables|Default|GetDist)))))
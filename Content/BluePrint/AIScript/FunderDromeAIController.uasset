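; Server-side AI controller for FunderDrome payload, car and turret pawns, toggled by AIExecute and AIHalt.
; On tick it identifies its pawn once and runs the matching behavior tree, seeding the blackboard with the first waypoint for payloads or the payload actor for cars.
; For payloads and cars, three angled forward line traces then update Left, Center and Right obstacle flags against static geometry each tick.
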(event Custom|AIExecute
  (Variables|Default|SetAIStart true))

(event Custom|AIHalt
  (Variables|Default|SetAIStart false))

(event EventBeginPlay
  (Networking|SwitchHasAuthority
    (:Authority
      (Actor|Tick|SetActorTickEnabled true))))

(event EventTick
  (params (DeltaSeconds :type Float%20%28single-precision%29))
  (bind _returnvalue (AI|GetBlackboard 0))
  (bind _returnvalue_2 (Pawn|GetControlledPawn))
  (bind _array (Utilities|Array|MakeArray "ObjectTypeQuery1"))
  (bind _detectlength (Variables|Default|GetDetectLength))
  (Networking|SwitchHasAuthority
    (:Authority
      (if (Variables|Default|GetAIStart)
        (if (Variables|Default|GetPawnSet)
          (if (Variables|Default|GetIsCar&Ready)
            (Utilities|IsValid (Variables|Default|GetPawnRef)
              (:Is%20Valid
                (bind _returnvalue_3 (Collision|LineTraceForObjects (+ (Transformation|GetActorLocation (Variables|Default|GetPawnRef)) (* (Transformation|GetActorUpVector (Variables|Default|GetPawnRef)) (Variables|Default|GetUpOffset))) (+ (+ (Transformation|GetActorLocation (Variables|Default|GetPawnRef)) (* (Transformation|GetActorUpVector (Variables|Default|GetPawnRef)) (Variables|Default|GetUpOffset))) (* (Math|Vector|RotateVectorAroundAxis (Transformation|GetActorForwardVector (Variables|Default|GetPawnRef)) -3e+01 (Transformation|GetActorUpVector (Variables|Default|GetPawnRef))) _detectlength) (* (Transformation|GetActorUpVector (Variables|Default|GetPawnRef)) (Variables|Default|GetUpOffset))) _array false 0 "ForOneFrame"))
                (Variables|Default|SetLeft _returnvalue_3)
                (bind _returnvalue_4 (Collision|LineTraceForObjects (+ (Transformation|GetActorLocation (Variables|Default|GetPawnRef)) (* (Transformation|GetActorUpVector (Variables|Default|GetPawnRef)) (Variables|Default|GetUpOffset))) (+ (+ (Transformation|GetActorLocation (Variables|Default|GetPawnRef)) (* (Transformation|GetActorUpVector (Variables|Default|GetPawnRef)) (Variables|Default|GetUpOffset))) (* (Transformation|GetActorForwardVector (Variables|Default|GetPawnRef)) _detectlength) (* (Transformation|GetActorUpVector (Variables|Default|GetPawnRef)) (Variables|Default|GetUpOffset))) _array false 0 "ForOneFrame"))
                (Variables|Default|SetCenter _returnvalue_4)
                (bind _returnvalue_5 (Collision|LineTraceForObjects (+ (Transformation|GetActorLocation (Variables|Default|GetPawnRef)) (* (Transformation|GetActorUpVector (Variables|Default|GetPawnRef)) (Variables|Default|GetUpOffset))) (+ (+ (Transformation|GetActorLocation (Variables|Default|GetPawnRef)) (* (Transformation|GetActorUpVector (Variables|Default|GetPawnRef)) (Variables|Default|GetUpOffset))) (* (Math|Vector|RotateVectorAroundAxis (Transformation|GetActorForwardVector (Variables|Default|GetPawnRef)) 3e+01 (Transformation|GetActorUpVector (Variables|Default|GetPawnRef))) _detectlength) (* (Transformation|GetActorUpVector (Variables|Default|GetPawnRef)) (Variables|Default|GetUpOffset))) _array false 0 "ForOneFrame"))
                (Variables|Default|SetRight _returnvalue_5))))
          (else
            (Utilities|IsValid (Variables|Default|GetPawnRef)
              (:Is%20Not%20Valid
                (bind _astest_payload_bp (Utilities|Casting|CastToTestPayloadBP _returnvalue_2)
                  (:then
                    (Variables|Default|SetPawnRef _astest_payload_bp)
                    (Variables|Default|SetPawnSet true)
                    (Variables|Default|SetIsCar&Ready true)
                    (AI|RunBehaviorTree "/Game/BluePrint/AIScript/PayloadAI.PayloadAI")
                    (bind _outactors (Actor|GetAllActorsOfClass "/Game/BluePrint/Property/PayloadMoveNode.PayloadMoveNode_C"))
                    (AI|Components|Blackboard|SetValueasObject _returnvalue (Variables|Default|GetWaypoint) (Utilities|Array|Get(acopy) _outactors))
                    (bind _loc (Default|GetNodeLoc (Utilities|Array|Get(acopy) _outactors)))
                    (AI|Components|Blackboard|SetValueasVector _returnvalue (Variables|Default|GetTargetLocation) _loc))
                  (:CastFailed
                    (bind _asfunder_drome_car_base (Utilities|Casting|CastToFunderDromeCarBase _returnvalue_2)
                      (:then
                        (Variables|Default|SetPawnRef _asfunder_drome_car_base)
                        (Variables|Default|SetPawnSet true)
                        (Variables|Default|SetIsCar&Ready true)
                        (AI|RunBehaviorTree "/Game/BluePrint/AIScript/CarAI.CarAI")
                        (bind _outactors_2 (Actor|GetAllActorsOfClass "/Game/TestCar/BP/TestPayloadBP.TestPayloadBP_C"))
                        (AI|Components|Blackboard|SetValueasObject _returnvalue (Variables|Default|GetPayload) (Utilities|Array|Get(acopy) _outactors_2)))
                      (:CastFailed
                        (bind _asfunder_drome_turret_base (Utilities|Casting|CastToFunderDromeTurretBase _returnvalue_2))
                        (Variables|Default|SetPawnRef _asfunder_drome_turret_base)
                        (Variables|Default|SetPawnSet true)
                        (AI|RunBehaviorTree "/Game/BluePrint/AIScript/GunnerAI.GunnerAI")))))))))))))

(fn ConstructionScript)
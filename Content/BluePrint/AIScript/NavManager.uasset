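; Server-only navigation manager that computes waypoint paths from requesting controllers to the level's CenterPoint; on clients it destroys itself and all NavNodeBP actors.
; LinkNavPoints connects nodes within range and clear line of sight, at BeginPlay or via the construction-script Link toggle.
; FindRoute runs an A*-like best-first search scored by step distance plus Manhattan distance to target, without accumulated cost.
; Requests arriving while busy are queued and served by a looping timer.
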(event Custom|RequestPath
  (params (Cointroller :type Funder%20Drome%20AI%20Controller%20Object%20Reference))
  (if (Variables|Default|GetBusy)
    (Utilities|Array|Add (Variables|Default|GetControllers) Cointroller)
    (else
      (CallFunction|GivePath Cointroller))))

(event Custom|GivePath
  (params (Controller%20Ref :type Funder%20Drome%20AI%20Controller%20Object%20Reference))
  (bind _returnvalue (Transformation|GetActorLocation Controller%20Ref))
  (bind _centerpoint (Variables|Default|GetCenterPoint))
  (bind _returnvalue_2 (Transformation|GetActorLocation _centerpoint))
  (bind (_newpath _error) (CallFunction|FindRoute _returnvalue _returnvalue_2))
  (Variables|Default|SetBusy true)
  (Default|UpdatePath Controller%20Ref _error _newpath))

(event Custom|CheckQueue
  (bind _controllers (Variables|Default|GetControllers))
  (if (and (> (Utilities|Array|Length (Variables|Default|GetControllers)) 0) (not (Variables|Default|GetBusy)))
    (CallFunction|GivePath (Utilities|Array|Get(acopy) _controllers))
    (Utilities|Array|RemoveIndex _controllers)))

(event EventBeginPlay
  (if (Networking|IsServer)
    (bind _outactors (Actor|GetAllActorsOfClass "/Game/BluePrint/AIScript/centerPoint.centerPoint_C"))
    (Variables|Default|SetCenterPoint (Utilities|Array|Get(acopy) _outactors))
    (CallFunction|LinkNavPoints)
    (Utilities|Time|SetTimerbyEvent (delegate Custom|CheckQueue) 0.5 true)
    (else
      ;[1 1 1] Destroy all evidence!!!
      (bind _outactors_2 (Actor|GetAllActorsOfClass "/Game/BluePrint/AIScript/NavNodeBP.NavNodeBP_C"))
      (for _array_element _outactors_2
        (Actor|DestroyActor _array_element))
      (Actor|DestroyActor))))

(event Collision|EventActorBeginOverlap
  (params (OtherActor :type Actor%20Object%20Reference)))

(event EventTick
  (params (DeltaSeconds :type Float%20%28single-precision%29)))

(fn ConstructionScript
  (if (Variables|Default|Getlink)
    (Variables|Default|Setlink false)
    (CallFunction|LinkNavPoints)
    (else
      (CallFunction|RedrawLines))))

(fn LinkNavPoints
  (bind _outactors (Actor|GetAllActorsOfClass "/Game/BluePrint/AIScript/NavNodeBP.NavNodeBP_C"))
  (bind _output_get (Variables|Default|SetNode _outactors))
  (for (_array_element _array_index) _output_get
    (Variables|/Game/BluePrint/AIScript/NavNodeBP.NavNodeBP_C|SetGroundCorrection _array_element (Variables|Default|GetGroundCorrectionDist))
    (Variables|/Game/BluePrint/AIScript/NavNodeBP.NavNodeBP_C|SetGroundOffset _array_element (Variables|Default|GetGroundOffset))
    (Utilities|Array|Clear (Variables|/Game/BluePrint/AIScript/NavNodeBP.NavNodeBP_C|GetLinkedNodes _array_element))
    (LocalVariables|SetCNode _array_index)
    (Variables|Default|SetCLoc (Transformation|GetActorLocation _array_element))
    (for _array_element_2 (Variables|Default|GetNode)
      (if (!= _array_element_2 (Utilities|Array|Get(acopy) (Variables|Default|GetNode) (LocalVariables|GetCNode)))
        (if (< (Math|Vector|VectorLength (- (Transformation|GetActorLocation _array_element_2) (Variables|Default|GetCLoc))) (Variables|Default|GetLinkDist))
          (bind _returnvalue (Collision|LineTraceByChannel (+ (Transformation|GetActorLocation _array_element_2) (Variables|Default|GetGroundOffset)) (+ (Variables|Default|GetGroundOffset) (Variables|Default|GetCLoc)) "TraceTypeQuery1" false 0 "ForOneFrame" true "(R=1.000000,G=0.000000,B=0.000000,A=1.000000)" "(R=0.000000,G=1.000000,B=0.000000,A=1.000000)" 2.0))
          (if (not _returnvalue)
            (Utilities|Array|AddUnique (Variables|/Game/BluePrint/AIScript/NavNodeBP.NavNodeBP_C|GetLinkedNodes (Utilities|Array|Get(acopy) (Variables|Default|GetNode) (LocalVariables|GetCNode))) _array_element_2))))))
  (CallFunction|RedrawLines))

(fn FindRoute
  (params (CurrentLoc :type Vector) (TargetLoc :type Vector))
  (bind _visitedlist (LocalVariables|GetVisitedList))
  (bind _openlist (LocalVariables|GetOpenList))
  (bind _openlist_2 (LocalVariables|GetOpenList))
  (bind _path (LocalVariables|GetPath))
  (bind _openlist_3 (LocalVariables|GetOpenList))
  (bind _visitedlist_2 (LocalVariables|GetVisitedList))
  (bind _path_2 (LocalVariables|GetPath))
  (bind _path_3 (LocalVariables|GetPath))
  ;[1 1 1] Cache Everything
  (LocalVariables|SetStartLoc CurrentLoc)
  (LocalVariables|SetTarget TargetLoc)
  (LocalVariables|SetStart (.NodeIndex (CallFunction|GetClosetPoint CurrentLoc)))
  (LocalVariables|SetEnd (.NodeIndex (CallFunction|GetClosetPoint TargetLoc)))
  ;[1 1 1] First Link
  (Utilities|Array|Clear _path_2)
  (Utilities|Array|Add _path_2 (LocalVariables|GetStartLoc))
  (Utilities|Array|Add _path_2 (Transformation|GetActorLocation (Utilities|Array|Get(acopy) (Variables|Default|GetNode) (LocalVariables|GetStart))))
  (Utilities|Array|Clear (LocalVariables|GetVisitedList))
  (Utilities|Array|Clear (LocalVariables|GetOpenList))
  (LocalVariables|SetNextStep (LocalVariables|GetStart))
  (LocalVariables|SetNotFinish true)
  (Utilities|Array|Add (LocalVariables|GetOpenList) (Utilities|Struct|MakeNavPoint (LocalVariables|GetNextStep) 0 (Utilities|Array|Get(acopy) (Variables|Default|GetNode) (LocalVariables|GetNextStep)) (Math|Vector|VectorLength (- (Transformation|GetActorLocation (Utilities|Array|Get(acopy) (Variables|Default|GetNode) (LocalVariables|GetNextStep))) (LocalVariables|GetTarget)))))
  (while (LocalVariables|GetNotFinish)
    (LocalVariables|SetStarterCount 0)
    (for (_array_element _array_index) _openlist
      (if (== _array_index 0)
        (LocalVariables|SetFindCost (.NavCost (Utilities|Struct|BreakNavPoint _array_element)))
        (elif (< (.NavCost (Utilities|Struct|BreakNavPoint _array_element)) (LocalVariables|GetFindCost))
          (LocalVariables|SetFindCost (.NavCost (Utilities|Struct|BreakNavPoint _array_element)))
          (LocalVariables|SetStarterCount _array_index))))
    (bind _returnvalue (Utilities|Array|AddUnique _visitedlist_2 (Utilities|Array|Get(acopy) _openlist (LocalVariables|GetStarterCount))))
    (Utilities|Array|RemoveIndex _openlist (LocalVariables|GetStarterCount))
    (bind _output_get (LocalVariables|SetCSelfNode (.Self (Utilities|Struct|BreakNavPoint (Utilities|Array|Get(acopy) _visitedlist_2 _returnvalue)))))
    (for _array_element_2 (Variables|/Game/BluePrint/AIScript/NavNodeBP.NavNodeBP_C|GetLinkedNodes _output_get)
      (LocalVariables|SetCLinkNode _array_element_2)
      (LocalVariables|SetContains false)
      (bind _array_element_3 (Utilities|Array|ForEachLoopwithBreak (LocalVariables|GetVisitedList) :!label _label)
        (:LoopBody
          (if (== (.Self (Utilities|Struct|BreakNavPoint _array_element_3)) (LocalVariables|GetCLinkNode))
            (LocalVariables|SetContains true)
            (goto _label Break)))
        (:Completed
          (if (not (LocalVariables|GetContains))
            (bind (_array_element_4 _array_index_2) (Utilities|Array|ForEachLoopwithBreak (LocalVariables|GetOpenList) :!label _label_2)
              (:LoopBody
                (if (== (.Self (Utilities|Struct|BreakNavPoint _array_element_4)) (LocalVariables|GetCLinkNode))
                  (LocalVariables|SetFinder _array_index_2)
                  (LocalVariables|SetContains true)
                  (goto _label_2 Break)))
              (:Completed
                (if (LocalVariables|GetContains)
                  (if (< (+ (Transformation|GetDistanceTo (LocalVariables|GetCLinkNode) (LocalVariables|GetCSelfNode)) (+ (Math|Float|Absolute(Float) (.X (Math|Vector|BreakVector (- (Transformation|GetActorLocation (LocalVariables|GetCLinkNode)) (LocalVariables|GetTarget))))) (Math|Float|Absolute(Float) (.Y (Math|Vector|BreakVector (- (Transformation|GetActorLocation (LocalVariables|GetCLinkNode)) (LocalVariables|GetTarget))))) (Math|Float|Absolute(Float) (.Z (Math|Vector|BreakVector (- (Transformation|GetActorLocation (LocalVariables|GetCLinkNode)) (LocalVariables|GetTarget))))))) (.NavCost (Utilities|Struct|BreakNavPoint (Utilities|Array|Get(acopy) _openlist_2 (LocalVariables|GetFinder)))))
                    (bind _structout (Utilities|Struct|SetmembersinNavPoint (Utilities|Array|Get(acopy) _openlist_2 (LocalVariables|GetFinder)) (Utilities|Array|FindItem (Variables|Default|GetNode) (LocalVariables|GetCLinkNode)) (LocalVariables|GetCSelfNode) (LocalVariables|GetCLinkNode) (+ (Transformation|GetDistanceTo (LocalVariables|GetCLinkNode) (LocalVariables|GetCSelfNode)) (+ (Math|Float|Absolute(Float) (.X (Math|Vector|BreakVector (- (Transformation|GetActorLocation (LocalVariables|GetCLinkNode)) (LocalVariables|GetTarget))))) (Math|Float|Absolute(Float) (.Y (Math|Vector|BreakVector (- (Transformation|GetActorLocation (LocalVariables|GetCLinkNode)) (LocalVariables|GetTarget))))) (Math|Float|Absolute(Float) (.Z (Math|Vector|BreakVector (- (Transformation|GetActorLocation (LocalVariables|GetCLinkNode)) (LocalVariables|GetTarget)))))))))
                    (Utilities|Array|SetArrayElem _openlist_2 (LocalVariables|GetFinder) _structout))
                  (else
                    (Utilities|Array|Add _openlist_2 (Utilities|Struct|MakeNavPoint (Utilities|Array|FindItem (Variables|Default|GetNode) (LocalVariables|GetCLinkNode)) (LocalVariables|GetCSelfNode) (LocalVariables|GetCLinkNode) (+ (Transformation|GetDistanceTo (LocalVariables|GetCLinkNode) (LocalVariables|GetCSelfNode)) (+ (Math|Float|Absolute(Float) (.X (Math|Vector|BreakVector (- (Transformation|GetActorLocation (LocalVariables|GetCLinkNode)) (LocalVariables|GetTarget))))) (Math|Float|Absolute(Float) (.Y (Math|Vector|BreakVector (- (Transformation|GetActorLocation (LocalVariables|GetCLinkNode)) (LocalVariables|GetTarget))))) (Math|Float|Absolute(Float) (.Z (Math|Vector|BreakVector (- (Transformation|GetActorLocation (LocalVariables|GetCLinkNode)) (LocalVariables|GetTarget)))))))))))))))))
    (if (== (Utilities|Array|Length _openlist_3) 0)
      (LocalVariables|SetNotFinish false)
      (LocalVariables|SetPathFindError true)
      (else
        (bind _array_element_5 (Utilities|Array|ForEachLoopwithBreak _openlist_3 :!label _label_3)
          (:LoopBody
            (if (== (.Index (Utilities|Struct|BreakNavPoint _array_element_5)) (LocalVariables|GetEnd))
              (bind _returnvalue_2 (Utilities|Array|Add (LocalVariables|GetVisitedList) _array_element_5))
              (LocalVariables|SetFinder _returnvalue_2)
              (LocalVariables|SetNotFinish false)
              (goto _label_3 Break)))
          (:Completed
            (LocalVariables|SetNextStep (Utilities|Array|FindItem (Variables|Default|GetNode) (.self (Utilities|Array|Get(acopy) (LocalVariables|GetOpenList) (LocalVariables|GetStarterCount))))))))))
  (if (LocalVariables|GetPathFindError)
    (Utilities|Array|Add :TargetArray _path_3)
    (Variables|Default|SetBusy false)
    (return _path_3 true)
    (else
      (LocalVariables|SetNotFinish true)
      (while (LocalVariables|GetNotFinish)
        (if (== (.index (Utilities|Array|Get(acopy) _visitedlist (LocalVariables|GetFinder))) (LocalVariables|GetStart))
          (LocalVariables|SetNotFinish false)
          (else
            (Utilities|Array|Insert _path (Transformation|GetActorLocation (.self (Utilities|Array|Get(acopy) _visitedlist (LocalVariables|GetFinder)))) 2)
            (bind (_array_element_6 _array_index_3) (Utilities|Array|ForEachLoopwithBreak _visitedlist :!label _label_4)
              (:LoopBody
                (if (== (.Self (Utilities|Struct|BreakNavPoint _array_element_6)) (.searchparent (Utilities|Array|Get(acopy) _visitedlist (LocalVariables|GetFinder))))
                  (LocalVariables|SetFinder _array_index_3)
                  (goto _label_4 Break)))))))
      (Utilities|Array|Add _path (Transformation|GetActorLocation (Utilities|Array|Get(acopy) (Variables|Default|GetNode) (LocalVariables|GetEnd))))
      (Utilities|Array|Add _path (LocalVariables|GetTarget))
      (Variables|Default|SetBusy false)
      (return (LocalVariables|GetPath) false))))

(fn RedrawLines
  (Rendering|Debug|FlushPersistentDebugLines))

(fn GetClosetPoint
  (params (Location :type Vector))
  (LocalVariables|SetSeaarchLoc Location)
  (LocalVariables|SetCIndex 0)
  (for (_array_element _array_index) (Variables|Default|GetNode)
    (if (== _array_index 0)
      (LocalVariables|SetLength (Math|Vector|VectorLength (- (Transformation|GetActorLocation _array_element) (LocalVariables|GetSeaarchLoc))))
      (elif (<= (Math|Vector|VectorLength (- (Transformation|GetActorLocation _array_element) (LocalVariables|GetSeaarchLoc))) (LocalVariables|GetLength))
        (LocalVariables|SetLength (Math|Vector|VectorLength (- (Transformation|GetActorLocation _array_element) (LocalVariables|GetSeaarchLoc))))
        (LocalVariables|SetCIndex _array_index))))
  (return (LocalVariables|GetCIndex) (LocalVariables|GetLength)))

(fn Updatemap
  (Utilities|IsValid (Variables|Default|GetCenterPoint)
    (:Is%20Valid
      (for _array_element (Variables|Default|GetNode)
        (Variables|/Game/BluePrint/AIScript/NavNodeBP.NavNodeBP_C|SetDist _array_element (Transformation|GetDistanceTo _array_element (Variables|Default|GetCenterPoint)))
        (Default|UpdateMap _array_element)))))
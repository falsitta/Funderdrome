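; Behavior tree task that picks a FunderDrome turret's target and stops its firing when it runs.
; Team 2 turrets use a random, looping MultiGate to pick either the first payload actor or the closest enemy car; other teams always seek the car.
; The car search scans all car actors for the nearest opposing one within a maximum distance.
; Results go to the Target and HaveTarget blackboard keys, and the task always succeeds.
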(event EventReceiveExecuteAI
  (params (OwnerController :type AI%20Controller%20Object%20Reference) (ControlledPawn :type Pawn%20Object%20Reference))
  (bind _asfunder_drome_turret_base (Utilities|Casting|CastToFunderDromeTurretBase ControlledPawn))
  (Variables|/Game/BluePrint/Turret/FunderDromeTurretBase.FunderDromeTurretBase_C|SetFireing _asfunder_drome_turret_base false)
  (Variables|Default|SetDist 1e+05)
  (if (== (Variables|/Game/BluePrint/Turret/FunderDromeTurretBase.FunderDromeTurretBase_C|GetTeam _asfunder_drome_turret_base) 2)
    (Utilities|FlowControl|MultiGate true true -1
      (:Out%200
        (bind _outactors (Actor|GetAllActorsOfClass "/Game/TestCar/BP/TestPayloadBP.TestPayloadBP_C"))
        (Variables|Default|SetTargetRef (Utilities|Array|Get(acopy) _outactors))
        (Class|BTFunctionLibrary|SetBlackboardValueasObject (Variables|Default|GetTarget) (Variables|Default|GetTargetRef))
        (Class|BTFunctionLibrary|SetBlackboardValueasBool (Variables|Default|GetHaveTarget) true)
        (AI|BehaviorTree|FinishExecute true))
      (:Out%201
        (bind _outactors_2 (Actor|GetAllActorsOfClass "/Game/TestCar/BP/FunderDromeCarBase.FunderDromeCarBase_C" :!label _label))
        (for _array_element _outactors_2
          (if (not (== (Variables|/Game/TestCar/BP/FunderDromeCarBase.FunderDromeCarBase_C|GetTeam _array_element) (Variables|/Game/BluePrint/Turret/FunderDromeTurretBase.FunderDromeTurretBase_C|GetTeam _asfunder_drome_turret_base)))
            (if (<= (Math|Vector|VectorLength (- (Transformation|GetActorLocation _array_element) (Transformation|GetActorLocation ControlledPawn))) (Variables|Default|GetDist))
              (Variables|Default|SetTargetRef _array_element)
              (Variables|Default|SetDist (Math|Vector|VectorLength (- (Transformation|GetActorLocation _array_element) (Transformation|GetActorLocation ControlledPawn)))))))
        (Utilities|IsValid (Variables|Default|GetTargetRef)
          (:Is%20Valid
            (Class|BTFunctionLibrary|SetBlackboardValueasObject (Variables|Default|GetTarget) (Variables|Default|GetTargetRef))
            (Class|BTFunctionLibrary|SetBlackboardValueasBool (Variables|Default|GetHaveTarget) true)
            (AI|BehaviorTree|FinishExecute true))
          (:Is%20Not%20Valid
            (Class|BTFunctionLibrary|SetBlackboardValueasBool (Variables|Default|GetHaveTarget) false)
            (AI|BehaviorTree|FinishExecute true)))))
    (else
      (goto _label))))
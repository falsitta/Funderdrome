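; Behavior tree task that drives a FunderDromeCarBase or TestPayloadBP vehicle toward the blackboard TargetLocation, without calling FinishExecute.
; Threshold tiers on heading angle, distance and speed choose throttle and brake, while clamped negated angle sets steering.
; GetAngle subtracts yaws, but its ±360 correction pushes out-of-range angles further out instead of wrapping them.
; Each execution also draws a raised debug line to the target.
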(event EventReceiveExecuteAI
  (params (OwnerController :type AI%20Controller%20Object%20Reference) (ControlledPawn :type Pawn%20Object%20Reference))
  (bind _returnvalue (Math|Vector|MakeVector 0.0 0.0 5e+02))
  (bind _targetlocation (Variables|Default|GetTargetLocation))
  (bind _returnvalue_2 (Class|BTFunctionLibrary|GetBlackboardValueasVector _targetlocation))
  (bind _asfunder_drome_car_base (Utilities|Casting|CastToFunderDromeCarBase ControlledPawn)
    (:then
      (Variables|Default|SetVehiclePawn _asfunder_drome_car_base)
      (Variables|Default|SetVehicleMove (Variables|/Game/TestCar/BP/FunderDromeCarBase.FunderDromeCarBase_C|GetFunderDromeVehicleMovement _asfunder_drome_car_base)))
    (:CastFailed
      (bind _astest_payload_bp (Utilities|Casting|CastToTestPayloadBP ControlledPawn))
      (Variables|Default|SetVehiclePawn _astest_payload_bp)
      (Variables|Default|SetVehicleMove (Variables|/Game/TestCar/BP/TestPayloadBP.TestPayloadBP_C|GetFunderDromeVehicleMovement _astest_payload_bp))))
  (Variables|Default|SetSpeed (Math|Vector|VectorLength (Variables|/Game/TestCar/BP/FunderDromeVehicleMovement.FunderDromeVehicleMovement_C|GetVel (Variables|Default|GetVehicleMove))))
  (Variables|Default|SetAngle (CallFunction|GetAngle (Variables|/Game/TestCar/BP/FunderDromeVehicleMovement.FunderDromeVehicleMovement_C|GetForward (Variables|Default|GetVehicleMove)) (- _returnvalue_2 (Variables|/Game/TestCar/BP/FunderDromeVehicleMovement.FunderDromeVehicleMovement_C|GetLoc (Variables|Default|GetVehicleMove)))))
  (Rendering|Debug|DrawDebugLine (+ (Variables|/Game/TestCar/BP/FunderDromeVehicleMovement.FunderDromeVehicleMovement_C|GetLoc (Variables|Default|GetVehicleMove)) _returnvalue) (+ _returnvalue_2 _returnvalue) "(R=0.118086,G=0.725743,B=0.920000,A=1.000000)" 0.5 1.0)
  (Variables|Default|SetDistance (Math|Vector|VectorLength (- _returnvalue_2 (Variables|/Game/TestCar/BP/FunderDromeVehicleMovement.FunderDromeVehicleMovement_C|GetLoc (Variables|Default|GetVehicleMove)))))
  (if (<= (Math|Float|Absolute(Float) (Variables|Default|GetAngle)) 45.0)
    (if (>= (Variables|Default|GetDistance) 5e+03)
      (Class|VehicleAIInterface|SetThrottle(Message) (Variables|Default|GetVehiclePawn) 1.0 :!label _label)
      (Class|VehicleAIInterface|SetBrake(Message) (Variables|Default|GetVehiclePawn) 0.0)
      (elif (> (Variables|Default|GetAngle) 2e+01)
        (Class|VehicleAIInterface|SetThrottle(Message) (Variables|Default|GetVehiclePawn) 0.75)
        (Class|VehicleAIInterface|SetBrake(Message) (Variables|Default|GetVehiclePawn) 0.0)
        (else
          (goto _label))))
    (elif (<= (Math|Float|Absolute(Float) (Variables|Default|GetAngle)) 135.0)
      (if (>= (Variables|Default|GetDistance) 5e+03)
        (if (>= (Variables|Default|GetSpeed) 1.5e+03)
          (Class|VehicleAIInterface|SetThrottle(Message) (Variables|Default|GetVehiclePawn) 0.0)
          (Class|VehicleAIInterface|SetBrake(Message) (Variables|Default|GetVehiclePawn) 0.5)
          (elif (<= (Variables|Default|GetSpeed) 5e+02)
            (Class|VehicleAIInterface|SetThrottle(Message) (Variables|Default|GetVehiclePawn) 1.0)
            (Class|VehicleAIInterface|SetBrake(Message) (Variables|Default|GetVehiclePawn) 0.0)
            (else
              (Class|VehicleAIInterface|SetThrottle(Message) (Variables|Default|GetVehiclePawn) 0.75)
              (Class|VehicleAIInterface|SetBrake(Message) (Variables|Default|GetVehiclePawn) 0.0))))
        (elif (>= (Variables|Default|GetSpeed) 1.5e+03)
          (Class|VehicleAIInterface|SetThrottle(Message) (Variables|Default|GetVehiclePawn) 0.0)
          (Class|VehicleAIInterface|SetBrake(Message) (Variables|Default|GetVehiclePawn) 0.75)
          (elif (<= (Variables|Default|GetSpeed) 5e+02)
            (Class|VehicleAIInterface|SetThrottle(Message) (Variables|Default|GetVehiclePawn) 0.75)
            (Class|VehicleAIInterface|SetBrake(Message) (Variables|Default|GetVehiclePawn) 0.0)
            (else
              (Class|VehicleAIInterface|SetThrottle(Message) (Variables|Default|GetVehiclePawn) 0.5)
              (Class|VehicleAIInterface|SetBrake(Message) (Variables|Default|GetVehiclePawn) 0.0)))))
      (elif (>= (Variables|Default|GetDistance) 1e+04)
        (Class|VehicleAIInterface|SetThrottle(Message) (Variables|Default|GetVehiclePawn) 1.0)
        (Class|VehicleAIInterface|SetBrake(Message) (Variables|Default|GetVehiclePawn) 0.0)
        (elif (>= (Variables|Default|GetDistance) 5e+03)
          (if (>= (Variables|Default|GetSpeed) 1.5e+03)
            (Class|VehicleAIInterface|SetThrottle(Message) (Variables|Default|GetVehiclePawn) 0.0)
            (Class|VehicleAIInterface|SetBrake(Message) (Variables|Default|GetVehiclePawn) 0.5)
            (elif (<= (Variables|Default|GetSpeed) 5e+02)
              (Class|VehicleAIInterface|SetThrottle(Message) (Variables|Default|GetVehiclePawn) 0.75)
              (Class|VehicleAIInterface|SetBrake(Message) (Variables|Default|GetVehiclePawn) 0.0)
              (else
                (Class|VehicleAIInterface|SetThrottle(Message) (Variables|Default|GetVehiclePawn) 0.5)
                (Class|VehicleAIInterface|SetBrake(Message) (Variables|Default|GetVehiclePawn) 0.0))))
          (elif (>= (Variables|Default|GetSpeed) 1.5e+03)
            (Class|VehicleAIInterface|SetThrottle(Message) (Variables|Default|GetVehiclePawn) 0.0)
            (Class|VehicleAIInterface|SetBrake(Message) (Variables|Default|GetVehiclePawn) 1.0)
            (elif (<= (Variables|Default|GetSpeed) 5e+02)
              (Class|VehicleAIInterface|SetThrottle(Message) (Variables|Default|GetVehiclePawn) 0.0)
              (Class|VehicleAIInterface|SetBrake(Message) (Variables|Default|GetVehiclePawn) 0.5)
              (else
                (Class|VehicleAIInterface|SetThrottle(Message) (Variables|Default|GetVehiclePawn) 0.5)
                (Class|VehicleAIInterface|SetBrake(Message) (Variables|Default|GetVehiclePawn) 0.0))))))))
  (Class|VehicleAIInterface|SetTurn(Message) (Variables|Default|GetVehiclePawn) (Math|Float|Clamp(Float) (/ (- 0.0 (Variables|Default|GetAngle)) 3e+01) -1.0 1.0)))

(fn GetAngle
  (params (Forward :type Vector) (TargetVector :type Vector))
  (bind _returnvalue (Math|Conversions|RotationFromXVector TargetVector))
  (bind _returnvalue_2 (Math|Conversions|RotationFromXVector Forward))
  (bind _yaw (Math|Rotator|BreakRotator _returnvalue_2))
  (bind _yaw_2 (Math|Rotator|BreakRotator _returnvalue))
  (bind _returnvalue_3 (- _yaw _yaw_2))
  (if (> _returnvalue_3 1.8e+02)
    (LocalVariables|SetTAngle (+ _returnvalue_3 3.6e+02))
    (elif (< _returnvalue_3 -1.8e+02)
      (LocalVariables|SetTAngle (- _returnvalue_3 3.6e+02))
      (else
        (LocalVariables|SetTAngle _returnvalue_3))))
  (return (LocalVariables|GetTAngle)))
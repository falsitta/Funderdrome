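; NavMeshTestActor is a debug actor that visualises a route from its own location to a CenterPoint actor.
; On BeginPlay it caches the first NavManager and CenterPoint actors found in the level.
; Its DrawPath event asks the manager's FindRoute for a path, flushes persistent debug lines, then draws timed debug line segments between consecutive path points.
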(event Custom|DrawPath
  (Variables|Default|SetPath (.NewPath (Default|FindRoute (Variables|Default|GetManager) (Transformation|GetActorLocation) (Transformation|GetActorLocation (Variables|Default|GetCPoint)))))
  (Rendering|Debug|FlushPersistentDebugLines)
  (for (_array_element _array_index) (Variables|Default|GetPath)
    (if (!= _array_index 0)
      (Rendering|Debug|DrawDebugLine (Utilities|Array|Get(acopy) (Variables|Default|GetPath) (- _array_index 1)) _array_element "(R=0.000000,G=4.000000,B=20.000000,A=1.000000)" 3e+01 3.0))))

(event EventBeginPlay
  (bind _outactors (Actor|GetAllActorsOfClass "/Game/BluePrint/AIScript/NavManager.NavManager_C"))
  (Variables|Default|SetManager (Utilities|Array|Get(acopy) _outactors))
  (bind _outactors_2 (Actor|GetAllActorsOfClass "/Game/BluePrint/AIScript/centerPoint.centerPoint_C"))
  (Variables|Default|SetCPoint (Utilities|Array|Get(acopy) _outactors_2)))

(event Collision|EventActorBeginOverlap
  (params (OtherActor :type Actor%20Object%20Reference)))

(event EventTick
  (params (DeltaSeconds :type Float%20%28single-precision%29)))

(fn ConstructionScript)
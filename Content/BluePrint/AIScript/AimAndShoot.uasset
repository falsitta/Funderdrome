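; Behavior Tree task that makes a FunderDrome turret aim and fire at its blackboard Target.
; Each execution lerps SpringRot a fraction toward the target's mesh, using PayloadMesh for a payload or NewCarMesh otherwise, then finishes successfully.
; It sets Fireing when the signed sum of rotation deltas falls below a small threshold, without taking absolute values.
; Fireing is cleared only when the Target is invalid.
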(event EventReceiveExecuteAI
  (params (OwnerController :type AI%20Controller%20Object%20Reference) (ControlledPawn :type Pawn%20Object%20Reference))
  (bind _target (Variables|Default|GetTarget))
  (bind _returnvalue (Class|BTFunctionLibrary|GetBlackboardValueasObject _target))
  (bind (_astest_payload_bp _bsuccess) (Utilities|Casting|CastToTestPayloadBP _returnvalue))
  (Utilities|IsValid _returnvalue
    (:Is%20Valid
      (bind _asfunder_drome_turret_base (Utilities|Casting|CastToFunderDromeTurretBase ControlledPawn)
        (:then
          (Variables|/Game/BluePrint/Turret/FunderDromeTurretBase.FunderDromeTurretBase_C|SetSpringRot _asfunder_drome_turret_base (Math|Rotator|Lerp(Rotator) (Variables|/Game/BluePrint/Turret/FunderDromeTurretBase.FunderDromeTurretBase_C|GetSpringRot _asfunder_drome_turret_base) (Math|Conversions|RotationFromXVector (- (Transformation|GetWorldLocation (select _bsuccess (Variables|/Game/TestCar/BP/TestPayloadBP.TestPayloadBP_C|GetPayloadMesh _astest_payload_bp) (Variables|/Game/TestCar/BP/FunderDromeCarBase.FunderDromeCarBase_C|GetNewCarMesh (.AsFunder%20Drome%20Car%20Base (Utilities|Casting|CastToFunderDromeCarBase _returnvalue))))) (Transformation|GetActorLocation _asfunder_drome_turret_base))) 0.1 true))
          (if (<= (+ (.Roll (Math|Rotator|BreakRotator (Math|Rotator|Delta(Rotator) (Math|Conversions|RotationFromXVector (- (Transformation|GetWorldLocation (select _bsuccess (Variables|/Game/TestCar/BP/TestPayloadBP.TestPayloadBP_C|GetPayloadMesh _astest_payload_bp) (Variables|/Game/TestCar/BP/FunderDromeCarBase.FunderDromeCarBase_C|GetNewCarMesh (.AsFunder%20Drome%20Car%20Base (Utilities|Casting|CastToFunderDromeCarBase _returnvalue))))) (Transformation|GetActorLocation _asfunder_drome_turret_base))) (Variables|/Game/BluePrint/Turret/FunderDromeTurretBase.FunderDromeTurretBase_C|GetSpringRot _asfunder_drome_turret_base)))) (.Pitch (Math|Rotator|BreakRotator (Math|Rotator|Delta(Rotator) (Math|Conversions|RotationFromXVector (- (Transformation|GetWorldLocation (select _bsuccess (Variables|/Game/TestCar/BP/TestPayloadBP.TestPayloadBP_C|GetPayloadMesh _astest_payload_bp) (Variables|/Game/TestCar/BP/FunderDromeCarBase.FunderDromeCarBase_C|GetNewCarMesh (.AsFunder%20Drome%20Car%20Base (Utilities|Casting|CastToFunderDromeCarBase _returnvalue))))) (Transformation|GetActorLocation _asfunder_drome_turret_base))) (Variables|/Game/BluePrint/Turret/FunderDromeTurretBase.FunderDromeTurretBase_C|GetSpringRot _asfunder_drome_turret_base)))) (.Yaw (Math|Rotator|BreakRotator (Math|Rotator|Delta(Rotator) (Math|Conversions|RotationFromXVector (- (Transformation|GetWorldLocation (select _bsuccess (Variables|/Game/TestCar/BP/TestPayloadBP.TestPayloadBP_C|GetPayloadMesh _astest_payload_bp) (Variables|/Game/TestCar/BP/FunderDromeCarBase.FunderDromeCarBase_C|GetNewCarMesh (.AsFunder%20Drome%20Car%20Base (Utilities|Casting|CastToFunderDromeCarBase _returnvalue))))) (Transformation|GetActorLocation _asfunder_drome_turret_base))) (Variables|/Game/BluePrint/Turret/FunderDromeTurretBase.FunderDromeTurretBase_C|GetSpringRot _asfunder_drome_turret_base))))) 5.0)
            ;[1 1 1] This should be true
            (Variables|/Game/BluePrint/Turret/FunderDromeTurretBase.FunderDromeTurretBase_C|SetFireing _asfunder_drome_turret_base true))
          (AI|BehaviorTree|FinishExecute true))
        (:CastFailed
          (AI|BehaviorTree|FinishExecute true :!label _label))))
    (:Is%20Not%20Valid
      (bind _asfunder_drome_turret_base_2 (Utilities|Casting|CastToFunderDromeTurretBase ControlledPawn)
        (:then
          (Variables|/Game/BluePrint/Turret/FunderDromeTurretBase.FunderDromeTurretBase_C|SetFireing _asfunder_drome_turret_base_2 false)
          (goto _label))
        (:CastFailed
          (goto _label))))))
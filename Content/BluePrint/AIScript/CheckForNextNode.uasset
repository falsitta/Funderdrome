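; Behavior tree task that advances an AI pawn's target to the next node on a PayloadMoveNode waypoint path.
; When the pawn is within a fixed range of TargetLocation and NextIndicator is not equal to the path's Length, it writes the next node's location and incremented index to the blackboard and succeeds.
; It fails if the pawn is out of range or the index equals Length.
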(event EventReceiveExecuteAI
  (params (OwnerController :type AI%20Controller%20Object%20Reference) (ControlledPawn :type Pawn%20Object%20Reference))
  (bind _waypoint (Variables|Default|GetWaypoint))
  (bind _nextindicator (Variables|Default|GetNextIndicator))
  (bind _returnvalue (Class|BTFunctionLibrary|GetBlackboardValueasInt _nextindicator))
  (bind _returnvalue_2 (Class|BTFunctionLibrary|GetBlackboardValueasObject _waypoint))
  (bind _returnvalue_3 (+ _returnvalue 1))
  (bind _aspayload_move_node (Utilities|Casting|CastToPayloadMoveNode _returnvalue_2))
  (if (<= (Math|Vector|VectorLength (- (Class|BTFunctionLibrary|GetBlackboardValueasVector (Variables|Default|GetTargetLocation)) (Transformation|GetActorLocation ControlledPawn))) 5e+03)
    (if (== _returnvalue (Variables|/Game/BluePrint/Property/PayloadMoveNode.PayloadMoveNode_C|GetLength _aspayload_move_node))
      (AI|BehaviorTree|FinishExecute false :!label _label)
      (else
        (bind _loc (Default|GetNodeLoc _aspayload_move_node _returnvalue_3))
        (AI|BehaviorTree|SetBlackboardValueasVector (Variables|Default|GetTargetLocation) _loc)
        (Class|BTFunctionLibrary|SetBlackboardValueasInt _nextindicator _returnvalue_3)
        (AI|BehaviorTree|FinishExecute true)))
    (else
      (goto _label))))
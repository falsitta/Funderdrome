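; Hover suspension component for a vehicle that pushes a physics primitive away from the surface beneath it like a damped spring.
; InitComponent derives spring stiffness from trace length and equilibrium percentage using hard-coded load and gravity constants, then scales damping from that stiffness.
; While simulating, Tick traces along local down, applies spring plus damping force at the component's location, and records ground contact, normal and compression.
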(event Custom|StopSimulating
  (Variables|Default|SetSimulating false))

(event Custom|InitComponent
  (params (Mesh :type Primitive%20Component%20Object%20Reference) (TraceLength :type Float%20%28single-precision%29) (SpringConstant :type Float%20%28single-precision%29) (EquilibriumPercentage :type Float%20%28single-precision%29))
  (Variables|Default|SetPrimitiveComponent Mesh)
  (Variables|Default|SetTraceLength TraceLength)
  (bind _output_get (Variables|Default|SetSpringConstant (/ (* 5.0 9.8e+02) (* (- 1.0 EquilibriumPercentage) (Variables|Default|GetTraceLength)))))
  (Variables|Default|SetDampingCoeffcient (* (Math|Float|Sqrt (* _output_get 5.0)) (/ 2.0 4.0)))
  (Variables|Default|SetPastLength (Variables|Default|GetTraceLength))
  (Variables|Default|SetSimulating true))

(event EventBeginPlay)

(event EventTick
  (params (DeltaSeconds :type Float%20%28single-precision%29))
  (bind _returnvalue (Transformation|GetWorldLocation))
  (bind _tracelength (Variables|Default|GetTraceLength))
  (Variables|Default|SetDeltaTime DeltaSeconds)
  (if (Variables|Default|GetSimulating)
    (bind (_outhit _returnvalue_2) (Collision|LineTraceByChannel _returnvalue (+ _returnvalue (* (Math|Vector|GetUpVector) (* -1.0 (Variables|Default|GetTraceLength)))) "TraceTypeQuery1" false 0 "None"))
    (if _returnvalue_2
      (Variables|Default|SetOnGround true)
      (Variables|Default|SetGroundNormal (.Normal (Collision|BreakHitResult _outhit)))
      (Variables|Default|SetHitPoint (.Location (Collision|BreakHitResult _outhit)))
      (bind _output_get (Variables|Default|SetThisLength (Math|Vector|VectorLength (- (.Location (Collision|BreakHitResult _outhit)) (.TraceStart (Collision|BreakHitResult _outhit))))))
      (Variables|Default|SetCompressedDist (- (Math|Vector|VectorLength (- (.Location (Collision|BreakHitResult _outhit)) (.TraceStart (Collision|BreakHitResult _outhit)))) _tracelength))
      (Variables|Default|SetCompressionRatio (/ _output_get _tracelength))
      (Variables|Default|SetSuspVelocity (/ (- (Variables|Default|GetThisLength) (Variables|Default|GetPastLength)) (Variables|Default|GetDeltaTime)))
      (Variables|Default|SetPastLength (Variables|Default|GetThisLength))
      (Variables|Default|SetOutForce (CallFunction|SuspensionForce))
      (Class|PrimitiveComponent|AddForceatLocation (Variables|Default|GetPrimitiveComponent) (* (Math|Vector|GetUpVector) (Variables|Default|GetOutForce)) (Transformation|GetWorldLocation) "None")
      (else
        (Variables|Default|SetOnGround false)
        (Variables|Default|SetGroundNormal "0, 0, 0")
        (Variables|Default|SetCompressedDist 0.0)
        (Variables|Default|SetOutForce 0.0)
        (Variables|Default|SetThisLength (Variables|Default|GetTraceLength))
        (Variables|Default|SetCompressionRatio 1.0)))))

(fn SuspensionForce
  (bind _output_get (Variables|Default|SetHoverForce (* (Variables|Default|GetSpringConstant) (Variables|Default|GetCompressedDist) -1.0)))
  (bind _output_get_2 (Variables|Default|SetDampingForce (* (Variables|Default|GetDampingCoeffcient) (Variables|Default|GetSuspVelocity) -1.0)))
  (return (+ _output_get_2 _output_get)))
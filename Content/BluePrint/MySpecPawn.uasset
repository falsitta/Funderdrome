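; A spectator-style pawn that picks other pawns by line trace from the player camera and destroys itself when unpossessed.
; Each right mouse press fires one long Visibility trace along the camera's forward vector, with debug drawing, and stores any hit Pawn as the selection.
; Tick prints the selected pawn's name on screen.
; Logic for possessing the selection and for timed self-destruction is present but disconnected.
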(event EventBeginPlay)

(event Collision|EventActorBeginOverlap
  (params (OtherActor :type Actor%20Object%20Reference)))

(event EventUnpossessed
  (params (OldController :type Controller%20Object%20Reference))
  (Actor|DestroyActor))

(event EventTick
  (params (DeltaSeconds :type Float%20%28single-precision%29))
  (bind _pawnselected (Variables|Default|GetPawnSelected))
  (Utilities|IsValid _pawnselected
    (:Is%20Valid
      (Development|PrintString (Utilities|GetDisplayName _pawnselected) true false "(R=0.000000,G=0.660000,B=1.000000,A=1.000000)" DeltaSeconds))))

(event Input|ActionEvents|InputActionDebugKey
  (params (Key :type Key%20Structure :default "AnyKey")))

(event Input|MouseEvents|RightMouseButton
  (params (Key :type Key%20Structure :default "AnyKey"))
  (bind _returnvalue (Game|GetPlayerCameraManager 0))
  (bind _returnvalue_2 (Camera|GetCameraLocation _returnvalue))
  (:Pressed
    (Utilities|FlowControl|DoOnce false :!label _label
      (:Completed
        (bind (_outhit _returnvalue_3) (Collision|LineTraceByChannel _returnvalue_2 (+ _returnvalue_2 (* (Transformation|GetActorForwardVector _returnvalue) 3e+05)) "TraceTypeQuery1" true 0 "ForDuration"))
        (if _returnvalue_3
          (bind _output_get (Variables|Default|SetTraceHIt _outhit))
          (bind _aspawn (Utilities|Casting|CastToPawn (.HitActor (Collision|BreakHitResult _output_get))))
          (Variables|Default|SetPawnSelected _aspawn)))))
  (:Released
    (goto _label Reset)))

(fn ConstructionScript)
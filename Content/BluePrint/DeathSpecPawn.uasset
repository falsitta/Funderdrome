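; DeathSpecPawn is a spectator pawn, apparently used after death, that slowly orbits its camera by yawing the spring arm every tick.
; A DeathCam flag selects a closer arm and steadily raises the camera's post-process blend weight over about five seconds.
; Without the flag, the arm sits farther out with post-processing off.
; The pawn destroys itself when unpossessed.
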(event EventUnpossessed
  (params (OldController :type Controller%20Object%20Reference))
  (Actor|DestroyActor))

(event EventBeginPlay)

(event EventActorBeginOverlap
  (params (OtherActor :type Actor%20Object%20Reference)))

(event EventTick
  (params (DeltaSeconds :type Float%20%28single-precision%29))
  (bind _springarm (Variables|Default|GetSpringArm))
  (bind _camera (Variables|Default|GetCamera))
  (Transformation|AddRelativeRotation _springarm (Math|Rotator|MakeRotator 0.0 0.0 (* DeltaSeconds 3e+01)) false false)
  (if (Variables|Default|GetDeathCam)
    (Variables|/Script/Engine.SpringArmComponent|SetTargetArmLength _springarm 2e+03)
    (Variables|/Script/Engine.CameraComponent|SetPostProcessBlendWeight _camera (+ (Variables|/Script/Engine.CameraComponent|GetPostProcessBlendWeight _camera) (/ DeltaSeconds 5.0)))
    (else
      (Variables|/Script/Engine.SpringArmComponent|SetTargetArmLength _springarm 5e+03)
      (Variables|/Script/Engine.CameraComponent|SetPostProcessBlendWeight _camera 0.0))))

(fn ConstructionScript)
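; Interceptor missile projectile that seeks out and destroys other projectiles implementing the AdvancedProjectile interface.
; On BeginPlay it picks the nearest such projectile's mesh, within distance limits, as a high-acceleration homing target for its movement component.
; Its first collision fires a radial impulse, executes the explosion payload, attaches an impact decal, sends destroy messages to its rocket child actor and the hit actor, and applies radial damage.
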(event OnComponentHit(CollisionComponent)
  (params (HitComponent :type Primitive%20Component%20Object%20Reference) (OtherActor :type Actor%20Object%20Reference) (OtherComp :type Primitive%20Component%20Object%20Reference) (NormalImpulse :type Vector :default "0, 0, 0") (Hit :type Hit%20Result%20Structure%20%28by%20ref%29))
  (bind _explosionforce (Variables|Default|GetExplosionForce))
  ;[1 1 1] On hit save hit result
  (Utilities|FlowControl|DoOnce false
    (:Completed
      (Variables|Default|SetHitResult Hit)
      ;[1 1 1] Fire impulse
      (Class|RadialForceComponent|FireImpulse (Variables|Default|GetExplosionForce))
      ;[1 1 1] Save hit actor and hit component
      (Variables|Default|SetHitActor (.HitActor (Collision|BreakHitResult (Variables|Default|GetHitResult))))
      (Variables|Default|SetHitComponent (.HitComponent (Collision|BreakHitResult (Variables|Default|GetHitResult))))
      ;[1 1 1] Execute payload
      (Default|Execute (Variables|Default|GetSimpleExplosionPayload) (Transformation|GetWorldLocation (Variables|Default|GetExplosionForce)))
      ;[1 1 1] Spawn decal
      (Class|GameplayStatics|SpawnDecalAttached "/Game/NewProjectilesPack/Materials/Bullet/M_Impact_Decal.M_Impact_Decal" "200.000000,200.000000,200.000000" (Variables|Default|GetHitComponent) "None" (.Location (Collision|BreakHitResult (Variables|Default|GetHitResult))) (Math|Conversions|RotationFromXVector (.Normal (Collision|BreakHitResult (Variables|Default|GetHitResult)))) "KeepWorldPosition" 6.0)
      ;[1 1 1] Destroy rocket
      (Class|AdvancedProjectile|Destroy(Message) (Variables|/Script/Engine.ChildActorComponent|GetChildActor (Variables|Default|GetBP_Rocket)))
      ;[1 1 1] Destroy target projectile
      (Class|AdvancedProjectile|Destroy(Message) (Variables|Default|GetHitActor))
      ;[1 1 1] Apply damage
      (Game|Damage|ApplyRadialDamage (Variables|/Script/Engine.RadialForceComponent|GetDestructibleDamage _explosionforce) (Transformation|GetWorldLocation _explosionforce) (Variables|/Script/Engine.RadialForceComponent|GetRadius _explosionforce) "/Script/Engine.DamageType" 0 self 0 false "ECC_Visibility"))))

(event EventBeginPlay
  ;[1 1 1] Find nearest target projectile
  (CallFunction|FindNearestAdvancedProjectile)
  ;[1 1 1] Check for vaildity
  (if (Utilities|IsValid (Variables|Default|GetNearestProjectile))
    ;[1 1 1] Set homing target
    (Variables|/Script/Engine.ProjectileMovementComponent|SetHomingTargetComponent (Variables|MyProjectile|GetProjectile) (Variables|Default|GetNearestProjectile))
    ;[1 1 1] Mark as homing projectile and set homing acceleration magnitude
    (Variables|/Script/Engine.ProjectileMovementComponent|SetbIsHomingProjectile (Variables|MyProjectile|GetProjectile) true)
    (Variables|/Script/Engine.ProjectileMovementComponent|SetHomingAccelerationMagnitude (Variables|MyProjectile|GetProjectile) 3e+04)))

(fn ConstructionScript)

(fn FindNearestAdvancedProjectile
  ;[1 1 1] Find all advanced projectiles
  (bind _outactors (Actor|GetAllActorswithInterface "/Game/NewProjectilesPack/Blueprints/Common/AdvancedProjectile.AdvancedProjectile_C"))
  ;[1 1 1] For each advanced projectile
  (for _array_element _outactors
    (Variables|Default|SetAdvancedProjectile _array_element)
    ;[1 1 1] Check for validity
    (if (Utilities|IsValid (Variables|Default|GetAdvancedProjectile))
      ;[1 1 1] Return static mesh for projectile
      (bind _mesh (Class|AdvancedProjectile|ReturnMesh(Message) (Variables|Default|GetAdvancedProjectile)))
      ;[1 1 1] Check it for validity
      (Variables|Default|SetAdvancedProjectileMesh _mesh)
      (if (Utilities|IsValid (Variables|Default|GetAdvancedProjectileMesh))
        ;[1 1 1] If it's a nearest projectile
        (if (and (< (Transformation|GetDistanceTo (Variables|Default|GetAdvancedProjectile)) (Variables|Default|GetClosestDistance)) (> (Transformation|GetDistanceTo (Variables|Default|GetAdvancedProjectile)) (Variables|Default|GetMinDistance)))
          ;[1 1 1] Then set nearest projectile variable
          (Variables|Default|SetNearestProjectile (Variables|Default|GetAdvancedProjectileMesh))
          ;[1 1 1] And save current closest distance
          (Variables|Default|SetClosestDistance (Transformation|GetDistanceTo (Variables|Default|GetAdvancedProjectile))))))))

(fn ReturnProjectileMovementComponent
  (return (Variables|MyProjectile|GetProjectile)))
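; Sliding double door in a projectiles pack environment that opens when its trigger box is entered and closes on exit, or prints a hint if locked.
; One reversible timeline rotates the center lock, slides both panels in mirrored directions and drives the motor sounds' pitch.
; Timeline events and direction checks time click, impact and lock sounds, swap the lock's glow material and fire a door-closed event.
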(event OnComponentBeginOverlap(TriggerBox)
  (params (OverlappedComponent :type Primitive%20Component%20Object%20Reference) (OtherActor :type Actor%20Object%20Reference) (OtherComp :type Primitive%20Component%20Object%20Reference) (OtherBodyIndex :type Integer) (bFromSweep :type Boolean) (SweepResult :type Hit%20Result%20Structure%20%28by%20ref%29))
  ;[1 1 1] Open door if it's not locked
  (if (Variables|Default|GetisLocked)
    (Development|PrintString "The door is locked. Try to find more projectiles to open the door." true true "(R=0.000000,G=0.660000,B=1.000000,A=1.000000)" 5.0)
    (else
      (CallFunction|OpenDoors))))

(event OnComponentEndOverlap(TriggerBox)
  (params (OverlappedComponent :type Primitive%20Component%20Object%20Reference) (OtherActor :type Actor%20Object%20Reference) (OtherComp :type Primitive%20Component%20Object%20Reference) (OtherBodyIndex :type Integer))
  ;[1 1 1] Close door if it's not locked
  (if (not (Variables|Default|GetisLocked))
    (CallFunction|CloseDoors)))

(event Custom|Open%20doors
  ;[1 1 1] Open door - change lock material and play sound
  (Rendering|Material|SetMaterial (Variables|BP_Double_Doors|GetLock) 0 "/Game/NewProjectilesPack/Materials/Environment/M_UE4_Logo_Door.M_UE4_Logo_Door") ; Switch to non-glowing material
  (Audio|SpawnSoundAttached "/Game/NewProjectilesPack/Sounds/Environment/Door_Unlock_Cue.Door_Unlock_Cue" (Variables|Audio|GetDoor%20Opening%20Audio) "None" "0, 0, 0" "0, 0, 0" "EAttachLocation::KeepRelativeOffset" false 1.0 1.0)
  (Audio|Components|Audio|Play (Variables|Audio|GetDoor%20Opening%20Audio) 0.0)
  ;[1 1 1] Open/close timeline
  (bind (_direction _lock_rotation _doormovement) (Timeline|Open/close Play)
    (:Update
      ;[1 1 1] Set variables
      (Variables|Default|SetLockRotation _lock_rotation)
      (Variables|Default|SetDoorMovement _doormovement)
      ;[1 1 1] Change sound pitch multiplier
      (Audio|Components|Audio|SetPitchMultiplier (Variables|Audio|GetDoor%20Opening%20Audio) (* (Variables|Default|GetDoorMovement) (Variables|Audio|GetDefault%20Pitch)))
      ;[1 1 1] Rotate lock portion
      (Transformation|SetRelativeRotation (Variables|BP_Double_Doors|GetLock) (Math|Rotator|MakeRotator (Variables|Default|GetLockRotation) 0.0 0.0) false false)
      ;[1 1 1] Move doors
      (Transformation|SetRelativeLocation (Variables|BP_Double_Doors|GetRight%20door) (Math|Vector|MakeVector 0.0 (Variables|Default|GetDoorMovement) 0.0) false false)
      ;[1 1 1] Mirror movement for opposite door
      (Transformation|SetRelativeLocation (Variables|BP_Double_Doors|GetLeft%20door) (Math|Vector|MakeVector 0.0 (* (Variables|Default|GetDoorMovement) -1.0) 0.0) false false))
    (:Finished
      ;[1 1 1] If the timeline finished reversing...
      (if (Utilities|Enum|Equal(Enum) _direction "Backward")
        ;[1 1 1] Switch to glowing material
        (Rendering|Material|SetMaterial (Variables|BP_Double_Doors|GetLock) 0 "/Game/NewProjectilesPack/Materials/Environment/M_UE4_Logo_Doors.M_UE4_Logo_Doors")
        ;[1 1 1] Stop sound and call event
        (Audio|Components|Audio|Stop (Variables|Audio|GetDoor%20Opening%20Audio))
        (Audio|SpawnSoundAttached "/Game/NewProjectilesPack/Sounds/Environment/Door_Lock_Cue.Door_Lock_Cue" (Variables|Audio|GetDoor%20Opening%20Audio) "None" "0, 0, 0" "0, 0, 0" "EAttachLocation::KeepRelativeOffset" false 1.0 1.0)
        (Default|CallDoorCloseEvent)
        (else
          ;[1 1 1] Fade existing sound and play open door sound
          (Audio|Components|Audio|FadeOut (Variables|Audio|GetDoor%20Opening%20Audio) 0.2 0.0 :!class /Script/Engine.AudioComponent)
          (Audio|SpawnSoundAttached "/Game/NewProjectilesPack/Sounds/Environment/Door_Impact_Cue.Door_Impact_Cue" (Variables|Audio|GetDoor%20Opening%20Audio) "None" "0, 0, 0" "0, 0, 0" "EAttachLocation::KeepRelativeOffset" false 1.0 1.0))))
    (:Close%20Impact
      ;[1 1 1] If the timeline finished reversing...
      (if (Utilities|Enum|Equal(Enum) _direction "Backward")
        (Audio|SpawnSoundAttached "/Game/NewProjectilesPack/Sounds/Environment/Door_Impact_Cue.Door_Impact_Cue" (Variables|Audio|GetDoor%20Opening%20Audio) "None" "0, 0, 0" "0, 0, 0" "EAttachLocation::KeepRelativeOffset" false 1.0 1.0)
        (Audio|Components|Audio|FadeOut (Variables|Audio|GetDoor%20Opening%20Audio) 0.2 0.0 :!class /Script/Engine.AudioComponent)))
    (:Start%20Open
      ;[1 1 1] If the timeline finished reversing...
      (if (Utilities|Enum|Equal(Enum) _direction "Forward")
        (Audio|SpawnSoundAttached "/Game/NewProjectilesPack/Sounds/Environment/Door_StartClick_Cue.Door_StartClick_Cue" (Variables|BP_Double_Doors|GetLock) "None" "0, 0, 0" "0, 0, 0" "EAttachLocation::KeepRelativeOffset" false 1.0 1.0)))))

(event Custom|Close%20doors
  ;[1 1 1] Close door - play sound
  (Audio|Components|Audio|Play (Variables|Audio|GetDoor%20Closing%20Audio) 0.0)
  (Audio|SpawnSoundAttached "/Game/NewProjectilesPack/Sounds/Environment/Door_StartClick_Cue.Door_StartClick_Cue" (Variables|BP_Double_Doors|GetLock) "None" "0, 0, 0" "0, 0, 0" "EAttachLocation::KeepRelativeOffset" false 1.0 1.0)
  ;[1 1 1] Open/close timeline
  (bind (_direction _lock_rotation _doormovement) (Timeline|Open/close Reverse)
    (:Update
      ;[1 1 1] Set variables
      (Variables|Default|SetLockRotation _lock_rotation)
      (Variables|Default|SetDoorMovement _doormovement)
      ;[1 1 1] Change sound pitch multiplier
      (Audio|Components|Audio|SetPitchMultiplier (Variables|Audio|GetDoor%20Opening%20Audio) (* (Variables|Default|GetDoorMovement) (Variables|Audio|GetDefault%20Pitch)))
      ;[1 1 1] Rotate lock portion
      (Transformation|SetRelativeRotation (Variables|BP_Double_Doors|GetLock) (Math|Rotator|MakeRotator (Variables|Default|GetLockRotation) 0.0 0.0) false false)
      ;[1 1 1] Move doors
      (Transformation|SetRelativeLocation (Variables|BP_Double_Doors|GetRight%20door) (Math|Vector|MakeVector 0.0 (Variables|Default|GetDoorMovement) 0.0) false false)
      ;[1 1 1] Mirror movement for opposite door
      (Transformation|SetRelativeLocation (Variables|BP_Double_Doors|GetLeft%20door) (Math|Vector|MakeVector 0.0 (* (Variables|Default|GetDoorMovement) -1.0) 0.0) false false))
    (:Finished
      ;[1 1 1] If the timeline finished reversing...
      (if (Utilities|Enum|Equal(Enum) _direction "Backward")
        ;[1 1 1] Switch to glowing material
        (Rendering|Material|SetMaterial (Variables|BP_Double_Doors|GetLock) 0 "/Game/NewProjectilesPack/Materials/Environment/M_UE4_Logo_Doors.M_UE4_Logo_Doors")
        ;[1 1 1] Stop sound and call event
        (Audio|Components|Audio|Stop (Variables|Audio|GetDoor%20Opening%20Audio))
        (Audio|SpawnSoundAttached "/Game/NewProjectilesPack/Sounds/Environment/Door_Lock_Cue.Door_Lock_Cue" (Variables|Audio|GetDoor%20Opening%20Audio) "None" "0, 0, 0" "0, 0, 0" "EAttachLocation::KeepRelativeOffset" false 1.0 1.0)
        (Default|CallDoorCloseEvent)
        (else
          ;[1 1 1] Fade existing sound and play open door sound
          (Audio|Components|Audio|FadeOut (Variables|Audio|GetDoor%20Opening%20Audio) 0.2 0.0 :!class /Script/Engine.AudioComponent)
          (Audio|SpawnSoundAttached "/Game/NewProjectilesPack/Sounds/Environment/Door_Impact_Cue.Door_Impact_Cue" (Variables|Audio|GetDoor%20Opening%20Audio) "None" "0, 0, 0" "0, 0, 0" "EAttachLocation::KeepRelativeOffset" false 1.0 1.0))))
    (:Close%20Impact
      ;[1 1 1] If the timeline finished reversing...
      (if (Utilities|Enum|Equal(Enum) _direction "Backward")
        (Audio|SpawnSoundAttached "/Game/NewProjectilesPack/Sounds/Environment/Door_Impact_Cue.Door_Impact_Cue" (Variables|Audio|GetDoor%20Opening%20Audio) "None" "0, 0, 0" "0, 0, 0" "EAttachLocation::KeepRelativeOffset" false 1.0 1.0)
        (Audio|Components|Audio|FadeOut (Variables|Audio|GetDoor%20Opening%20Audio) 0.2 0.0 :!class /Script/Engine.AudioComponent)))
    (:Start%20Open
      ;[1 1 1] If the timeline finished reversing...
      (if (Utilities|Enum|Equal(Enum) _direction "Forward")
        (Audio|SpawnSoundAttached "/Game/NewProjectilesPack/Sounds/Environment/Door_StartClick_Cue.Door_StartClick_Cue" (Variables|BP_Double_Doors|GetLock) "None" "0, 0, 0" "0, 0, 0" "EAttachLocation::KeepRelativeOffset" false 1.0 1.0)))))

(event EventBeginPlay
  ;[1 1 1] Set door materials
  (Rendering|Material|SetMaterial (Variables|BP_Double_Doors|GetLeft%20door) 0 "/Game/NewProjectilesPack/Materials/Environment/M_DemoWall_Inst_3.M_DemoWall_Inst_3")
  (Rendering|Material|SetMaterial (Variables|BP_Double_Doors|GetLeft%20door) 1 "/Game/NewProjectilesPack/Materials/Environment/M_GlasDoor_Inst.M_GlasDoor_Inst")
  (Rendering|Material|SetMaterial (Variables|BP_Double_Doors|GetLock) 1 "/Game/NewProjectilesPack/Materials/Environment/M_DemoWall_Inst_3.M_DemoWall_Inst_3")
  (Rendering|Material|SetMaterial (Variables|BP_Double_Doors|GetLock) 0 "/Game/NewProjectilesPack/Materials/Environment/M_UE4_Logo_Doors.M_UE4_Logo_Doors"))

(fn ConstructionScript
  (Rendering|SetTranslucentSortPriority (Variables|BP_Double_Doors|GetLeft%20door) (Variables|Default|GetSort%20Priority)))
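; A destructible sphere target that respawns after it is broken.
; On BeginPlay it removes the placeholder sphere, spawns an enlarged flare explosion above its start location and adds a destructible mesh component at runtime.
; The component's fracture event passes through a DoOnce, waits a few seconds, then loops back to add a fresh target with the flare and re-arm the gate.
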(event Custom|OnComponentFracture_DestructibleMesh
  (params (HitPoint :type Vector%20%28by%20ref%29) (HitDirection :type Vector%20%28by%20ref%29))
  (bind _startlocation (Variables|Default|GetStartLocation))
  (bind (_location _rotation) (Math|Transform|BreakTransform _startlocation))
  ;[1 1 1] If player hits the target
  (Utilities|FlowControl|DoOnce false :!label _label
    (:Completed
      ;[1 1 1] Wait a few moments
      (Utilities|FlowControl|Delay 5.0)
      ;[1 1 1] Flare effect
      (bind _returnvalue (Effects|SpawnEmitteratLocation "/Game/NewProjectilesPack/Particles/BlackHoleGenerator/P_Flare_Explosion.P_Flare_Explosion" (+ _location "0, 0,500.000000") _rotation))
      (Transformation|SetWorldScale3D _returnvalue "3.000000,3.000000,3.000000")
      ;[1 1 1] Add new target
      (bind _returnvalue_2 (AddComponent|AddDestructibleComponent false))
      (Class|DestructibleComponent|SetDestructibleMesh _returnvalue_2 "/Game/NewProjectilesPack/Meshes/Environment/Shape_Sphere_DM.Shape_Sphere_DM")
      (Variables|Default|SetDestructibleMesh _returnvalue_2)
      ;[1 1 1] Bind event
      (EventDispatchers|BindEventtoOnComponentFracture _returnvalue_2 (delegate Custom|OnComponentFracture_DestructibleMesh))
      (goto _label Reset))))

(event EventBeginPlay
  ;[1 1 1] Save start location and remove existing sphere
  (Variables|Default|SetStartLocation (Transformation|GetActorTransform))
  (Components|DestroyComponent (Variables|Default|GetSphere))
  ;[1 1 1] Flare effect
  (bind _returnvalue (Effects|SpawnEmitteratLocation "/Game/NewProjectilesPack/Particles/BlackHoleGenerator/P_Flare_Explosion.P_Flare_Explosion" (+ (.Location (Math|Transform|BreakTransform (Variables|Default|GetStartLocation))) "0, 0,500.000000") (.Rotation (Math|Transform|BreakTransform (Variables|Default|GetStartLocation)))))
  (Transformation|SetWorldScale3D _returnvalue "3.000000,3.000000,3.000000")
  ;[1 1 1] Add new target
  (bind _returnvalue_2 (AddComponent|AddDestructibleComponent false))
  (Class|DestructibleComponent|SetDestructibleMesh _returnvalue_2 "/Game/NewProjectilesPack/Meshes/Environment/Shape_Sphere_DM.Shape_Sphere_DM")
  (Variables|Default|SetDestructibleMesh _returnvalue_2)
  ;[1 1 1] Bind event
  (EventDispatchers|BindEventtoOnComponentFracture _returnvalue_2 (delegate Custom|OnComponentFracture_DestructibleMesh))
  ;[1 1 1] If player hits the target
  (Utilities|FlowControl|DoOnce false) ; enters at Reset
)

(fn ConstructionScript)
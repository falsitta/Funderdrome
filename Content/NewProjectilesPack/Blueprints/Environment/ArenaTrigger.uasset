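; Trigger actor that gates the player's transition into the Arena level once they hold at least 13 projectiles.
; Tick reveals the entrance text at that count, while box overlap enables the E key or prints a warning.
; Pressing E plays the arena cinematic behind fixed delays, writes a new save, and teleports the player.
; It then restores control with a camera fade, starts battleship cinematics, spawns strategic AI and toggles snow.
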(event OnComponentBeginOverlap(TriggerBox)
  (params (OverlappedComponent :type Primitive%20Component%20Object%20Reference) (OtherActor :type Actor%20Object%20Reference) (OtherComp :type Primitive%20Component%20Object%20Reference) (OtherBodyIndex :type Integer) (bFromSweep :type Boolean) (SweepResult :type Hit%20Result%20Structure%20%28by%20ref%29))
  ;[1 1 1] If player overlaps trigger's bounds
  ;[1 1 1] Check amount of projectiles
  (bind _asfirst_person_character (Utilities|Casting|CastToFirstPersonCharacter (Game|Player|GetPlayerPawn 0))
    (:then
      (if (>= (Utilities|Array|Length (Variables|/Game/NewProjectilesPack/Blueprints/FirstPerson/FirstPersonCharacter.FirstPersonCharacter_C|GetProjectiles _asfirst_person_character)) 13)
        ;[1 1 1] Enable arena transition
        (Variables|Default|SetisArenaTransitionAvailable true)
        (Input|EnableInput (Game|GetPlayerController 0))
        (else
          ;[1 1 1] Warning message
          (Development|PrintString "You have to get all projectiles at this level to get access into arena" true true "(R=0.000000,G=0.660000,B=1.000000,A=1.000000)" 8.0))))
    (:CastFailed
      (CallFunction|FPCCastFailed))))

(event OnComponentEndOverlap(TriggerBox)
  (params (OverlappedComponent :type Primitive%20Component%20Object%20Reference) (OtherActor :type Actor%20Object%20Reference) (OtherComp :type Primitive%20Component%20Object%20Reference) (OtherBodyIndex :type Integer))
  ;[1 1 1] If player is leaving trigger's bounds
  ;[1 1 1] Check amount of projectiles
  (bind _asfirst_person_character (Utilities|Casting|CastToFirstPersonCharacter (Game|Player|GetPlayerPawn 0))
    (:then
      (if (>= (Utilities|Array|Length (Variables|/Game/NewProjectilesPack/Blueprints/FirstPerson/FirstPersonCharacter.FirstPersonCharacter_C|GetProjectiles _asfirst_person_character)) 13)
        ;[1 1 1] Disable arena transition
        (Variables|Default|SetisArenaTransitionAvailable false)
        (Input|DisableInput (Game|GetPlayerController 0))))
    (:CastFailed
      (CallFunction|FPCCastFailed))))

(event Custom|FPCCastFailed
  ;[1 1 1] Failed to cast to FPC
  (Development|PrintString "Failed to cast to FirstPersonCharacter in ArenaTrigger blueprint" false))

(event EventTick
  (params (DeltaSeconds :type Float%20%28single-precision%29))
  ;[1 1 1] Toggle arena entrance text visibility
  ;;[1 1 1] If arena text is not visible
  (if (not (Variables|Default|GetisArenaTextVisible))
    ;;[1 1 1] Check amount of projectiles
    (bind _asfirst_person_character (Utilities|Casting|CastToFirstPersonCharacter (Game|Player|GetPlayerPawn 0))
      (:then
        (if (>= (Utilities|Array|Length (Variables|/Game/NewProjectilesPack/Blueprints/FirstPerson/FirstPersonCharacter.FirstPersonCharacter_C|GetProjectiles _asfirst_person_character)) 13)
          ;;[1 1 1] Enable arena entrance text visibility
          (Rendering|ToggleVisibility (Variables|/Script/Engine.TextRenderActor|GetTextRender (Variables|Default|GetText)) false)
          (Variables|Default|SetisArenaTextVisible true)))
      (:CastFailed
        (CallFunction|FPCCastFailed)))))

(event Input|KeyboardEvents|E
  (params (Key :type Key%20Structure :default "AnyKey"))
  ;[1 1 1] Check for arena transition availability
  (:Pressed
    (if (Variables|Default|GetisArenaTransitionAvailable)
      ;[1 1 1] Disable player's HUD
      (bind _ashud (Utilities|Casting|CastToHUD (HUD|GetHUD (Game|GetPlayerController 0)))
        (:then
          (Variables|/Game/NewProjectilesPack/Blueprints/UI/HUD.HUD_C|SetIsHidden _ashud true)
          ;[1 1 1] Disable player
          (bind _asfirst_person_character (Utilities|Casting|CastToFirstPersonCharacter (Game|Player|GetPlayerPawn 0))
            (:then
              (Default|Disable _asfirst_person_character)
              ;[1 1 1] Hide arena entrance text visibility
              (Rendering|ToggleVisibility (Variables|/Script/Engine.TextRenderActor|GetTextRender (Variables|Default|GetText)) false)
              ;[1 1 1] Disable input
              (Input|DisableInput (Game|GetPlayerController 0))
              ;[1 1 1] Play arena cinematic
              (Class|PlayerController|SetCinematicMode (Game|GetPlayerController 0) true true true false true)
              (Audio|Components|Audio|Play (Variables|Default|GetArenaCinematic))
              (Utilities|FlowControl|Delay 38.0)
              (Class|PlayerController|SetCinematicMode (Game|GetPlayerController 0) false true true true true)
              ;[1 1 1] Enable player's HUD
              (bind _ashud_2 (Utilities|Casting|CastToHUD (HUD|GetHUD (Game|GetPlayerController 0)))
                (:then
                  (Variables|/Game/NewProjectilesPack/Blueprints/UI/HUD.HUD_C|SetIsHidden _ashud_2 false)
                  ;[1 1 1] Show loading screen
                  (bind _asfirst_person_character_2 (Utilities|Casting|CastToFirstPersonCharacter (Game|Player|GetPlayerPawn 0))
                    (:then
                      (Variables|/Game/NewProjectilesPack/Blueprints/FirstPerson/FirstPersonCharacter.FirstPersonCharacter_C|SetisLoading _asfirst_person_character_2 true)
                      ;[1 1 1] Create save game object
                      (bind _returnvalue (SaveGame|CreateSaveGameObject "/Game/NewProjectilesPack/Blueprints/UI/SaveGame.SaveGame_C"))
                      (bind _assave_game (Utilities|Casting|CastToSaveGame _returnvalue)
                        (:then
                          (Variables|Default|SetSaveGameReference _assave_game)
                          ;[1 1 1] Set current level
                          (Variables|/Game/NewProjectilesPack/Blueprints/Environment/LevelWorkflowController.LevelWorkflowController_C|SetCurrentLevel (Variables|Default|GetLevelWorkflowController) "Arena")
                          (Variables|/Game/NewProjectilesPack/Blueprints/UI/SaveGame.SaveGame_C|SetLevel (Variables|Default|GetSaveGameReference) "Arena")
                          ;[1 1 1] Set player's location, rotation and projectiles
                          (bind _asfirst_person_character_3 (Utilities|Casting|CastToFirstPersonCharacter (Game|GetPlayerCharacter 0))
                            (:then
                              (Variables|/Game/NewProjectilesPack/Blueprints/UI/SaveGame.SaveGame_C|SetPlayerRotation (Variables|Default|GetSaveGameReference) "0.000000,-140.000000,0.000000")
                              (Variables|/Game/NewProjectilesPack/Blueprints/UI/SaveGame.SaveGame_C|SetPlayerLocation (Variables|Default|GetSaveGameReference) "63920.000000,5822250.000000,1746.000000")
                              (Variables|/Game/NewProjectilesPack/Blueprints/UI/SaveGame.SaveGame_C|SetProjectiles (Variables|Default|GetSaveGameReference) (Variables|/Game/NewProjectilesPack/Blueprints/FirstPerson/FirstPersonCharacter.FirstPersonCharacter_C|GetProjectiles _asfirst_person_character_3))
                              ;[1 1 1] Save game
                              (SaveGame|SaveGametoSlot (Variables|Default|GetSaveGameReference) "ProjectilesPackSaveGame")
                              ;[1 1 1] Teleport player into the arena
                              (bind _asfirst_person_character_4 (Utilities|Casting|CastToFirstPersonCharacter (Game|Player|GetPlayerPawn 0))
                                (:then
                                  (Transformation|Teleport _asfirst_person_character_4 "65160.000000,1882210.000000,1746.000000" "0, 0, 0")
                                  (Pawn|SetControlRotation (Game|GetPlayerController 0) (Math|Rotator|MakeRotator 0.0 0.0 -1.4e+02))
                                  ;[1 1 1] Remove loading screen and enable player
                                  (Utilities|FlowControl|Delay 2.0)
                                  (bind _asfirst_person_character_5 (Utilities|Casting|CastToFirstPersonCharacter (Game|Player|GetPlayerPawn 0))
                                    (:then
                                      (Variables|/Game/NewProjectilesPack/Blueprints/FirstPerson/FirstPersonCharacter.FirstPersonCharacter_C|SetisLoading _asfirst_person_character_5 false)
                                      (Default|Enable _asfirst_person_character_5)
                                      ;[1 1 1] Camera fade
                                      (CameraFades|StartCameraFade :self (Variables|/Script/Engine.PlayerController|GetPlayerCameraManager (Game|GetPlayerController 0)) :FromAlpha 1.0 :Duration 4.0 :bShouldFadeAudio true)
                                      ;[1 1 1] Run battleships cinematics
                                      (Audio|Components|Audio|Play (Variables|Default|GetBattleship_Cinematic))
                                      (Audio|Components|Audio|Play (Variables|Default|GetBattleship_Trio_Cinematic))
                                      ;[1 1 1] Spawn strategic AI
                                      (Default|SpawnStrategicAI (Variables|Default|GetLevelWorkflowController))
                                      ;[1 1 1] Toggle snow
                                      (bind _asfirst_person_character_6 (Utilities|Casting|CastToFirstPersonCharacter (Game|GetPlayerCharacter 0))
                                        (:then
                                          (Default|ToggleSnow _asfirst_person_character_6))
                                        (:CastFailed
                                          (CallFunction|FPCCastFailed))))
                                    (:CastFailed
                                      (CallFunction|FPCCastFailed))))
                                (:CastFailed
                                  (Development|PrintString "Failed to cast to FirstPersonCharacter in ArenaTrigger blueprint" false))))
                            (:CastFailed
                              (Development|PrintString "Failed to cast to FirstPersonCharacter in ArenaTrigger blueprint" false))))
                        (:CastFailed
                          (Development|PrintString "Failed to cast to SaveGame in ArenaTrigger blueprint" false))))
                    (:CastFailed
                      (CallFunction|FPCCastFailed))))
                (:CastFailed
                  (Development|PrintString "Failed to cast to HUD in ArenaTrigger blueprint" false))))
            (:CastFailed
              (CallFunction|FPCCastFailed))))
        (:CastFailed
          (Development|PrintString "Failed to cast to HUD in ArenaTrigger blueprint" false))))))

(fn ConstructionScript)
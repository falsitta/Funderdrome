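; A trigger actor that unlocks grenade projectiles for the player in the environment.
; The first overlap of its TriggerBox, by any actor, casts player pawn 0 to FirstPersonCharacter and adds explosive, smoke and toxic grenades to its Projectiles array without duplicates.
; It then prints an unlock message and spawns a particle effect at the player's location.
; A DoOnce limits this to one firing.
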(event OnComponentBeginOverlap(TriggerBox)
  (params (OverlappedComponent :type Primitive%20Component%20Object%20Reference) (OtherActor :type Actor%20Object%20Reference) (OtherComp :type Primitive%20Component%20Object%20Reference) (OtherBodyIndex :type Integer) (bFromSweep :type Boolean) (SweepResult :type Hit%20Result%20Structure%20%28by%20ref%29))
  ;[1 1 1] If player overlaps trigger's bounds
  ;[1 1 1] Add grenades
  (Utilities|FlowControl|DoOnce false
    (:Completed
      (bind _asfirst_person_character (Utilities|Casting|CastToFirstPersonCharacter (Game|Player|GetPlayerPawn 0))
        (:then
          (Utilities|Array|AddUnique (Variables|/Game/NewProjectilesPack/Blueprints/FirstPerson/FirstPersonCharacter.FirstPersonCharacter_C|GetProjectiles _asfirst_person_character) "/Game/NewProjectilesPack/Blueprints/Grenades/ExplosiveGrenadeProjectile.ExplosiveGrenadeProjectile_C")
          (Utilities|Array|AddUnique (Variables|/Game/NewProjectilesPack/Blueprints/FirstPerson/FirstPersonCharacter.FirstPersonCharacter_C|GetProjectiles _asfirst_person_character) "/Game/NewProjectilesPack/Blueprints/Grenades/SmokeGrenadeProjectile.SmokeGrenadeProjectile_C")
          (Utilities|Array|AddUnique (Variables|/Game/NewProjectilesPack/Blueprints/FirstPerson/FirstPersonCharacter.FirstPersonCharacter_C|GetProjectiles _asfirst_person_character) "/Game/NewProjectilesPack/Blueprints/Grenades/ToxicGrenadeProjectile.ToxicGrenadeProjectile_C")
          ;[1 1 1] Notify player about new projectile
          (Development|PrintString "New projectile has been unlocked!" true true "(R=0.000000,G=0.660000,B=1.000000,A=1.000000)" 5.0)
          (Effects|SpawnEmitteratLocation "/Game/NewProjectilesPack/Particles/MicrodestructorMissile/P_Microdestructor_Swarm.P_Microdestructor_Swarm" (Transformation|GetActorLocation (Game|GetPlayerCharacter 0))))
        (:CastFailed
          (Development|PrintString "Failed to cast to FirstPersonCharacter in GrenadesTrigger blueprint" false))))))

(fn ConstructionScript)
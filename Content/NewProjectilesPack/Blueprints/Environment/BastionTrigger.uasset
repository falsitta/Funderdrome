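; BastionTrigger is a level trigger that starts the bastion sequence and unlocks new projectiles for the player.
; The first overlap of its box, with no check on the overlapping actor, plays BastionCinematic and enables air mode through LevelWorkflowController via a DoOnce.
; It then adds six special projectiles, including teleport and strike types, to the FirstPersonCharacter's list, prints an unlock message and spawns a particle burst at the player.
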(event OnComponentBeginOverlap(TriggerBox)
  (params (OverlappedComponent :type Primitive%20Component%20Object%20Reference) (OtherActor :type Actor%20Object%20Reference) (OtherComp :type Primitive%20Component%20Object%20Reference) (OtherBodyIndex :type Integer) (bFromSweep :type Boolean) (SweepResult :type Hit%20Result%20Structure%20%28by%20ref%29))
  ;[1 1 1] If player overlaps trigger's bounds
  (Utilities|FlowControl|DoOnce false
    (:Completed
      ;[1 1 1] Play cinematic
      (Audio|Components|Audio|Play (Variables|Default|GetBastionCinematic))
      ;[1 1 1] Enable air mode
      (Default|EnableAirMode (Variables|Default|GetLevelWorkflowController))
      ;[1 1 1] Add teleport projectile
      (bind _asfirst_person_character (Utilities|Casting|CastToFirstPersonCharacter (Game|Player|GetPlayerPawn 0))
        (:then
          (Utilities|Array|AddUnique (Variables|/Game/NewProjectilesPack/Blueprints/FirstPerson/FirstPersonCharacter.FirstPersonCharacter_C|GetProjectiles _asfirst_person_character) "/Game/NewProjectilesPack/Blueprints/Teleport/TeleportProjectile.TeleportProjectile_C")
          ;[1 1 1] Add blade swarm
          (Utilities|Array|AddUnique (Variables|/Game/NewProjectilesPack/Blueprints/FirstPerson/FirstPersonCharacter.FirstPersonCharacter_C|GetProjectiles _asfirst_person_character) "/Game/NewProjectilesPack/Blueprints/BladeSwarm/BladeSwarmStrikePointer.BladeSwarmStrikePointer_C")
          ;[1 1 1] Add prizmatic arrow
          (Utilities|Array|AddUnique (Variables|/Game/NewProjectilesPack/Blueprints/FirstPerson/FirstPersonCharacter.FirstPersonCharacter_C|GetProjectiles _asfirst_person_character) "/Game/NewProjectilesPack/Blueprints/PrizmaticArrow/PrizmaticArrowStrikePointer.PrizmaticArrowStrikePointer_C")
          ;[1 1 1] Add bombardment
          (Utilities|Array|AddUnique (Variables|/Game/NewProjectilesPack/Blueprints/FirstPerson/FirstPersonCharacter.FirstPersonCharacter_C|GetProjectiles _asfirst_person_character) "/Game/NewProjectilesPack/Blueprints/Bombardment/BombardmentBeacon.BombardmentBeacon_C")
          ;[1 1 1] Add time bomb
          (Utilities|Array|AddUnique (Variables|/Game/NewProjectilesPack/Blueprints/FirstPerson/FirstPersonCharacter.FirstPersonCharacter_C|GetProjectiles _asfirst_person_character) "/Game/NewProjectilesPack/Blueprints/TimeBomb/TimeBombProjectile.TimeBombProjectile_C")
          ;[1 1 1] Add ECM strike
          (Utilities|Array|AddUnique (Variables|/Game/NewProjectilesPack/Blueprints/FirstPerson/FirstPersonCharacter.FirstPersonCharacter_C|GetProjectiles _asfirst_person_character) "/Game/NewProjectilesPack/Blueprints/ECMStrike/ECMStrikeProjectile.ECMStrikeProjectile_C")
          ;[1 1 1] Notify player about new projectile
          (Development|PrintString "New projectile has been unlocked!")
          (Effects|SpawnEmitteratLocation "/Game/NewProjectilesPack/Particles/MicrodestructorMissile/P_Microdestructor_Swarm.P_Microdestructor_Swarm" (Transformation|GetActorLocation (Game|Player|GetPlayerPawn 0))))
        (:CastFailed
          (Development|PrintString "Failed to cast to FirstPersonCharacter in BastionTrigger blueprint" false))))))

(fn ConstructionScript)
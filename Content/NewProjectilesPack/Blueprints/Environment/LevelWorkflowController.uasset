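; Level controller that runs the showcase's game flow: main menu, pause menu, showcase cinematic and gameplay start.
; StartGame restores player position, rotation and projectiles from the save, starts a looping autosave and, in the Arena, plays battleship cinematics and spawns a strategic AI once.
; Air mode, enabled in the Arena when enough projectiles are owned, lets E swap possession between the first-person character and Cratos.
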(event Custom|FPCCastFailed
  ;[1 1 1] FPC Cast failed event
  (Development|PrintString "Failed to cast to FirstPersonCharacter in LevelWorkflowController blueprint" false))

(event Custom|StartGame
  ;[1 1 1] Start Game
  ;;[1 1 1] Set input mode
  (Input|SetInputModeGameOnly (Game|GetPlayerController 0))
  ;;[1 1 1] Set camera and enable player
  (bind _asfirst_person_character (Utilities|Casting|CastToFirstPersonCharacter (Game|Player|GetPlayerPawn 0))
    (:then
      (Game|Player|SetViewTargetwithBlend (Game|GetPlayerController 0) _asfirst_person_character 0.0 "VTBlend_Linear" 0.0 false)
      (Default|Enable _asfirst_person_character)
      ;;[1 1 1] Enable HUD
      (bind _ashud (Utilities|Casting|CastToHUD (HUD|GetHUD (Game|GetPlayerController 0)))
        (:then
          (Variables|/Game/NewProjectilesPack/Blueprints/UI/HUD.HUD_C|SetIsHidden _ashud false)
          ;;[1 1 1] Load game data
          (bind _returnvalue (SaveGame|LoadGamefromSlot "ProjectilesPackSaveGame"))
          (bind _assave_game (Utilities|Casting|CastToSaveGame _returnvalue)
            (:then
              (Variables|Default|SetSaveGameReference _assave_game)
              ;;[1 1 1] Set player location, rotation and projectiles
              (bind _asfirst_person_character_2 (Utilities|Casting|CastToFirstPersonCharacter (Game|Player|GetPlayerPawn 0))
                (:then
                  (Variables|/Game/NewProjectilesPack/Blueprints/FirstPerson/FirstPersonCharacter.FirstPersonCharacter_C|SetProjectiles _asfirst_person_character_2 (Variables|/Game/NewProjectilesPack/Blueprints/UI/SaveGame.SaveGame_C|GetProjectiles (Variables|Default|GetSaveGameReference)))
                  (Transformation|SetActorLocation _asfirst_person_character_2 (Variables|/Game/NewProjectilesPack/Blueprints/UI/SaveGame.SaveGame_C|GetPlayerLocation (Variables|Default|GetSaveGameReference)) false false)
                  (Pawn|SetControlRotation (Game|GetPlayerController 0) (Variables|/Game/NewProjectilesPack/Blueprints/UI/SaveGame.SaveGame_C|GetPlayerRotation (Variables|Default|GetSaveGameReference)))
                  ;;[1 1 1] Camera fade
                  (CameraFades|StartCameraFade :self (Variables|/Script/Engine.PlayerController|GetPlayerCameraManager (Game|GetPlayerController 0)) :FromAlpha 1.0 :Duration 4.0 :bShouldFadeAudio true)
                  ;;[1 1 1] Enable autosave
                  (CallFunction|EnableAutosave)
                  ;;[1 1 1] If current level is Arena
                  (if (Utilities|Enum|Equal(Enum) (Variables|/Game/NewProjectilesPack/Blueprints/UI/SaveGame.SaveGame_C|GetLevel (Variables|Default|GetSaveGameReference)) "Arena")
                    ;;[1 1 1] Play battleships cinematics
                    (Audio|Components|Audio|Play (Variables|Default|GetBattleship_Cinematic))
                    (Audio|Components|Audio|Play (Variables|Default|GetBattleship_Trio_Cinematic))
                    ;;[1 1 1] Spawn strategic AI
                    (CallFunction|SpawnStrategicAI)
                    ;;[1 1 1] Toggle snow and enable air mode, if player have enough projectiles
                    (bind _asfirst_person_character_3 (Utilities|Casting|CastToFirstPersonCharacter (Game|Player|GetPlayerPawn 0))
                      (:then
                        (Default|ToggleSnow _asfirst_person_character_3)
                        (if (>= (Utilities|Array|Length (Variables|/Game/NewProjectilesPack/Blueprints/FirstPerson/FirstPersonCharacter.FirstPersonCharacter_C|GetProjectiles _asfirst_person_character_3)) 14)
                          (CallFunction|EnableAirMode)))
                      (:CastFailed
                        (CallFunction|FPCCastFailed)))))
                (:CastFailed
                  (CallFunction|FPCCastFailed))))
            (:CastFailed
              (Development|PrintString "Failed to cast to SaveGame in LevelWorkflowController blueprint" false))))
        (:CastFailed
          (CallFunction|HUDCastFailed))))
    (:CastFailed
      (CallFunction|FPCCastFailed))))

(event Custom|HUDCastFailed
  ;[1 1 1] HUD Cast failed event
  (Development|PrintString "Failed to cast to HUD in LevelWorkflowController blueprint" false))

(event Custom|Pause
  ;[1 1 1] Pause menu
  ;;[1 1 1] Check pause widget
  (if (Utilities|IsValid (Variables|Default|GetPauseWidget))
    _
    (else
      ;;[1 1 1] Create pause widget
      (bind _returnvalue (UserInterface|CreateWidget "/Game/NewProjectilesPack/Blueprints/UI/PauseMenu.PauseMenu_C"))
      (Variables|Default|SetPauseWidget _returnvalue)
      (Variables|/Game/NewProjectilesPack/Blueprints/UI/PauseMenu.PauseMenu_C|SetLevelWorkflowControllerReference _returnvalue self)))
  ;;[1 1 1] Show pause widget
  (Variables|/Script/Engine.PlayerController|SetbShowMouseCursor (Game|GetPlayerController 0) true)
  (Input|SetInputModeUIOnly (Game|GetPlayerController 0) (Variables|Default|GetPauseWidget) "DoNotLock")
  (UserInterface|Viewport|AddtoViewport (Variables|Default|GetPauseWidget) 0)
  ;;[1 1 1] Pause game
  (Game|SetGamePaused true))

(event Custom|DisableAutosave
  ;[1 1 1] Disable autosave
  (if (Utilities|Time|IsValidTimerHandle (Variables|Default|GetAutosaveTimer))
    (Utilities|Time|ClearandInvalidateTimerbyHandle (Variables|Default|GetAutosaveTimer))))

(event Custom|EnableAllProjectiles
  ;[1 1 1] Enable all projectiles
  (bind _asfirst_person_character (Utilities|Casting|CastToFirstPersonCharacter (Game|Player|GetPlayerPawn 0))
    (:then
      (Variables|/Game/NewProjectilesPack/Blueprints/FirstPerson/FirstPersonCharacter.FirstPersonCharacter_C|SetProjectiles _asfirst_person_character (Utilities|Array|MakeArray "/Game/NewProjectilesPack/Blueprints/Bullet/BulletStrikePointer.BulletStrikePointer_C" "/Game/NewProjectilesPack/Blueprints/HomingMissile/HomingMissileProjectile.HomingMissileProjectile_C" "/Game/NewProjectilesPack/Blueprints/Grenades/ExplosiveGrenadeProjectile.ExplosiveGrenadeProjectile_C" "/Game/NewProjectilesPack/Blueprints/PlasmaBall/PlasmaBallProjectile.PlasmaBallProjectile_C" "/Game/NewProjectilesPack/Blueprints/Grenades/SmokeGrenadeProjectile.SmokeGrenadeProjectile_C" "/Game/NewProjectilesPack/Blueprints/OrbitalLaserBeam/OrbitalLaserBeam.OrbitalLaserBeam_C" "/Game/NewProjectilesPack/Blueprints/OrbitalKineticMissile/KineticMissileBeacon.KineticMissileBeacon_C" "/Game/NewProjectilesPack/Blueprints/Grenades/ToxicGrenadeProjectile.ToxicGrenadeProjectile_C" "/Game/NewProjectilesPack/Blueprints/Railgun/RailgunProjectile.RailgunProjectile_C" "/Game/NewProjectilesPack/Blueprints/Flamethrower/Flamethrower.Flamethrower_C" "/Game/NewProjectilesPack/Blueprints/Multimissile/MultiMissileProjectile.MultiMissileProjectile_C" "/Game/NewProjectilesPack/Blueprints/MicrodestructorMissile/MicrodestructorMissileProjectile.MicrodestructorMissileProjectile_C" "/Game/NewProjectilesPack/Blueprints/Teleport/TeleportProjectile.TeleportProjectile_C" "/Game/NewProjectilesPack/Blueprints/BlackHoleGenerator/BlackHole.BlackHole_C" "/Game/NewProjectilesPack/Blueprints/InterceptorMissile/InterceptorMissileProjectile.InterceptorMissileProjectile_C")))
    (:CastFailed
      (CallFunction|FPCCastFailed))))

(event Custom|EnableAirMode
  ;[1 1 1] Enable/disable air mode
  (Variables|Default|SetisAirModeEnabled true))

(event Custom|DisableAirMode
  ;[1 1 1] Enable/disable air mode
  (Variables|Default|SetisAirModeEnabled false))

(event Custom|AutoSave
  ;[1 1 1] Enable autosave
  (CallFunction|SaveGame (Variables|Default|GetCurrentLevel))
  (Development|PrintString "Saving game..." true true "(R=0.000000,G=0.660000,B=1.000000,A=1.000000)" 5.0))

(event Custom|SpawnStrategicAI
  ;[1 1 1] Spawn Strategic AI
  (Utilities|FlowControl|DoOnce false
    (:Completed
      (Game|SpawnActorfromClass "/Game/NewProjectilesPack/Blueprints/Common/StrategicAI.StrategicAI_C" (Math|Transform|MakeTransform (Utilities|Select :Index (Math|Random|RandomIntegerinRange 0 2) :Option%200 (Variables|Default|GetAISpawn_01) :Option%201 (Variables|Default|GetAISpawn_02) :Option%202 (Variables|Default|GetAISpawn_03)) "0, 0, 0" "10.000000,10.000000,10.000000") "AlwaysSpawn" 0 0))))

(event Custom|StartShowcaseCinematic
  ;[1 1 1] Start showcase cinematic and start game
  (Class|PlayerController|SetCinematicMode (Game|GetPlayerController 0) true true true true true)
  (Audio|Components|Audio|Play (Variables|Default|GetShowcaseCinematic))
  (Utilities|FlowControl|Delay 23.0)
  (Class|PlayerController|SetCinematicMode (Game|GetPlayerController 0) false true true true true)
  (CallFunction|StartGame))

(event Custom|ShowMainMenu
  ;[1 1 1] Show main menu
  ;;[1 1 1] Disable player
  (bind _asfirst_person_character (Utilities|Casting|CastToFirstPersonCharacter (Game|Player|GetPlayerPawn 0))
    (:then
      (Default|Disable _asfirst_person_character)
      ;;[1 1 1] Change camera
      (Game|Player|SetViewTargetwithBlend (Game|GetPlayerController 0) (Variables|Default|GetStartupCamera) 0.0 "VTBlend_Linear" 0.0 false)
      ;;[1 1 1] Hide HUD
      (bind _ashud (Utilities|Casting|CastToHUD (HUD|GetHUD (Game|GetPlayerController 0)))
        (:then
          (Variables|/Game/NewProjectilesPack/Blueprints/UI/HUD.HUD_C|SetIsHidden _ashud true)
          ;;[1 1 1] Check main menu widget
          (if (Utilities|IsValid (Variables|Default|GetMainMenuWidget))
            _
            (else
              ;;[1 1 1] Create main menu widget
              (bind _returnvalue (UserInterface|CreateWidget "/Game/NewProjectilesPack/Blueprints/UI/MainMenu.MainMenu_C"))
              (Variables|/Game/NewProjectilesPack/Blueprints/UI/MainMenu.MainMenu_C|SetLevelWorkflowControllerReference _returnvalue self)
              (Variables|Default|SetMainMenuWidget _returnvalue)))
          ;;[1 1 1] Show main menu widget
          (Input|SetInputModeUIOnly (Game|GetPlayerController 0) (Variables|Default|GetMainMenuWidget) "DoNotLock")
          (UserInterface|Viewport|AddtoViewport (Variables|Default|GetMainMenuWidget) 0)
          (Variables|/Script/Engine.PlayerController|SetbShowMouseCursor (Game|GetPlayerController 0) true)
          ;;[1 1 1] Disable autosave
          (CallFunction|DisableAutosave)
          ;;[1 1 1] Camera fade
          (CameraFades|StartCameraFade :self (Variables|/Script/Engine.PlayerController|GetPlayerCameraManager (Game|GetPlayerController 0)) :FromAlpha 1.0 :Duration 4.0 :bShouldFadeAudio true))
        (:CastFailed
          (CallFunction|HUDCastFailed))))
    (:CastFailed
      (CallFunction|FPCCastFailed))))

(event Custom|EnableAutosave
  ;[1 1 1] Enable autosave
  (bind _returnvalue (Utilities|Time|SetTimerbyEvent (delegate Custom|AutoSave) 6e+01 true))
  (Variables|Default|SetAutosaveTimer _returnvalue))

(event EventBeginPlay
  ;[1 1 1] Init sequence
  (Input|EnableInput (Game|GetPlayerController 0))
  (CallFunction|ShowMainMenu))

(event Input|KeyboardEvents|E
  (params (Key :type Key%20Structure :default "AnyKey"))
  ;[1 1 1] Change player's pawn
  (:Pressed
    (if (Variables|Default|GetisAirModeEnabled)
      (if (Variables|Default|GetisPossessed)
        (Variables|Default|SetisPossessed false)
        (Pawn|Possess (Game|GetPlayerController 0) (Variables|Default|GetFirstPersonCharacterReference))
        (Transformation|Teleport (Variables|Default|GetFirstPersonCharacterReference) (Transformation|GetActorLocation (Variables|Default|GetCratosReference)) "0, 0, 0")
        (Pawn|SetControlRotation (Game|GetPlayerController 0) (Transformation|GetWorldRotation (Variables|/Game/NewProjectilesPack/Blueprints/Common/BP_Cratos.BP_Cratos_C|GetCamera (Variables|Default|GetCratosReference))))
        (else
          (Variables|Default|SetisPossessed true)
          (Pawn|Possess (Game|GetPlayerController 0) (Variables|Default|GetCratosReference)))))))

(event Input|KeyboardEvents|Escape
  (params (Key :type Key%20Structure :default "AnyKey"))
  ;[1 1 1] Pause menu
  ;;[1 1 1] Open pause menu
  (:Pressed
    (CallFunction|Pause)))

(event Input|KeyboardEvents|M
  (params (Key :type Key%20Structure :default "AnyKey"))
  ;[1 1 1] Pause menu
  ;;[1 1 1] Open pause menu
  (:Pressed
    (CallFunction|Pause)))

(fn ConstructionScript)
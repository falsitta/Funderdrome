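; A moving, destructible target that respawns after it is fractured.
; At BeginPlay it replaces its placeholder mesh with a spawned destructible component, which Tick moves by a fixed delta, snapping it back to the origin once any axis reaches the distance limit.
; A fracture passes a DoOnce gate to play a sound, count the spawn and stop movement, then after a delay destroys the component and spawns a new one, resetting the gate.
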(event Custom|OnComponentFracture_DestructibleMesh
  (params (HitPoint :type Vector%20%28by%20ref%29) (HitDirection :type Vector%20%28by%20ref%29))
  ;[1 1 1] If player hits the target
  (Utilities|FlowControl|DoOnce false :!label _label
    (:Completed
      ;[1 1 1] Play hit sound
      (Audio|PlaySoundatLocation "/Game/NewProjectilesPack/Sounds/Environment/Target_Destroyed_Cue.Target_Destroyed_Cue" (Transformation|GetWorldLocation (Variables|Default|GetDefaultSceneRoot)))
      ;[1 1 1] Update spawn count
      (Variables|Default|SetSpawnCount (+ (Variables|Default|GetSpawnCount) 1))
      ;[1 1 1] Disable movement and wait a few seconds
      (Variables|Default|SetIsMovable false)
      (Utilities|FlowControl|Delay 2.1)
      ;[1 1 1] Destroy old target
      (Components|DestroyComponent (Variables|Default|GetDestructibleMesh))
      ;[1 1 1] Spawn new target
      (bind _returnvalue (AddComponent|AddDestructibleComponent false))
      (Class|DestructibleComponent|SetDestructibleMesh _returnvalue "/Game/NewProjectilesPack/Meshes/Environment/SM_Target_DM.SM_Target_DM")
      (Variables|Default|SetDestructibleMesh _returnvalue)
      ;[1 1 1] Bind event
      (EventDispatchers|AssignOnComponentFracture _returnvalue (delegate Custom|OnComponentFracture_DestructibleMesh))
      ;[1 1 1] Enable movement for target
      (Variables|Default|SetIsMovable true)
      (goto _label Reset))))

(event EventTick
  (params (DeltaSeconds :type Float%20%28single-precision%29))
  ;[1 1 1] If movement enabled
  (if (Variables|Default|GetIsMovable)
    ;[1 1 1] If mesh is valid
    (if (Utilities|IsValid (Variables|Default|GetDestructibleMesh))
      ;[1 1 1] Move target
      (Transformation|AddRelativeLocation (Variables|Default|GetDestructibleMesh) (Variables|Default|GetDeltaLocation) false false)
      ;[1 1 1] Check target's movement bounds at X axis
      (if (>= (Math|Float|Absolute(Float) (.X (Math|Vector|BreakVector (Variables|/Script/Engine.SceneComponent|GetRelativeLocation (Variables|Default|GetDestructibleMesh))))) (Variables|Default|GetDistance))
        ;[1 1 1] Return target at start position
        (Variables|Default|SetIsMovable false :!label _label)
        (if (Utilities|IsValid (Variables|Default|GetDestructibleMesh))
          (Transformation|SetRelativeLocation (Variables|Default|GetDestructibleMesh) "0, 0, 0" false false)
          (Variables|Default|SetIsMovable true))
        (else
          ;[1 1 1] Check target's movement bounds at Y axis
          (if (>= (Math|Float|Absolute(Float) (.Y (Math|Vector|BreakVector (Variables|/Script/Engine.SceneComponent|GetRelativeLocation (Variables|Default|GetDestructibleMesh))))) (Variables|Default|GetDistance))
            (goto _label)
            (else
              ;[1 1 1] Check target's movement bounds at Z axis
              (if (>= (Math|Float|Absolute(Float) (.Z (Math|Vector|BreakVector (Variables|/Script/Engine.SceneComponent|GetRelativeLocation (Variables|Default|GetDestructibleMesh))))) (Variables|Default|GetDistance))
                (goto _label)))))))))

(event EventBeginPlay
  ;[1 1 1] Remove existing target
  (Components|DestroyComponent (Variables|Default|GetSM_Target))
  ;[1 1 1] Spawn new target
  (bind _returnvalue (AddComponent|AddDestructibleComponent false))
  (Class|DestructibleComponent|SetDestructibleMesh _returnvalue "/Game/NewProjectilesPack/Meshes/Environment/SM_Target_DM.SM_Target_DM")
  (Variables|Default|SetDestructibleMesh _returnvalue)
  ;[1 1 1] Bind event
  (EventDispatchers|AssignOnComponentFracture _returnvalue (delegate Custom|OnComponentFracture_DestructibleMesh))
  ;[1 1 1] Enable movement for target
  (Variables|Default|SetIsMovable true)
  ;[1 1 1] If player hits the target
  (Utilities|FlowControl|DoOnce false) ; enters at Reset
)

(fn ConstructionScript)
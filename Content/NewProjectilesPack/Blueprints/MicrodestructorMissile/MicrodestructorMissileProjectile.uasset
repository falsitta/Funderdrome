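; Homing missile projectile that releases a microdestructor swarm on impact, dissolving and destroying the static mesh actor it hits.
; HomingMissile points the projectile movement at a target actor's mesh.
; The first hit applies radial damage and impulse from ExplosionForce, plus particles, sound and camera shake.
; Static mesh actors get a dynamic dissolve material driven by a timeline before destruction; otherwise the missile removes itself after a delay.
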(event OnComponentHit(CollisionComponent)
  (params (HitComponent :type Primitive%20Component%20Object%20Reference) (OtherActor :type Actor%20Object%20Reference) (OtherComp :type Primitive%20Component%20Object%20Reference) (NormalImpulse :type Vector :default "0, 0, 0") (Hit :type Hit%20Result%20Structure%20%28by%20ref%29))
  (bind _explosionforce (Variables|Default|GetExplosionForce))
  ;[1 1 1] On hit save hit result
  (Utilities|FlowControl|DoOnce false
    (:Completed
      (Variables|Default|SetHitResult Hit)
      ;[1 1 1] Apply damage
      (Game|Damage|ApplyRadialDamage (Variables|/Script/Engine.RadialForceComponent|GetDestructibleDamage _explosionforce) (Transformation|GetWorldLocation _explosionforce) (Variables|/Script/Engine.RadialForceComponent|GetRadius _explosionforce) "/Script/Engine.DamageType" 0 self 0 false "ECC_Visibility")
      ;[1 1 1] Fire impulse
      (Class|RadialForceComponent|FireImpulse (Variables|Default|GetExplosionForce))
      ;[1 1 1] Spawn microdestructors swarm
      (bind _returnvalue (Effects|SpawnEmitteratLocation "/Game/NewProjectilesPack/Particles/MicrodestructorMissile/P_Microdestructor_Fire.P_Microdestructor_Fire" (Transformation|GetWorldLocation (Variables|Default|GetExplosionForce))))
      (Transformation|SetRelativeScale3D _returnvalue "5.000000,5.000000,5.000000")
      (bind _returnvalue_2 (Effects|SpawnEmitteratLocation "/Game/NewProjectilesPack/Particles/MicrodestructorMissile/P_Microdestructor_Swarm.P_Microdestructor_Swarm" (Transformation|GetWorldLocation (Variables|Default|GetExplosionForce))))
      (Transformation|SetRelativeScale3D _returnvalue_2 "3.000000,3.000000,3.000000")
      ;[1 1 1] Explosion sound
      (Audio|PlaySoundatLocation "/Game/NewProjectilesPack/Sounds/Common/Explosion_01_Cue.Explosion_01_Cue" (Transformation|GetWorldLocation (Variables|Default|GetExplosionForce)))
      ;[1 1 1] Dissolution sound
      (Audio|Components|Audio|SetSound (Variables|Default|GetFire_Sparks01_Cue) "/Game/NewProjectilesPack/Sounds/Common/Fire_Sparks.Fire_Sparks")
      (Audio|Components|Audio|Play (Variables|Default|GetFire_Sparks01_Cue) 0.0)
      (Audio|Components|Audio|FadeOut (Variables|Default|GetFire_Sparks01_Cue) 5.0 0.0 :!class /Script/Engine.AudioComponent)
      ;[1 1 1] Camera shake
      (Class|PlayerCameraManager|PlayCameraShake (Variables|/Script/Engine.PlayerController|GetPlayerCameraManager (Game|GetPlayerController 0)) "/Game/NewProjectilesPack/Blueprints/OrbitalLaserBeam/OrbitalLaserBeamShakeBlueprint.OrbitalLaserBeamShakeBlueprint_C" 1.0 "CameraLocal" "0, 0, 0")
      ;[1 1 1] If we hit staticMeshActor
      (bind _asstatic_mesh_actor (Utilities|Casting|CastToStaticMeshActor (.HitActor (Collision|BreakHitResult (Variables|Default|GetHitResult))))
        (:then
          ;[1 1 1] Create dissolve material
          (bind _returnvalue_3 (Rendering|Material|CreateDynamicMaterialInstance (Variables|/Script/Engine.StaticMeshActor|GetStaticMeshComponent _asstatic_mesh_actor) 0 "/Game/NewProjectilesPack/Materials/MicrodestructorMissile/Dissolve_Inst.Dissolve_Inst" :!class /Script/Engine.PrimitiveComponent))
          (Variables|Default|SetDissolveMaterial _returnvalue_3)
          ;[1 1 1] Apply it for each actor's material
          (for (_ _array_index) (Rendering|Material|GetMaterials (Variables|/Script/Engine.StaticMeshActor|GetStaticMeshComponent _asstatic_mesh_actor))
            (Rendering|Material|SetMaterial (Variables|/Script/Engine.StaticMeshActor|GetStaticMeshComponent _asstatic_mesh_actor) _array_index (Variables|Default|GetDissolveMaterial)))
          ;[1 1 1] Destroy rocket
          (Class|AdvancedProjectile|Destroy(Message) (Variables|/Script/Engine.ChildActorComponent|GetChildActor (Variables|Default|GetBP_Rocket)))
          ;[1 1 1] Dissolve animation
          (bind _dissolving (Timeline|Dissolve PlayFromStart)
            (:Update
              (Rendering|Material|SetScalarParameterValue (Variables|Default|GetDissolveMaterial) "Dissolve" _dissolving :!class /Script/Engine.MaterialInstanceDynamic))
            (:Finished
              ;[1 1 1] Try to destroy target and destroy rocket instance
              (if (Utilities|IsValid (.HitActor (Collision|BreakHitResult (Variables|Default|GetHitResult))))
                (Actor|DestroyActor (.HitActor (Collision|BreakHitResult (Variables|Default|GetHitResult))))
                (Actor|DestroyActor)
                (else
                  (Actor|DestroyActor))))))
        (:CastFailed
          ;[1 1 1] Else destroy rocket
          (Class|AdvancedProjectile|Destroy(Message) (Variables|/Script/Engine.ChildActorComponent|GetChildActor (Variables|Default|GetBP_Rocket)))
          (Utilities|FlowControl|Delay 5.0)
          (Actor|DestroyActor))))))

(event EventHomingMissile
  (params (TargetObject :type Static%20Mesh%20Actor%20Object%20Reference))
  ;[1 1 1] Set target
  (Variables|Default|SetTargetObject TargetObject)
  ;[1 1 1] If target is valid
  (if (Utilities|IsValid (Variables|Default|GetTargetObject))
    ;[1 1 1] Set as homing target
    (Variables|/Script/Engine.ProjectileMovementComponent|SetHomingTargetComponent (Variables|MyProjectile|GetProjectile) (Variables|/Script/Engine.StaticMeshActor|GetStaticMeshComponent (Variables|Default|GetTargetObject)))
    ;[1 1 1] Mark as homing projectile and set homing acceleration magnitude
    (Variables|/Script/Engine.ProjectileMovementComponent|SetbIsHomingProjectile (Variables|MyProjectile|GetProjectile) true)
    (Variables|/Script/Engine.ProjectileMovementComponent|SetHomingAccelerationMagnitude (Variables|MyProjectile|GetProjectile) 2e+04)))

(fn ConstructionScript)

(fn ReturnMesh
  ;[1 1 1] Return projectile's mesh
  (Class|AdvancedProjectile|ReturnMesh(Message) (Variables|/Script/Engine.ChildActorComponent|GetChildActor (Variables|Default|GetBP_Rocket)))
  (return 0))

(fn ReturnProjectileMovementComponent
  (return (Variables|MyProjectile|GetProjectile)))
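; Orbital laser strike payload Blueprint that handles the effects for a two-stage projectile strike.
; The first stage saves the impact location, spawns laser beam and scaled flare particle effects there, and plays the beam impact sound.
; The second stage plays a loud explosion sound at the given location and triggers an orbital laser camera shake on the first player's camera.
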(event EventExecute
  (params (Location :type Vector))
  ;[1 1 1] First stage
  ;;[1 1 1] Save impact location
  (Variables|Default|SetImpactLocation Location)
  ;;[1 1 1] Laser beam and explosion effects
  (Effects|SpawnEmitteratLocation "/Game/NewProjectilesPack/Particles/OrbitalLaserBeam/P_LaserBeam.P_LaserBeam" (Variables|Default|GetImpactLocation) "90.000000, 0, 0")
  (bind _returnvalue (Effects|SpawnEmitteratLocation "/Game/NewProjectilesPack/Particles/OrbitalLaserBeam/P_Flare_Laser.P_Flare_Laser" (Variables|Default|GetImpactLocation) "90.000000, 0, 0"))
  (Transformation|SetRelativeScale3D _returnvalue "1.500000,1.500000,1.500000")
  ;;[1 1 1] Laser beam sound
  (Audio|PlaySoundatLocation "/Game/NewProjectilesPack/Sounds/Common/LaserBeamImpact_Cue.LaserBeamImpact_Cue" (Variables|Default|GetImpactLocation)))

(event EventExecuteSecondStage
  (params (Location :type Vector))
  ;[1 1 1] Second stage
  ;;[1 1 1] Play explosion sound
  (Audio|PlaySoundatLocation "/Game/NewProjectilesPack/Sounds/Common/Explosion_03_1.Explosion_03_1" Location "0, 0, 0" 2.0)
  ;;[1 1 1] Camera shake
  (Class|PlayerCameraManager|PlayCameraShake (Variables|/Script/Engine.PlayerController|GetPlayerCameraManager (Game|GetPlayerController 0)) "/Game/NewProjectilesPack/Blueprints/OrbitalLaserBeam/OrbitalLaserBeamShakeBlueprint.OrbitalLaserBeamShakeBlueprint_C" 1.0 "CameraLocal" "0, 0, 0"))
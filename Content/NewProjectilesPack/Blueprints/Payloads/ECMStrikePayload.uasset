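; ECM strike payload that disrupts the homing weapons in the level when executed.
; Execute spawns a scaled explosion emitter at the given location and plays an explosion sound at the world origin.
; It gathers projectile movement components from every HomingWeapon interface actor through an interface message, with no range check.
; Each component gets its gravity scale and homing acceleration overwritten to interrupt its flight.
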(event EventExecute
  (params (Location :type Vector))
  ;[1 1 1] Explosion effect
  (bind _returnvalue (Effects|SpawnEmitteratLocation "/Game/NewProjectilesPack/Particles/ECMStrike/P_ECMStrike_Explosion.P_ECMStrike_Explosion" Location))
  (Transformation|SetRelativeScale3D _returnvalue (Variables|Default|GetExplosionScale))
  ;[1 1 1] Explosion sound
  (Audio|PlaySoundatLocation "/Game/NewProjectilesPack/Sounds/Common/Explosion_02_Cue.Explosion_02_Cue" "0, 0, 0")
  ;[1 1 1] Get all projectile movement components
  (bind _projectilemovementcomponents (CallFunction|GetAllProjectileMovementComponents))
  ;[1 1 1] Interrupt each projectile movement
  (for _array_element _projectilemovementcomponents
    (Variables|/Script/Engine.ProjectileMovementComponent|SetProjectileGravityScale _array_element 1.0)
    (Variables|/Script/Engine.ProjectileMovementComponent|SetHomingAccelerationMagnitude _array_element 1e+02)))

(fn GetAllProjectileMovementComponents
  ;[1 1 1] Find all advanced projectiles
  (bind _outactors (Actor|GetAllActorswithInterface "/Game/NewProjectilesPack/Blueprints/Common/HomingWeapon.HomingWeapon_C"))
  ;[1 1 1] For each homing weapon
  (for _array_element _outactors
    (Variables|Default|SetHomingWeapon _array_element)
    ;[1 1 1] Check for validity
    (if (Utilities|IsValid (Variables|Default|GetHomingWeapon))
      ;[1 1 1] Get projectile movement component
      (bind _projectilemovementcomponent (Class|HomingWeapon|ReturnProjectileMovementComponent(Message) (Variables|Default|GetHomingWeapon)))
      (Variables|Default|SetProjectileMovementComponent _projectilemovementcomponent)
      ;[1 1 1] Check it for validity
      (if (Utilities|IsValid (Variables|Default|GetProjectileMovementComponent))
        ;[1 1 1] Add it to array
        (Utilities|Array|AddUnique (Variables|Default|GetProjectileMovementComponents) (Variables|Default|GetProjectileMovementComponent)))))
  ;[1 1 1] Return all projectile movement components
  (return (Variables|Default|GetProjectileMovementComponents)))
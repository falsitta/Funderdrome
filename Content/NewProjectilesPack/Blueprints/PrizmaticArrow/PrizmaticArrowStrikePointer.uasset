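; Strike pointer projectile for the Prizmatic Arrow effect that bursts into a spread of PrizmaticArrow actors where it hits.
; Its first collision fires an explosion impulse after a brief delay, then runs SpawnPrizmaticRays.
; That loop spawns RaysCount arrows at randomly offset positions, stepping roll, pitch and yaw together by equal fractions of 360 degrees.
; The pointer then stops bouncing and destroys itself after a delay.
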(event OnComponentHit(CollisionComponent)
  (params (HitComponent :type Primitive%20Component%20Object%20Reference) (OtherActor :type Actor%20Object%20Reference) (OtherComp :type Primitive%20Component%20Object%20Reference) (NormalImpulse :type Vector :default "0, 0, 0") (Hit :type Hit%20Result%20Structure%20%28by%20ref%29))
  ;[1 1 1] Execute payload on hit
  (Utilities|FlowControl|DoOnce false
    (:Completed
      (Variables|Default|SetHitResult Hit)
      ;[1 1 1] Delay before spawn
      (Utilities|FlowControl|Delay 0.01)
      ;[1 1 1] Fire impulse
      (Class|RadialForceComponent|FireImpulse (Variables|Default|GetExplosionForce))
      ;[1 1 1] Spawn prizmatic rays
      (CallFunction|SpawnPrizmaticRays (Math|Transform|MakeTransform (Transformation|GetActorLocation) (Transformation|GetWorldRotation (Variables|MyProjectile|GetCollisionComponent))) (Variables|Default|GetTargetObject))
      ;[1 1 1] Destroy actor
      (Variables|/Script/Engine.ProjectileMovementComponent|SetbShouldBounce (Variables|MyProjectile|GetProjectile) false)
      (Utilities|FlowControl|Delay 4.0)
      (Actor|DestroyActor))))

(fn ConstructionScript)

(fn SpawnPrizmaticRays
  (params (Transform :type Transform) (TargetObject :type Static%20Mesh%20Actor%20Object%20Reference))
  ;[1 1 1] Set missile transform and target
  (Variables|Default|SetMissileTransform Transform)
  (Variables|Default|SetTargetObject TargetObject)
  ;[1 1 1] Repeat until all rockets won't be launched
  (if (< (Variables|Default|GetIndex) (Variables|Default|GetRaysCount)) :!label _label
    ;[1 1 1] Increment index
    (Math|Integer|IncrementInt (Variables|Default|GetIndex)
      (:%20%20
        ;[1 1 1] Apply transform
        (bind _outputtransform (CallFunction|RaysTransform))
        ;[1 1 1] Spawn missile
        (Game|SpawnActorfromClass "/Game/NewProjectilesPack/Blueprints/PrizmaticArrow/PrizmaticArrow.PrizmaticArrow_C" _outputtransform "AdjustIfPossibleButDontSpawnIfColliding" 0 0) ; Spawn projectile
        (goto _label)))))

(fn RaysTransform
  (bind _rayscount (Variables|Default|GetRaysCount))
  (bind _missiletransform (Variables|Default|GetMissileTransform))
  (bind _rotation (Math|Transform|BreakTransform _missiletransform))
  (bind _returnvalue (* _rayscount 10))
  (bind (_roll _pitch _yaw) (Math|Rotator|BreakRotator _rotation))
  ;[1 1 1] Calculate rotation shift
  (Variables|Default|SetRotationShift (Math|Conversions|ToFloat(Integer) (* (Variables|Default|GetIndex) (/ 360 (Variables|Default|GetRaysCount)))))
  ;[1 1 1] Return result
  (return (Math|Transform|MakeTransform (+ (.Location (Math|Transform|BreakTransform (Variables|Default|GetMissileTransform))) (Math|Vector|MakeVector (Math|Conversions|ToFloat(Integer) (Math|Random|RandomIntegerinRange 0 _returnvalue)) (Math|Conversions|ToFloat(Integer) (Math|Random|RandomIntegerinRange 0 _returnvalue)) (Math|Conversions|ToFloat(Integer) (Math|Random|RandomIntegerinRange 0 _returnvalue)))) (Math|Rotator|MakeRotator (+ _roll (Variables|Default|GetRotationShift)) (+ _pitch (Variables|Default|GetRotationShift)) (+ _yaw (Variables|Default|GetRotationShift))) (.Scale (Math|Transform|BreakTransform (Variables|Default|GetMissileTransform))))))
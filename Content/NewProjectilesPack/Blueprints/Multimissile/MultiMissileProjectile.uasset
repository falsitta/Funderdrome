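; Multi-missile projectile that can home on a target, then bursts into a cluster of homing missiles on impact or half a second after BeginPlay.
; A one-shot payload fires a radial impulse, smoke and sound, spawns the sub-missiles and destroys the rocket child actor.
; Sub-missiles spawn with random position offsets and evenly stepped rotation shifts, each inheriting the target set through HomingMissile.
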(event OnComponentHit(CollisionComponent)
  (params (HitComponent :type Primitive%20Component%20Object%20Reference) (OtherActor :type Actor%20Object%20Reference) (OtherComp :type Primitive%20Component%20Object%20Reference) (NormalImpulse :type Vector :default "0, 0, 0") (Hit :type Hit%20Result%20Structure%20%28by%20ref%29))
  ;[1 1 1] Execute payload on hir or after specified time
  (Utilities|FlowControl|DoOnce false
    (:Completed
      ;[1 1 1] Fire impulse
      (Class|RadialForceComponent|FireImpulse (Variables|Default|GetExplosionForce))
      ;[1 1 1] Smoke effect
      (Effects|SpawnEmitteratLocation "/Game/NewProjectilesPack/Particles/Effects/P_Smoke.P_Smoke" (Transformation|GetWorldLocation (Variables|Default|GetExplosionForce)) "0, 0,0.000000")
      ;[1 1 1] Explosion sound
      (Audio|PlaySoundatLocation "/Game/NewProjectilesPack/Sounds/Common/Explosion_02_Cue.Explosion_02_Cue" "0, 0, 0")
      ;[1 1 1] Spawn homing missiles
      (CallFunction|SpawnHomingMissiles (Math|Transform|MakeTransform (Transformation|GetActorLocation) (Transformation|GetWorldRotation (Variables|MyProjectile|GetCollisionComponent))) (Variables|Default|GetTargetObject))
      ;[1 1 1] Destroy multimissile
      (Class|AdvancedProjectile|Destroy(Message) (Variables|/Script/Engine.ChildActorComponent|GetChildActor (Variables|Default|GetBP_Rocket))))))

(event EventBeginPlay
  ;[1 1 1] Execute payload on hir or after specified time
  (Utilities|FlowControl|Delay 0.5)
  (Utilities|FlowControl|DoOnce false
    (:Completed
      ;[1 1 1] Fire impulse
      (Class|RadialForceComponent|FireImpulse (Variables|Default|GetExplosionForce))
      ;[1 1 1] Smoke effect
      (Effects|SpawnEmitteratLocation "/Game/NewProjectilesPack/Particles/Effects/P_Smoke.P_Smoke" (Transformation|GetWorldLocation (Variables|Default|GetExplosionForce)) "0, 0,0.000000")
      ;[1 1 1] Explosion sound
      (Audio|PlaySoundatLocation "/Game/NewProjectilesPack/Sounds/Common/Explosion_02_Cue.Explosion_02_Cue" "0, 0, 0")
      ;[1 1 1] Spawn homing missiles
      (CallFunction|SpawnHomingMissiles (Math|Transform|MakeTransform (Transformation|GetActorLocation) (Transformation|GetWorldRotation (Variables|MyProjectile|GetCollisionComponent))) (Variables|Default|GetTargetObject))
      ;[1 1 1] Destroy multimissile
      (Class|AdvancedProjectile|Destroy(Message) (Variables|/Script/Engine.ChildActorComponent|GetChildActor (Variables|Default|GetBP_Rocket))))))

(event EventHomingMissile
  (params (TargetObject :type Static%20Mesh%20Actor%20Object%20Reference))
  ;[1 1 1] Set target
  (Variables|Default|SetTargetObject TargetObject)
  ;[1 1 1] If target is valid
  (if (Utilities|IsValid (Variables|Default|GetTargetObject))
    ;[1 1 1] Set homing target
    (Variables|/Script/Engine.ProjectileMovementComponent|SetHomingTargetComponent (Variables|MyProjectile|GetProjectile) (Variables|/Script/Engine.StaticMeshActor|GetStaticMeshComponent (Variables|Default|GetTargetObject)))
    ;[1 1 1] Mark as homing projectile and set homing acceleration magnitude
    (Variables|/Script/Engine.ProjectileMovementComponent|SetbIsHomingProjectile (Variables|MyProjectile|GetProjectile) true)
    (Variables|/Script/Engine.ProjectileMovementComponent|SetHomingAccelerationMagnitude (Variables|MyProjectile|GetProjectile) 5e+03)))

(fn ConstructionScript)

(fn SpawnHomingMissiles
  (params (Transform :type Transform) (TargetObject :type Static%20Mesh%20Actor%20Object%20Reference))
  ;[1 1 1] Set missile transform and target
  (Variables|Default|SetMissileTransform Transform)
  (Variables|Default|SetTargetObject TargetObject)
  ;[1 1 1] Repeat until all rockets won't be launched
  (if (< (Variables|Default|GetIndex) (Variables|Default|GetRocketCount)) :!label _label
    ;[1 1 1] Increment index
    (Math|Integer|IncrementInt (Variables|Default|GetIndex)
      (:%20%20
        ;[1 1 1] Apply transform
        (bind _outputtransform (CallFunction|HomingTransform))
        ;[1 1 1] Spawn missile
        (bind _returnvalue (Game|SpawnActorfromClass "/Game/NewProjectilesPack/Blueprints/HomingMissile/HomingMissileProjectile.HomingMissileProjectile_C" _outputtransform "AdjustIfPossibleButDontSpawnIfColliding" 0 0)) ; Spawn projectile
        ;[1 1 1] Set target for spawned missile
        (Class|HomingWeapon|HomingMissile(Message) _returnvalue (Variables|Default|GetTargetObject))
        (goto _label)))))

(fn HomingTransform
  (bind _rocketcount (Variables|Default|GetRocketCount))
  (bind _missiletransform (Variables|Default|GetMissileTransform))
  (bind _rotation (Math|Transform|BreakTransform _missiletransform))
  (bind _returnvalue (* _rocketcount 10))
  (bind (_roll _pitch _yaw) (Math|Rotator|BreakRotator _rotation))
  ;[1 1 1] Calculate rotation shift
  (Variables|Default|SetRotationShift (Math|Conversions|ToFloat(Integer) (* (Variables|Default|GetIndex) (/ 360 (Variables|Default|GetRocketCount)))))
  ;[1 1 1] Return result
  (return (Math|Transform|MakeTransform (+ (.Location (Math|Transform|BreakTransform (Variables|Default|GetMissileTransform))) (Math|Vector|MakeVector (Math|Conversions|ToFloat(Integer) (Math|Random|RandomIntegerinRange 0 _returnvalue)) (Math|Conversions|ToFloat(Integer) (Math|Random|RandomIntegerinRange 0 _returnvalue)) (Math|Conversions|ToFloat(Integer) (Math|Random|RandomIntegerinRange 0 _returnvalue)))) (Math|Rotator|MakeRotator (+ _roll (Variables|Default|GetRotationShift)) (+ _pitch (Variables|Default|GetRotationShift)) (+ _yaw (Variables|Default|GetRotationShift))) (.Scale (Math|Transform|BreakTransform (Variables|Default|GetMissileTransform))))))

(fn ReturnMesh
  ;[1 1 1] Return projectile's mesh
  (Class|AdvancedProjectile|ReturnMesh(Message) (Variables|/Script/Engine.ChildActorComponent|GetChildActor (Variables|Default|GetBP_Rocket)))
  (return 0))

(fn ReturnProjectileMovementComponent
  (return (Variables|MyProjectile|GetProjectile)))
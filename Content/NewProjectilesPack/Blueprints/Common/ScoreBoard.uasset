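; Scoreboard that displays the player's total target score and unlocks new projectiles as it grows.
; Every Tick it recomputes the score by summing SpawnCount across its Targets array and writes it to a TextRender.
; Crossing rising thresholds adds the plasma ball, railgun and flamethrower to the FirstPersonCharacter's Projectiles list, gated by DoOnce nodes.
; Each unlock shares one notification: an on-screen message and a particle burst at the player.
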(event Custom|CastFailed
  ;[1 1 1] Message to log if cast to FPC was failed
  (Development|PrintString "Failed to cast to FirstPersonCharacter in ScoreBoard" false))

(event EventTick
  (params (DeltaSeconds :type Float%20%28single-precision%29))
  ;[1 1 1] Reset global score
  (Variables|Default|SetGlobalScore 0)
  ;[1 1 1] For each target
  (for _array_element (Variables|Default|GetTargets)
    ;[1 1 1] Add target hit score to global score
    (Variables|Default|SetGlobalScore (+ (Variables|Default|GetGlobalScore) (Variables|/Game/NewProjectilesPack/Blueprints/Environment/Target.Target_C|GetSpawnCount _array_element))))
  ;[1 1 1] Apply score to text render
  (Rendering|Components|TextRender|SetText (Variables|Default|GetTextRender) (Utilities|Text|ToText(String) (Utilities|String|Append (Variables|Default|GetScore%20Text) (Utilities|String|ToString(Integer) (Variables|Default|GetGlobalScore)))))
  ;[1 1 1] Sequence
  (Utilities|FlowControl|Sequence
    (:then_0
      ;[1 1 1] Add plasma ball if score > 10
      (if (> (Variables|Default|GetGlobalScore) 10)
        (Utilities|FlowControl|DoOnce false
          (:Completed
            (bind _asfirst_person_character (Utilities|Casting|CastToFirstPersonCharacter (Game|Player|GetPlayerPawn 0))
              (:then
                (Utilities|FlowControl|DoOnce false
                  (:Completed
                    (Utilities|Array|AddUnique (Variables|/Game/NewProjectilesPack/Blueprints/FirstPerson/FirstPersonCharacter.FirstPersonCharacter_C|GetProjectiles _asfirst_person_character) "/Game/NewProjectilesPack/Blueprints/PlasmaBall/PlasmaBallProjectile.PlasmaBallProjectile_C")
                    ;[1 1 1] Text message about new projectile
                    (Development|PrintString "New projectiles has been unlocked!" true true "(R=0.000000,G=0.660000,B=1.000000,A=1.000000)" 5.0 :!label _label)
                    ;[1 1 1] Effect to notify user about new projectile
                    (Effects|SpawnEmitteratLocation "/Game/NewProjectilesPack/Particles/MicrodestructorMissile/P_Microdestructor_Swarm.P_Microdestructor_Swarm" (Transformation|GetActorLocation (Game|GetPlayerCharacter 0))))))
              (:CastFailed
                (CallFunction|CastFailed)))))))
    (:then_1
      ;[1 1 1] Add railgun if score > 25
      (if (> (Variables|Default|GetGlobalScore) 25)
        (Utilities|FlowControl|DoOnce false
          (:Completed
            (bind _asfirst_person_character_2 (Utilities|Casting|CastToFirstPersonCharacter (Game|Player|GetPlayerPawn 0))
              (:then
                (Utilities|FlowControl|DoOnce false
                  (:Completed
                    (Utilities|Array|AddUnique (Variables|/Game/NewProjectilesPack/Blueprints/FirstPerson/FirstPersonCharacter.FirstPersonCharacter_C|GetProjectiles _asfirst_person_character_2) "/Game/NewProjectilesPack/Blueprints/Railgun/RailgunProjectile.RailgunProjectile_C")
                    (goto _label))))
              (:CastFailed
                (CallFunction|CastFailed)))))))
    (:then_2
      ;[1 1 1] Add flamethrower if score > 50
      (if (> (Variables|Default|GetGlobalScore) 50)
        (Utilities|FlowControl|DoOnce false
          (:Completed
            (bind _asfirst_person_character_3 (Utilities|Casting|CastToFirstPersonCharacter (Game|Player|GetPlayerPawn 0))
              (:then
                (Utilities|FlowControl|DoOnce false
                  (:Completed
                    (Utilities|Array|AddUnique (Variables|/Game/NewProjectilesPack/Blueprints/FirstPerson/FirstPersonCharacter.FirstPersonCharacter_C|GetProjectiles _asfirst_person_character_3) "/Game/NewProjectilesPack/Blueprints/Flamethrower/Flamethrower.Flamethrower_C")
                    (goto _label))))
              (:CastFailed
                (CallFunction|CastFailed)))))))))

(fn ConstructionScript)
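; Strategic AI boss pod that periodically bombards the player from orbit until it is destroyed to win.
; A looping timer, plus an earlier first strike, snapshots the player's location, plays a heartbeat warning, then alternates three kinetic missile beacons with an orbital laser beam.
; Damage drains hit points; at zero, a delayed loop runs bursts of explosions, then sets IsDestroyed, prints the win text and drives the pod's emissive material with a timeline.
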(event Custom|AttackPlayer
  ;[1 1 1] If strategic AI is alive
  (if (not (Variables|Default|GetIsDestroyed))
    ;[1 1 1] Set player location
    (Variables|Default|SetPlayerLocation (Transformation|GetActorLocation (Game|Player|GetPlayerPawn 0)))
    ;[1 1 1] Play sound to notify player
    (Audio|PlaySoundatLocation "/Game/NewProjectilesPack/Sounds/Common/HeartBeat_Cue.HeartBeat_Cue" (Variables|Default|GetPlayerLocation))
    (Utilities|FlowControl|Delay 6.0)
    ;[1 1 1] Change attack type
    (Utilities|FlowControl|FlipFlop
      (:A
        ;[1 1 1] Attack with kinetic orbital strike (3 times)
        (Game|SpawnActorfromClass "/Game/NewProjectilesPack/Blueprints/OrbitalKineticMissile/KineticMissileBeacon.KineticMissileBeacon_C" (Math|Transform|MakeTransform (Variables|Default|GetPlayerLocation)) "AlwaysSpawn" 0 0) ; Spawn projectile
        (Utilities|FlowControl|Delay 1.0)
        (Game|SpawnActorfromClass "/Game/NewProjectilesPack/Blueprints/OrbitalKineticMissile/KineticMissileBeacon.KineticMissileBeacon_C" (Math|Transform|MakeTransform (+ (Variables|Default|GetPlayerLocation) "4000.000000, 0, 0")) "AlwaysSpawn" 0 0) ; Spawn projectile
        (Utilities|FlowControl|Delay 1.0)
        (Game|SpawnActorfromClass "/Game/NewProjectilesPack/Blueprints/OrbitalKineticMissile/KineticMissileBeacon.KineticMissileBeacon_C" (Math|Transform|MakeTransform (+ (Variables|Default|GetPlayerLocation) "0,4000.000000, 0")) "AlwaysSpawn" 0 0) ; Spawn projectile
      )
      (:B
        ;[1 1 1] Attack with orbital laser beam
        (Game|SpawnActorfromClass "/Game/NewProjectilesPack/Blueprints/OrbitalLaserBeam/OrbitalLaserBeam.OrbitalLaserBeam_C" (Math|Transform|MakeTransform (+ (Variables|Default|GetPlayerLocation) "4000.000000, 0, 0")) "AlwaysSpawn" 0 0) ; Spawn projectile
      ))))

(event EventBeginPlay
  ;[1 1 1] Set explosion scale
  (Variables|/Game/NewProjectilesPack/Blueprints/Payloads/SimpleExplosionPayload.SimpleExplosionPayload_C|SetExplosionScale (Variables|Default|GetSimpleExplosionPayload) "10.000000,10.000000,10.000000")
  ;[1 1 1] Set attack timer
  (Utilities|Time|SetTimerbyEvent (delegate Custom|AttackPlayer) (Math|Random|RandomFloatinRange 5e+01 6e+01) true)
  ;[1 1 1] First attack on player
  (Utilities|FlowControl|Delay (Math|Random|RandomFloatinRange 1e+01 2e+01))
  (if (not (Variables|Default|GetIsDestroyed))
    (CallFunction|AttackPlayer)))

(event Game|Damage|EventAnyDamage
  (params (Damage :type Float%20%28single-precision%29) (DamageType :type Damage%20Type%20Object%20Reference) (InstigatedBy :type Controller%20Object%20Reference) (DamageCauser :type Actor%20Object%20Reference))
  ;[1 1 1] On any type of damage
  ;[1 1 1] If Strategic AI is alive
  (if (not (Variables|Default|GetIsDestroyed))
    ;[1 1 1] Decrease hit points
    (Variables|Default|SetHitPoints (- (Variables|Default|GetHitPoints) Damage))
    ;[1 1 1] If HitPoints <= 0
    (if (<= (Variables|Default|GetHitPoints) 0.0)
      ;[1 1 1] Start explosion animation
      (Utilities|FlowControl|DoOnce false
        (:Completed
          ;[1 1 1] Repeat explosions in different locations
          (if (< (Variables|Default|GetIndex) 20) :!label _label
            ;[1 1 1] Increment index
            (Math|Integer|IncrementInt (Variables|Default|GetIndex)
              (:%20%20
                ;[1 1 1] Make 4 explosions at one moment in different locations of AI Pod
                (Default|Execute (Variables|Default|GetSimpleExplosionPayload) (Utilities|GetExplosionLocation))
                (Default|Execute (Variables|Default|GetSimpleExplosionPayload) (Utilities|GetExplosionLocation))
                (Default|Execute (Variables|Default|GetSimpleExplosionPayload) (Utilities|GetExplosionLocation))
                (Default|Execute (Variables|Default|GetSimpleExplosionPayload) (Utilities|GetExplosionLocation))
                (Utilities|FlowControl|Delay 0.4)
                (goto _label)))
            (else
              ;[1 1 1] Strategic AI was destroyed
              (Variables|Default|SetIsDestroyed true)
              ;[1 1 1] Text about win
              (Development|PrintString "Now you can continue exploring arena. Until next load at least ;)" true true "(R=0.000000,G=0.660000,B=1.000000,A=1.000000)" 2e+01)
              (Development|PrintString "Strategic AI was destroyed. You win!" true true "(R=0.000000,G=0.660000,B=1.000000,A=1.000000)" 2e+01)
              ;[1 1 1] Fade out the lights on AI Pod
              (bind _returnvalue (Rendering|Material|CreateDynamicMaterialInstance (Variables|Default|GetSM_Strategic_AI_Pod) 0 "/Game/NewProjectilesPack/Materials/Common/M_Strategic_AI_Pod_Inst.M_Strategic_AI_Pod_Inst" :!class /Script/Engine.PrimitiveComponent))
              (Variables|Default|SetDynamicMaterialInstance _returnvalue)
              (Rendering|Material|SetScalarParameterValue (Variables|Default|GetDynamicMaterialInstance) "Timing" 0.0 :!class /Script/Engine.MaterialInstanceDynamic)
              (bind _power (Timeline|EmmisivePower PlayFromStart)
                (:Update
                  (Rendering|Material|SetScalarParameterValue (Variables|Default|GetDynamicMaterialInstance) "EmmisivePower" _power :!class /Script/Engine.MaterialInstanceDynamic))))))))))

(fn ConstructionScript)
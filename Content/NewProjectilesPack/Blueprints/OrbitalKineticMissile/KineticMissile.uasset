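; Orbital kinetic missile actor that detonates on the first hit of its collision component, then destroys itself.
; Impact fires a radial force impulse, spawns a scaled-up explosion effect with sound, plays a camera shake on the first player, and attaches a temporary decal to the hit component.
; Radial damage takes its amount and radius from the ExplosionForce component, so that component drives both physics push and damage.
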(event OnComponentHit(CollisionComponent)
  (params (HitComponent :type Primitive%20Component%20Object%20Reference) (OtherActor :type Actor%20Object%20Reference) (OtherComp :type Primitive%20Component%20Object%20Reference) (NormalImpulse :type Vector :default "0, 0, 0") (Hit :type Hit%20Result%20Structure%20%28by%20ref%29))
  (bind _explosionforce (Variables|Default|GetExplosionForce))
  ;[1 1 1] Only on first impact
  (Utilities|FlowControl|DoOnce false
    (:Completed
      ;[1 1 1] Set hit result
      (Variables|Default|SetHitResult Hit)
      ;[1 1 1] Fire impulse
      (Class|RadialForceComponent|FireImpulse (Variables|Default|GetExplosionForce))
      ;[1 1 1] Explosion effect
      (bind _returnvalue (Effects|SpawnEmitteratLocation "/Game/NewProjectilesPack/Particles/Effects/P_Explosion.P_Explosion" (Transformation|GetWorldLocation (Variables|Default|GetExplosionForce))))
      (Transformation|SetRelativeScale3D _returnvalue "20.000000,20.000000,20.000000")
      ;[1 1 1] Explosion sound
      (Audio|PlaySoundatLocation "/Game/NewProjectilesPack/Sounds/Common/Explosion_02_Cue.Explosion_02_Cue" (Transformation|GetWorldLocation (Variables|Default|GetExplosionForce)))
      ;[1 1 1] Camera shake
      (Class|PlayerCameraManager|PlayCameraShake (Variables|/Script/Engine.PlayerController|GetPlayerCameraManager (Game|GetPlayerController 0)) "/Game/NewProjectilesPack/Blueprints/OrbitalKineticMissile/KineticMissileShakeBlueprint.KineticMissileShakeBlueprint_C" 1.0 "CameraLocal" "0, 0, 0")
      ;[1 1 1] Set hit component
      (Variables|Default|SetHitComponent (.HitComponent (Collision|BreakHitResult (Variables|Default|GetHitResult))))
      ;[1 1 1] Spawn decal
      (Class|GameplayStatics|SpawnDecalAttached "/Game/NewProjectilesPack/Materials/Bullet/M_Impact_Decal.M_Impact_Decal" "2000.000000,2000.000000,2000.000000" (Variables|Default|GetHitComponent) "None" (.Location (Collision|BreakHitResult (Variables|Default|GetHitResult))) (Math|Conversions|RotationFromXVector (.Normal (Collision|BreakHitResult (Variables|Default|GetHitResult)))) "KeepWorldPosition" 15.0)
      ;[1 1 1] Apply damage
      (Game|Damage|ApplyRadialDamage (Variables|/Script/Engine.RadialForceComponent|GetDestructibleDamage _explosionforce) (Transformation|GetWorldLocation _explosionforce) (Variables|/Script/Engine.RadialForceComponent|GetRadius _explosionforce) "/Script/Engine.DamageType" 0 self 0 false "ECC_Visibility")
      ;[1 1 1] Destroy actor
      (Actor|DestroyActor))))

(fn ConstructionScript)
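; Ultradrome player controller that relays player name, UI and round-result events to the Ultradrome game instance.
; It copies the player name from the game instance and forwards death events to remove the UI.
; GameOverWin inverts the Team1Lose flag before passing it to RoundOver, while a separate GameOver event opens the MainMenu level.
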(event Custom|GameOver
  (Game|OpenLevel(byName) "MainMenu"))

(event Custom|GetPlayername
  (bind _asultradrome_game_instance (Utilities|Casting|CastToUltradrome_GameInstance (Game|GetGameInstance)))
  (CallFunction|SetPlayerName (Variables|/Game/Blueprints/Ultradrome_GameInstance.Ultradrome_GameInstance_C|GetPlayerName _asultradrome_game_instance)))

(event Custom|SetPlayerName
  (params (name :type String))
  (Variables|Default|SetPlayerName name))

(event Custom|GameOver%20Win
  (params (Team1Lose :type Boolean))
  (bind _asultradrome_game_instance (Utilities|Casting|CastToUltradrome_GameInstance (Game|GetGameInstance)))
  (Default|RoundOver _asultradrome_game_instance (not Team1Lose)))

(event Custom|Death%20removeUI
  (bind _asultradrome_game_instance (Utilities|Casting|CastToUltradrome_GameInstance (Game|GetGameInstance)))
  (Default|RemoveUI _asultradrome_game_instance))

(fn ConstructionScript)
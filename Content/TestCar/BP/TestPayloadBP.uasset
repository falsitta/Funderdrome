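; Drivable eight-wheeled payload for FunderDrome payload mode, moved by a vehicle movement component fed throttle, brake and turn.
; Team 2 turret damage lowers its health and notifies the game mode, which ends the match at zero.
; Team 2 cars inside the shield collider scale damage reduction along a lobby-selected linear, logarithmic or quadratic curve.
; The server replicates physics state on a timer; clients extrapolate, then blend or snap.
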(event OnComponentBeginOverlap(ShieldCollider)
  (params (OverlappedComponent :type Primitive%20Component%20Object%20Reference) (OtherActor :type Actor%20Object%20Reference) (OtherComp :type Primitive%20Component%20Object%20Reference) (OtherBodyIndex :type Integer) (bFromSweep :type Boolean) (SweepResult :type Hit%20Result%20Structure%20%28by%20ref%29))
  (if (Components|ComponentHasTag OtherComp "Car")
    (bind _asfunder_drome_car_base (Utilities|Casting|CastToFunderDromeCarBase OtherActor))
    (if (== (Variables|/Game/TestCar/BP/FunderDromeCarBase.FunderDromeCarBase_C|GetTeam _asfunder_drome_car_base) 2)
      (Math|Integer|IncrementInt (Variables|Default|GetAlliedCarsInRange)
        (:%20%20
          (CallFunction|ComputeDamageReduction))))))

(event OnComponentEndOverlap(ShieldCollider)
  (params (OverlappedComponent :type Primitive%20Component%20Object%20Reference) (OtherActor :type Actor%20Object%20Reference) (OtherComp :type Primitive%20Component%20Object%20Reference) (OtherBodyIndex :type Integer))
  (if (Components|ComponentHasTag OtherComp "Car")
    (bind _asfunder_drome_car_base (Utilities|Casting|CastToFunderDromeCarBase OtherActor))
    (if (== (Variables|/Game/TestCar/BP/FunderDromeCarBase.FunderDromeCarBase_C|GetTeam _asfunder_drome_car_base) 2)
      (Math|Integer|DecrementInt (Variables|Default|GetAlliedCarsInRange)
        (:%20%20
          (CallFunction|ComputeDamageReduction))))))

(event Custom|SyncStart%28Server%29
  (params (Package :type Sync%20Package%20Structure))
  ;[1 1 1] Sync Code
  (Variables|Default|SetSyncedPackage Package))

(event Custom|DataSync
  (bind _payloadmesh (Variables|Default|GetPayloadMesh))
  (bind _returnvalue (Transformation|GetWorldTransform _payloadmesh))
  (bind (_location _rotation) (Math|Transform|BreakTransform _returnvalue))
  (bind (_roll _pitch _yaw) (Math|Rotator|BreakRotator _rotation))
  ;[1 1 1] Sync Code
  (Networking|SwitchHasAuthority
    (:Authority
      (bind _returnvalue_2 (Physics|GetPhysicsLinearVelocity _payloadmesh "None"))
      (bind _returnvalue_3 (Class|PrimitiveComponent|GetPhysicsAngularVelocity _payloadmesh "None"))
      (CallFunction|SyncStart(Server) (Utilities|Struct|MakeSyncPackage (Utilities|Array|MakeArray _location (Math|Vector|MakeVector _roll _pitch _yaw) _returnvalue_2 _returnvalue_3) 0 (Utilities|Time|GetRealTimeSeconds))))))

(event Custom|Payload%20Initiation
  (Variables|Default|SetInitialized true)
  (Variables|Default|SetHealth (Variables|Default|GetMaxHealth))
  (Physics|SetEnableGravity (Variables|Default|GetPayloadMesh) true)
  (Default|EngineStart (Variables|Default|GetFunderDromeVehicleMovement)))

(event Custom|ComputeDamageReduction
  (bind _asultradrome_game_instance (Utilities|Casting|CastToUltradrome_GameInstance (Game|GetGameInstance)))
  (switch int (Variables|/Game/HUD/InGameMenu/Lobby_UI.Lobby_UI_C|GetDamageReductionScalingInfo (Variables|/Game/BluePrint/AllLevels/Ultradrome_GameInstance.Ultradrome_GameInstance_C|GetLobbyMenu _asultradrome_game_instance))
    (:Default
      ;[1 1 1] Linear (Neutral)
      (Development|PrintString (Utilities|String|ToString(Integer) (Variables|Default|GetAlliedCarsInRange)) :!label _label)
      (Variables|Default|SetDamageReductionModifier (/ (Math|Conversions|ToFloat(Integer) (Variables|Default|GetAlliedCarsInRange)) (Math|Conversions|ToFloat(Integer) (Variables|Default|GetNumAlliedCars)))))
    (:0
      (goto _label))
    (:1
      ;[1 1 1] Logarithmic (Defense favoured)
      (Development|PrintString (Utilities|String|ToString(Integer) (Variables|Default|GetAlliedCarsInRange)))
      (Variables|Default|SetDamageReductionModifier (CallFunction|LogBaseXofY (+ (Math|Conversions|ToFloat(Integer) (Variables|Default|GetNumAlliedCars)) 1.0) (+ (Math|Conversions|ToFloat(Integer) (Variables|Default|GetAlliedCarsInRange)) 1.0))))
    (:2
      ;[1 1 1] Quadratic (Offense favoured) we can change the exponent to make it more or less heavily favoured
      (Development|PrintString (Utilities|String|ToString(Integer) (Variables|Default|GetAlliedCarsInRange)))
      (Variables|Default|SetDamageReductionModifier (Math|Float|Square (/ (Math|Conversions|ToFloat(Integer) (Variables|Default|GetAlliedCarsInRange)) (Math|Conversions|ToFloat(Integer) (Variables|Default|GetNumAlliedCars))))))))

(event EventBeginPlay
  (if (Variables|Default|GetInitialized)
    (CallFunction|PayloadInitiation))
  (Default|Init (Variables|Default|GetFunderDromeVehicleMovement) (Variables|Default|GetPayloadMesh) (Utilities|Array|MakeArray (Variables|Default|GetWheelsL1) (Variables|Default|GetWheelsL2) (Variables|Default|GetWheelsR1) (Variables|Default|GetWheelsR2)) (Utilities|Array|MakeArray (Variables|Default|GetWheelsL3) (Variables|Default|GetWheelsL4) (Variables|Default|GetWheelsR3) (Variables|Default|GetWheelsR4)) (Utilities|Array|MakeArray (Variables|Default|GetmeshL1) (Variables|Default|GetmeshL2) (Variables|Default|GetmeshR1) (Variables|Default|GetmeshR2) (Variables|Default|GetmeshL3) (Variables|Default|GetmeshL4) (Variables|Default|GetmeshR3) (Variables|Default|GetmeshR4)) self)
  (bind _asfunder_drome_payload_mode (Utilities|Casting|CastToFunderDromePayloadMode (Game|GetGameMode))
    (:then
      (Variables|Default|SetGameModeRef _asfunder_drome_payload_mode)
      (Utilities|FlowControl|Sequence
        (:then_0
          ;[1 1 1] Sync Code
          (Utilities|Time|SetTimerbyEvent (delegate Custom|DataSync) 0.05 true :!label _label))
        (:then_1
          (bind _outactors (Actor|GetAllActorsOfClass "/Game/TestCar/BP/FunderDromeCarBase.FunderDromeCarBase_C"))
          (for _array_element _outactors
            (if (== (Variables|/Game/TestCar/BP/FunderDromeCarBase.FunderDromeCarBase_C|GetTeam _array_element) 2)
              (Math|Integer|IncrementInt (Variables|Default|GetNumAlliedCars))))
          (Development|PrintString (Utilities|String|ToString(Integer) (Variables|Default|GetNumAlliedCars)) true true "(R=1.000000,G=0.000000,B=0.272114,A=1.000000)" 1e+01))))
    (:CastFailed
      (goto _label))))

(event EventTick
  (params (DeltaSeconds :type Float%20%28single-precision%29))
  (Default|MoveControl (Variables|Default|GetFunderDromeVehicleMovement) (Variables|Default|GetThrottle) (Variables|Default|GetBrake) (Variables|Default|GetRight) false)
  (Variables|Default|SetSpeed (Math|Vector|VectorLength (Variables|/Game/TestCar/BP/FunderDromeVehicleMovement.FunderDromeVehicleMovement_C|GetVel (Variables|Default|GetFunderDromeVehicleMovement)))))

(event EventSetBrake
  (params (Input :type Float%20%28single-precision%29))
  (Variables|Default|SetBrake Input))

(event EventSetThrottle
  (params (Input :type Float%20%28single-precision%29))
  (Variables|Default|SetThrottle Input))

(event EventSetTurn
  (params (Input :type Float%20%28single-precision%29))
  (Variables|Default|SetRight Input))

(event Game|Damage|EventAnyDamage
  (params (Damage :type Float%20%28single-precision%29) (DamageType :type Damage%20Type%20Object%20Reference) (InstigatedBy :type Controller%20Object%20Reference) (DamageCauser :type Actor%20Object%20Reference))
  (bind _gamemoderef (Variables|Default|GetGameModeRef))
  (Utilities|Casting|CastToDuke_Projectile DamageCauser
    (:then
      (bind _asfunder_drome_turret_base (Utilities|Casting|CastToFunderDromeTurretBase (Variables|/Script/Engine.Actor|GetInstigator DamageCauser)))
      (if (== (Variables|/Game/BluePrint/Turret/FunderDromeTurretBase.FunderDromeTurretBase_C|GetTeam _asfunder_drome_turret_base) 2)
        (Default|DamageNotify _gamemoderef _asfunder_drome_turret_base)
        (bind _output_get (Variables|Default|SetHealth (- (Variables|Default|GetHealth) (* Damage (- 1.0 (Variables|Default|GetDamageReductionModifier)))) :!label _label))
        (Default|PayloadUpdateHealth _gamemoderef _output_get)
        (if (<= _output_get 0.0)
          (Utilities|FlowControl|DoOnce false
            (:Completed
              (Default|EndOfMatch _gamemoderef 2 (Transformation|GetActorLocation)))))))
    (:CastFailed
      (bind _asfunder_drome_turret_base_2 (Utilities|Casting|CastToFunderDromeTurretBase DamageCauser))
      (if (== (Variables|/Game/BluePrint/Turret/FunderDromeTurretBase.FunderDromeTurretBase_C|GetTeam _asfunder_drome_turret_base_2) 2)
        (Default|DamageNotify _gamemoderef _asfunder_drome_turret_base_2)
        (goto _label)))))

(event Input|AxisEvents|InputAxisThrottle
  (params (AxisValue :type Float%20%28single-precision%29))
  (Variables|Default|SetThrottle AxisValue))

(event Input|AxisEvents|InputAxisBrake
  (params (AxisValue :type Float%20%28single-precision%29))
  (Variables|Default|SetBrake AxisValue))

(event Input|AxisEvents|InputAxisTurnRight
  (params (AxisValue :type Float%20%28single-precision%29))
  (Variables|Default|SetRight AxisValue))

(fn ConstructionScript)

(fn OnRepSyncedPackage
  (bind _syncedpackage (Variables|Default|GetSyncedPackage))
  (bind _payloadmesh (Variables|Default|GetPayloadMesh))
  (bind _item (Utilities|Array|Get(acopy) (.orientation _syncedpackage) 3))
  (bind _item_2 (Utilities|Array|Get(acopy) (.orientation _syncedpackage) 2))
  (bind _returnvalue (Transformation|GetWorldTransform _payloadmesh))
  (LocalVariables|SetServerDelta (/ (- (.realworldtimepart _syncedpackage) (Variables|Default|GetServerRealSecond)) 2.0))
  (Variables|Default|SetServerRealSecond (.realworldtimepart _syncedpackage))
  (Networking|SwitchHasAuthority
    (:Remote
      (if (not (> (LocalVariables|GetServerDelta) 2.0))
        (Physics|SetPhysicsLinearVelocity _payloadmesh _item_2 false "None")
        (Class|PrimitiveComponent|SetPhysicsAngularVelocity _payloadmesh _item false "None")
        (bind _output_get (LocalVariables|SetPredictedTrans (Math|Transform|MakeTransform (+ (Utilities|Array|Get(acopy) (.orientation _syncedpackage)) (* _item_2 (LocalVariables|GetServerDelta))) (Math|Rotator|MakeRotator (.x (+ (Utilities|Array|Get(acopy) (.orientation _syncedpackage) 1) (* _item (LocalVariables|GetServerDelta)))) (.y (+ (Utilities|Array|Get(acopy) (.orientation _syncedpackage) 1) (* _item (LocalVariables|GetServerDelta)))) (.z (+ (Utilities|Array|Get(acopy) (.orientation _syncedpackage) 1) (* _item (LocalVariables|GetServerDelta))))))))
        (if (Class|KismetMathLibrary|NearlyEqualTransformTransform _returnvalue (Math|Transform|MakeTransform (+ (Utilities|Array|Get(acopy) (.orientation _syncedpackage)) (* _item_2 (LocalVariables|GetServerDelta))) (Math|Rotator|MakeRotator (.x (+ (Utilities|Array|Get(acopy) (.orientation _syncedpackage) 1) (* _item (LocalVariables|GetServerDelta)))) (.y (+ (Utilities|Array|Get(acopy) (.orientation _syncedpackage) 1) (* _item (LocalVariables|GetServerDelta)))) (.z (+ (Utilities|Array|Get(acopy) (.orientation _syncedpackage) 1) (* _item (LocalVariables|GetServerDelta)))))) 1e+03 1e+01 0.0001)
          (Transformation|SetWorldTransform _payloadmesh (Math|Transform|Lerp(Transform) _returnvalue _output_get 0.1) false true)
          (else
            (Transformation|SetWorldTransform _payloadmesh _output_get false true)))))))

(fn LogBaseXofY
  (params (X :type Float%20%28single-precision%29) (Y :type Float%20%28single-precision%29))
  (return (/ (Math|Float|Loge Y) (Math|Float|Loge X))))
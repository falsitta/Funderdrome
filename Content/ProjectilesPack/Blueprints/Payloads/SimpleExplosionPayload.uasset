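; Projectile payload Blueprint that produces a cosmetic explosion at the location passed to its Execute event.
; It spawns a shrapnel explosion particle effect scaled by ExplosionScale, plays an explosion sound and shakes the first player's camera.
; Shake strength falls linearly with camera distance, from double at the impact through normal at Radius to zero at twice Radius, with no clamp beyond that.
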(event EventExecute
  (params (Location :type Vector))
  (bind _returnvalue (Game|GetPlayerController 0))
  (bind _radius (Variables|Default|Getradius))
  (bind _playercameramanager (Variables|/Script/Engine.PlayerController|GetPlayerCameraManager _returnvalue))
  ;[1 1 1] Save impact location
  (Variables|Default|SetImpactLocation Location)
  ;[1 1 1] Explosion effect
  (bind _returnvalue_2 (Effects|SpawnEmitteratLocation "/Game/ProjectilesPack/Particles/Effects/P_ExplosionWithShrapnel.P_ExplosionWithShrapnel" (Variables|Default|GetImpactLocation)))
  (Transformation|SetRelativeScale3D _returnvalue_2 (Variables|Default|GetExplosionScale))
  ;[1 1 1] Explosion sound
  (Audio|PlaySoundatLocation "/Game/ProjectilesPack/Sounds/Common/Explosion_01_Cue.Explosion_01_Cue" (Variables|Default|GetImpactLocation))
  ;[1 1 1] Camera shake
  (Class|PlayerCameraManager|PlayCameraShake _playercameramanager "/Game/ProjectilesPack/Blueprints/Common/SimpleShakeBlueprint.SimpleShakeBlueprint_C" (- 1.0 (/ (- (Math|Vector|VectorLength (- (Variables|Default|GetImpactLocation) (Transformation|GetActorLocation _playercameramanager))) _radius) _radius)) "CameraLocal" "0, 0, 0"))